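; BP_PoseCharacter is a posed character actor, filed under cinematics, that is colored to match a chosen player class.
; Its construction script runs ApplyClass, which looks up the PlayerClass row in DT_PlayerStats by enum name.
; The row's LightColor sets the PrimaryColor parameter on a new dynamic instance of each mesh material and also tints the point light.
; It has no active runtime logic.
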(event EventBeginPlay)

(event Collision|EventActorBeginOverlap
  (params (OtherActor :type Actor%20Object%20Reference)))

(event EventTick
  (params (DeltaSeconds :type Float%20%28single-precision%29)))

(fn ConstructionScript
  (CallFunction|ApplyClass))

(fn ApplyClass
  (bind _returnvalue (Utilities|GetDataTableRow "/Game/Dynamic/Blueprints/Character/DT_PlayerStats.DT_PlayerStats" (Utilities|String|StringToName (Utilities|String|EnumtoString (Variables|Default|GetPlayerClass))))
    (:then
      (Utilities|FlowControl|Sequence
        (:then_0
          (for (_array_element _array_index) (Rendering|Material|GetMaterials (Variables|Character|GetMesh))
            (bind _returnvalue_2 (Rendering|Material|CreateDynamicMaterialInstance (Variables|Character|GetMesh) _array_index _array_element "None" :!class /Script/Engine.PrimitiveComponent))
            (Rendering|Material|SetVectorParameterValue _returnvalue_2 "PrimaryColor" (Utilities|Struct|BreakS_PlayerStat _returnvalue) :!class /Script/Engine.MaterialInstanceDynamic)))
        (:then_1
          (Rendering|Components|Light|SetLightColor (Variables|Default|GetPointLight) (Utilities|Struct|BreakS_PlayerStat _returnvalue) true))))))