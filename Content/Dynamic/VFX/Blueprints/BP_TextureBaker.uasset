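; BP_TextureBaker is an editor utility actor that bakes a material into a static texture asset.
; BakeTexture checks that the render target and material are valid, draws the material into the target, then saves it as a Texture2D named with a "T_" prefix plus TextureName.
; Asset creation is editor-only; the event graph is empty, and the construction script's text-label update is disconnected.
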(event EventBeginPlay)

(event Collision|EventActorBeginOverlap
  (params (OtherActor :type Actor%20Object%20Reference)))

(event EventTick
  (params (DeltaSeconds :type Float%20%28single-precision%29)))

(fn ConstructionScript)

(fn BakeTexture
  (bind _render_target_for_bake (Variables|Default|GetRender%20Target%20for%20Bake))
  (if (and (Utilities|IsValid (Variables|Default|GetRender%20Target%20for%20Bake)) (Utilities|IsValid (Variables|Default|GetMaterial%20to%20Bake)))
    (Rendering|DrawMaterialtoRenderTarget _render_target_for_bake (Variables|Default|GetMaterial%20to%20Bake))
    (Class|KismetRenderingLibrary|RenderTargetCreateStaticTexture2DEditorOnly _render_target_for_bake (Utilities|String|Append "T_" (Variables|Default|GetTextureName)) "TC_Default" "TMGS_FromTextureGroup")))