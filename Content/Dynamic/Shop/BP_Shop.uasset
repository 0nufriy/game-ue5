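; Multiplayer shopkeeper actor that sells items, ammo and player revives for the ship's shared money.
; Interact opens a per-player UW_Shop widget once the multicast money value arrives.
; The server handles purchases via DT_Items, launching items toward the buyer, adding ammo or reviving, then deducts money and multicasts stock to widgets.
; Activate shows the shop and adds that round's items, with player-count stock overrides, merging matching entries.
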(event OnComponentEndOverlap(PlayerTrigger)
  (params (OverlappedComponent :type Primitive%20Component%20Object%20Reference) (OtherActor :type Actor%20Object%20Reference) (OtherComp :type Primitive%20Component%20Object%20Reference) (OtherBodyIndex :type Integer))
  ;[0.01042 0.01042 0.01042] Player trigger
  (if (Actor|ActorHasTag OtherActor "Player")
    (bind _controller (Class|BPIPlayers|GetPlayerController(Message) OtherActor))
    (Widget|RemoveWidget _controller)))

(event Custom|SetMoneyServer
  ;[0.01042 0.01042 0.01042] Muticasts
  ;;[0.01042 0.01042 0.01042] Money
  (CallFunction|SetMoneyMulticast (Class|ResourceManager|GetResource (Class|ShipResourcesSubsystem|GetMoneyManager (Subsystems|GetShipResourcesSubsystem)))))

(event Custom|UpdateMoney
  (params (NewAmount :type Integer))
  ;[0.01042 0.01042 0.01042] Core
  (CallFunction|UpdateMoneyMulticast NewAmount))

(event Custom|SetMoneyMulticast
  (params (Money :type Integer))
  ;[0.01042 0.01042 0.01042] Muticasts
  ;;[0.01042 0.01042 0.01042] Money
  (Variables|Default|SetMoney Money)
  (Variables|Default|SetIsMoneyRecive true))

(event Custom|AddWidget
  (params (PlayerController :type Player%20Controller%20Object%20Reference))
  ;[0.01042 0.01042 0.01042] Interaction
  (if (Variables|Default|GetIsMoneyRecive) :!label _label
    (bind _returnvalue (UserInterface|CreateWidget "/Game/Dynamic/Shop/UI/UW_Shop.UW_Shop_C" PlayerController (Variables|Default|GetItems) self (Variables|Default|GetMoney)))
    (bind _output_get (Variables|Default|SetWidget _returnvalue))
    (Utilities|Map|Add (Variables|Default|GetPlayersWidgets) (Class|GameplayStatics|GetPlayerControllerID PlayerController) _output_get)
    (UserInterface|Viewport|AddtoPlayerScreen (Variables|Default|GetWidget))
    (Utilities|FlowControl|Sequence
      (:then_0
        (Variables|/Script/Engine.PlayerController|SetbShowMouseCursor PlayerController true)
        (Input|SetInputModeGameandUI PlayerController (Variables|Default|GetWidget) "DoNotLock" true false)
        (Input|SetIgnoreLookInput PlayerController true)
        (Input|AddMappingContext (PlayerController|LocalPlayerSubsystems|GetEnhancedInputLocalPlayerSubsystem PlayerController) "/Game/Dynamic/Input/IMC_Menu.IMC_Menu" 0 "(bIgnoreAllPressedKeysUntilRelease=True,bForceImmediately=False,bNotifyUserSettings=False)"))
      (:then_1
        (EventDispatchers|BindEventtoOnClose (Variables|Default|GetWidget) (EventDispatchers|CreateEvent :!event CloseWidget))))
    (else
      (Utilities|FlowControl|DelayUntilNextTick)
      (goto _label))))

(event Custom|AddItemToMapMulticast
  (params (Key :type Integer%20%28by%20ref%29) (Value :type Shop%20Item%20Structure%20%28by%20ref%29))
  ;[0.01042 0.01042 0.01042] Muticasts
  (Utilities|Map|Add (Variables|Default|GetItems) Key Value))

(event Custom|UpdateItemStockMulticast
  (params (ItemId :type Integer%20%28by%20ref%29) (NewStock :type Integer))
  ;[0.01042 0.01042 0.01042] Muticasts
  (bind _values (Utilities|Map|Values (Variables|Default|GetPlayersWidgets)))
  (for _array_element _values
    (Default|UpdateItemStock _array_element ItemId NewStock)))

(event Custom|UpdateMoneyMulticast
  (params (InputPin :type Integer))
  ;[0.01042 0.01042 0.01042] Muticasts
  (Variables|Default|SetMoney InputPin)
  (bind _values (Utilities|Map|Values (Variables|Default|GetPlayersWidgets)))
  (for _array_element _values
    (Default|UpdateMoney _array_element InputPin)))

(event Custom|AddItemMulticast
  (params (Item :type Shop%20Item%20Structure))
  ;[0.01042 0.01042 0.01042] ShopInterface
  (CallFunction|AddItemInternal Item))

(event Custom|StartWaving
  ;[0.01042 0.01042 0.01042] Animation
  (bind _asabp_shop_keeper (Utilities|Casting|CastToABP_ShopKeeper (Components|SkeletalMesh|GetAnimInstance (Variables|Default|GetSkeletalMesh))))
  (Default|StartWaving _asabp_shop_keeper))

(event EventBuy
  (params (ItemId :type Integer) (Amount :type Integer) (Buyer :type Player%20Controller%20Object%20Reference))
  ;[0.01042 0.01042 0.01042] ShopInterface
  (Networking|SwitchHasAuthority
    (:Authority
      (Buy|BuyItemAuth ItemId Amount Buyer))))

(event EventInteract
  (params (Owner :type Pawn%20Object%20Reference))
  ;[0.01042 0.01042 0.01042] Interaction
  (if (Collision|IsOverlappingActor (Variables|Default|GetPlayerTrigger) Owner :!class /Script/Engine.PrimitiveComponent)
    (bind _asplayer_controller (Utilities|Casting|CastToPlayerController (Pawn|GetController Owner)))
    (Variables|Default|SetIsMoneyRecive false)
    (Networking|SwitchHasAuthority
      (:Authority
        (CallFunction|SetMoneyServer))
      (:Remote
        _))
    (if (Pawn|IsLocalPlayerController _asplayer_controller)
      (if (not (.ReturnValue (Utilities|Map|Find (Variables|Default|GetPlayersWidgets) (Class|GameplayStatics|GetPlayerControllerID _asplayer_controller))))
        (CallFunction|AddWidget _asplayer_controller)))))

(event EventBeginPlay
  ;[0.01042 0.01042 0.01042] Core
  (Utilities|FlowControl|Sequence
    (:then_0
      ;;[0.01042 0.01042 0.01042] Set Max Key
      (bind _keys (Utilities|Map|Keys (Variables|Default|GetItems)))
      (for _array_element _keys
        (if (> _array_element (Variables|Default|GetItemKeyCounter))
          (Variables|Default|SetItemKeyCounter _array_element))))
    (:then_1
      (Networking|SwitchHasAuthority
        (:Authority
          (EventDispatchers|BindEventtoOnResourceUpdated (Class|ShipResourcesSubsystem|GetMoneyManager (Subsystems|GetShipResourcesSubsystem)) (delegate Custom|UpdateMoney)))))
    (:then_2
      (if (Variables|Initialization|GetbActivateOnStart)
        (CallFunction|ActivateInternal)))))

(event EventAddItem
  (params (Item :type Shop%20Item%20Structure))
  ;[0.01042 0.01042 0.01042] ShopInterface
  (CallFunction|AddItemMulticast Item))

(event EventCloseWidget
  (params (PlayerIndex :type Integer))
  ;[0.01042 0.01042 0.01042] ShopInterface
  (Widget|RemoveWidget (Class|GameplayStatics|GetPlayerControllerfromID PlayerIndex)))

(fn ConstructionScript
  (EventDispatchers|BindEventtoOnTrigger (Variables|Default|GetBPC_Trigger_CharacterDoorActivation) (EventDispatchers|CreateEvent :!event Custom|StartWaving)))

(fn BuyItemAuth
  (params (ItemId :type Integer%20%28by%20ref%29) (AmountToBuy :type Integer) (Buyer :type Player%20Controller%20Object%20Reference))
  (bind _items (Variables|Default|GetItems))
  (bind (_value _returnvalue) (Utilities|Map|Find _items ItemId))
  (if (and _returnvalue (CallFunction|CanBuyItem _value AmountToBuy))
    (bind _output_get (LocalVariables|SetItemToBuy _value))
    (if (>= (Utilities|Struct|BreakShopItem _output_get) AmountToBuy)
      (bind _returnvalue_2 (Utilities|GetDataTableRow "/Game/Dynamic/Shop/DT_Items.DT_Items" (Utilities|Struct|BreakShopItem (LocalVariables|GetItemToBuy)))
        (:then
          (LocalVariables|SetItemInfo _returnvalue_2)
          (LocalVariables|SetAmountToCreate (* AmountToBuy (Utilities|Struct|BreakShopItem (LocalVariables|GetItemToBuy))))
          (Utilities|FlowControl|Sequence
            (:then_0
              (switch Utilities|FlowControl|Switch|SwitchonESpawnType (Utilities|Struct|BreakSpawner (Utilities|Struct|BreakInventoryItem (LocalVariables|GetItemInfo)))
                (:World
                  (bind _returnvalue_3 (Utilities|LoadClassAssetBlocking (.SpawnItemClass (Utilities|Struct|BreakSpawner (Utilities|Struct|BreakInventoryItem (LocalVariables|GetItemInfo))))))
                  (bind _asitem_base (Utilities|Casting|CastToItemBaseClass _returnvalue_3))
                  (Buy|SpawnItem _asitem_base (LocalVariables|GetAmountToCreate) (Transformation|GetActorLocation (Pawn|GetControlledPawn Buyer))))
                (:WeaponAmmo
                  (Buy|AddWeaponAmmo (.WeaponAmmoType (Utilities|Struct|BreakSpawner (Utilities|Struct|BreakInventoryItem (LocalVariables|GetItemInfo)))) (LocalVariables|GetAmountToCreate)))
                (:ToolAmmo
                  (Buy|AddToolAmmo (.ToolAmmoType (Utilities|Struct|BreakSpawner (Utilities|Struct|BreakInventoryItem (LocalVariables|GetItemInfo)))) (Math|Conversions|ToFloat(Integer) (LocalVariables|GetAmountToCreate))))
                (:Revive
                  (bind _asbp_first_person_game_mode (Utilities|Casting|CastToBP_FirstPersonGameMode (Game|GetGameMode)))
                  (Default|RevivePlayer _asbp_first_person_game_mode (Utilities|Struct|BreakSpawner (Utilities|Struct|BreakInventoryItem (LocalVariables|GetItemInfo))) (+ (Transformation|GetActorLocation) "0.000000,0.000000,50.000000")))))
            (:then_1
              (Utilities|FlowControl|Sequence
                (:then_0
                  (bind _output_get_2 (LocalVariables|SetAmountLeft (- (.AvailableAmount (Utilities|Struct|BreakShopItem (LocalVariables|GetItemToBuy))) AmountToBuy)))
                  (bind _structout (Utilities|Struct|SetmembersinShopItem (LocalVariables|GetItemToBuy) _output_get_2))
                  (CallFunction|AddItemtoMapMulticast ItemId _structout)
                  (CallFunction|UpdateItemStockMulticast ItemId (LocalVariables|GetAmountLeft)))
                (:then_1
                  (Class|ResourceManager|DecreaseResource (Class|ShipResourcesSubsystem|GetMoneyManager (Subsystems|GetShipResourcesSubsystem)) (* AmountToBuy (.Price (Utilities|Struct|BreakShopItem (LocalVariables|GetItemToBuy))))))))))))))

(fn SpawnItem
  (params (Item%20Class :type Actor%20Class%20Reference) (Amount :type Integer) (LocationOfBuyer :type Vector))
  (bind _returnvalue (Transformation|GetActorLocation))
  (for _index (range 0 (- Amount 1))
    (bind _returnvalue_2 (Game|SpawnActorfromClass Item%20Class (Math|Transform|MakeTransform (Math|Vector|MakeVectorNetQuantize (.x _returnvalue) (.y _returnvalue) (+ (.z _returnvalue) (.z (Variables|/Script/Engine.SceneComponent|GetRelativeLocation (Variables|Default|GetOriginPosition))))) "0, 0, 0" "1.000000,1.000000,1.000000") "Undefined" "MultiplyWithRoot" 0 0))
    (Class|BPIMoveable|ApplyImpulse(Message) _returnvalue_2 (* (Math|Vector|GetForwardVector (Math|Rotator|FindLookatRotation (Transformation|GetWorldLocation (Variables|Default|GetOriginPosition)) LocationOfBuyer)) (* (Math|Vector|Distance2D(Vector) (Transformation|GetWorldLocation (Variables|Default|GetOriginPosition)) LocationOfBuyer) (LocalVariables|GetImpulsePower))))))

(fn AddWeaponAmmo
  (params (WeaponAmmo :type EWeaponAmmoType%20Enum :default "Light") (Amount :type Integer))
  (bind _returnvalue (Subsystems|GetShipResourcesSubsystem))
  (bind _returnvalue_2 (Class|ShipResourcesSubsystem|GetWeaponAmmoManager _returnvalue WeaponAmmo))
  (Utilities|IsValid _returnvalue
    (:Is%20Valid
      (Utilities|IsValid _returnvalue_2
        (:Is%20Valid
          (Class|ResourceManager|AddResource _returnvalue_2 Amount))
        (:Is%20Not%20Valid
          (Development|PrintString "Ammo Manager Invalid"))))
    (:Is%20Not%20Valid
      (Development|PrintString "ShipSystem invalid"))))

(fn AddToolAmmo
  (params (ToolAmmo :type EToolAmmoType%20Enum :default "Welding") (Amount :type Float%20%28double-precision%29))
  (Class|FloatResourceManager|AddResource (Class|ShipResourcesSubsystem|GetToolAmmoManager (Subsystems|GetShipResourcesSubsystem) ToolAmmo) Amount))

(fn RemoveWidget
  (params (PlayerController :type Player%20Controller%20Object%20Reference))
  (bind _returnvalue (Class|GameplayStatics|GetPlayerControllerID PlayerController))
  (bind _playerswidgets (Variables|Default|GetPlayersWidgets))
  (bind (_value _returnvalue_2) (Utilities|Map|Find _playerswidgets _returnvalue))
  (Utilities|IsValid PlayerController
    (:Is%20Valid
      (if _returnvalue_2
        (Widget|RemovefromParent _value)
        (Utilities|Map|Remove (Variables|Default|GetPlayersWidgets) _returnvalue)
        (Variables|/Script/Engine.PlayerController|SetbShowMouseCursor PlayerController false)
        (Input|SetInputModeGameOnly PlayerController false)
        (Input|SetIgnoreLookInput PlayerController false)
        (Input|RemoveMappingContext (PlayerController|LocalPlayerSubsystems|GetEnhancedInputLocalPlayerSubsystem PlayerController) "/Game/Dynamic/Input/IMC_Menu.IMC_Menu" "(bIgnoreAllPressedKeysUntilRelease=True,bForceImmediately=False,bNotifyUserSettings=False)")))))

(fn GetItemCounterIncremented
  (bind _output_get (Variables|Default|SetItemKeyCounter (+ (Variables|Default|GetItemKeyCounter) 1)))
  (return _output_get))

(fn IncreaseItemStock
  (params (ItemKey :type Integer%20%28by%20ref%29) (AddAmount :type Integer))
  (bind _items (Variables|Default|GetItems))
  (bind (_value _returnvalue) (Utilities|Map|Find _items ItemKey))
  (if _returnvalue
    (bind _structout (Utilities|Struct|SetmembersinShopItem _value (+ (.AvailableAmount (Utilities|Struct|BreakShopItem _value)) AddAmount)))
    (Utilities|Map|Add (Variables|Default|GetItems) ItemKey _structout)
    (bind _values (Utilities|Map|Values (Variables|Default|GetPlayersWidgets)))
    (for _array_element _values
      (Default|UpdateItemStock _array_element ItemKey (Utilities|Struct|BreakShopItem _structout)))))

(fn CreateItem
  (params (Item :type Shop%20Item%20Structure))
  (bind _newitemkey (CallFunction|GetItemCounterIncremented))
  (Utilities|Map|Add (Variables|Default|GetItems) _newitemkey Item)
  (bind _values (Utilities|Map|Values (Variables|Default|GetPlayersWidgets)))
  (for _array_element _values
    (Default|AddItem _array_element _newitemkey Item)))

(fn AddItemInternal
  (params (Item :type Shop%20Item%20Structure))
  (bind (_infoname _price _availableamount _amountperitem) (Utilities|Struct|BreakShopItem Item))
  (bind _keys (Utilities|Map|Keys (Variables|Default|GetItems)))
  (bind _array_element (Utilities|Array|ForEachLoopwithBreak _keys :!label _label)
    (:LoopBody
      (if (Math|Boolean|ANDBoolean (== (.InfoName (Utilities|Struct|BreakShopItem (.Value (Utilities|Map|Find (Variables|Default|GetItems) _array_element)))) _infoname) (== (.Price (Utilities|Struct|BreakShopItem (.Value (Utilities|Map|Find (Variables|Default|GetItems) _array_element)))) _price) (== (.AmountPerItem (Utilities|Struct|BreakShopItem (.Value (Utilities|Map|Find (Variables|Default|GetItems) _array_element)))) _amountperitem))
        (CallFunction|IncreaseItemStock _array_element _availableamount)
        (LocalVariables|SetAdded true)
        (goto _label Break)))
    (:Completed
      (if (not (LocalVariables|GetAdded))
        (CallFunction|CreateItem Item)))))

(fn CanBuyItem
  (params (ShopItem :type Shop%20Item%20Structure%20%28by%20ref%29) (AmountToBuy :type Integer))
  (return (and (> AmountToBuy 0) (<= (* AmountToBuy (.Price (Utilities|Struct|BreakShopItem ShopItem))) (Variables|Default|GetMoney)))))

(fn ActivateInternal
  (Utilities|FlowControl|Sequence
    (:then_0
      (Rendering|SetActorHiddenInGame false))
    (:then_1
      (Collision|SetCollisionResponsetoChannel (Variables|Default|GetSkeletalMesh) "ECC_GameTraceChannel3" "ECR_Block"))))

(fn Activate
  (params (Round :type Integer))
  (bind _rounditems (Variables|Default|GetRoundItems))
  (bind (_value _returnvalue) (Utilities|Map|Find _rounditems Round))
  (Utilities|FlowControl|Sequence
    (:then_0
      (if _returnvalue
        (bind _count (Class|BPIMultiplayer|GetMultiplayerPlayerCount(Message) (Game|GetGameInstance)))
        (bind _output_get (Variables|Default|SetPlayerCount _count))
        (if (> _output_get 1)
          (for _array_element (Utilities|Struct|BreakS_RoundShopItems _value)
            (bind _shopitem (Utilities|GetRoundItemAmount _array_element (Variables|Default|GetPlayerCount)))
            (CallFunction|AddItem _shopitem))
          (else
            (for _array_element_2 (Utilities|Struct|BreakS_RoundShopItems _value)
              (CallFunction|AddItem (.Item (Utilities|Struct|BreakRoundShopItem _array_element_2))))))))
    (:then_1
      (CallFunction|ActivateInternal))))

(fn Deactivate
  (Utilities|FlowControl|Sequence
    (:then_0
      (bind _values (Utilities|Map|Values (Variables|Default|GetPlayersWidgets)))
      (for _array_element _values
        (Widget|RemoveWidget (Widget|GetOwningPlayer _array_element))))
    (:then_1
      (Rendering|SetActorHiddenInGame true))
    (:then_2
      (Collision|SetCollisionResponsetoChannel (Variables|Default|GetSkeletalMesh) "ECC_GameTraceChannel3" "ECR_Ignore"))))

(fn GetInreactionWidgetLocation
  (return (Transformation|GetWorldLocation (Variables|Default|GetOriginPosition))))