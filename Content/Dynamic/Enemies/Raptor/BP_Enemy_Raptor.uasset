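; Raptor enemy Blueprint with a poison breath attack, flagged to use big doors only.
; An attack notify makes the server spawn a delayed poison cloud ahead of the mesh, passing it the current attack's damage.
; StartBreath and StopBreath toggle the breath effect and a Tick gate that drives its intensity from the PoisonIntensity animation curve, syncing the visual to the animation.
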(event Custom|AttackNotifyBegin
  (params (NotifyName :type Name))
  (switch name NotifyName
    (:Poison
      ;[0.01042 0.01042 0.01042] Posion Attack
      (Networking|SwitchHasAuthority
        (:Authority
          (Utilities|FlowControl|Delay (Variables|Default|GetPoisonDelay))
          (Game|SpawnActorfromClass "/Game/Dynamic/Combat/Abilities/PosionCloud/BP_PoisonCloud.BP_PoisonCloud_C" (Math|Transform|MakeTransform (+ (Transformation|GetWorldLocation (Variables|Character|GetMesh)) (* (Transformation|GetActorForwardVector) 4e+02) "0.000000,0.000000,20.000000") "0, 0, 0" "1.000000,1.000000,1.000000") "Undefined" "MultiplyWithRoot" 0 (.DamageAmount (Utilities|Struct|BreakS_DamageInfo (CallFunction|GetCurrentAttackDamageInfo))) 1e+01 3.7 self))))))

(event EventBeginPlay
  (|CallParentFunction) ; This node is disabled and will not be called.\nDrag off pins to build functionality.
)

(event Collision|EventActorBeginOverlap
  (params (OtherActor :type Actor%20Object%20Reference)))

(event EventTick
  (params (DeltaSeconds :type Float%20%28single-precision%29))
  (|CallParentFunction DeltaSeconds)
  ;[0.01042 0.01042 0.01042] Breath Control
  (Utilities|FlowControl|Gate true
    (:Exit
      (Niagara|SetNiagaraVariable(Float) (Variables|Default|GetNS_PosionBreath) "PoisonIntensity" (Animation|Curves|GetCurveValue (Components|SkeletalMesh|GetAnimInstance (Variables|Character|GetMesh)) "PoisonIntensity")))))

(event EventStartBreath
  ;[0.01042 0.01042 0.01042] Breath Control
  (Components|Activation|Activate (Variables|Default|GetNS_PosionBreath) true)
  (Utilities|FlowControl|Gate true) ; enters at Open
)

(event EventStopBreath
  ;[0.01042 0.01042 0.01042] Breath Control
  (Components|Activation|Deactivate (Variables|Default|GetNS_PosionBreath))
  (Utilities|FlowControl|Gate true) ; enters at Close
)

(fn ConstructionScript
  (|CallParentFunction)
  (EventDispatchers|BindEventtoOnAttackNotifyBegin (EventDispatchers|CreateEvent :!event Custom|AttackNotifyBegin)))

(fn IsUsingBigDoorsOnly
  (return true))