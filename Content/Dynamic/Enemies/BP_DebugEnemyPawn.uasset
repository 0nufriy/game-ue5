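; Debug pawn in the enemies folder that provides developer shortcuts for inspecting gameplay.
; On BeginPlay it runs a console command that turns on AI path drawing.
; X and Z each use a FlipFlop to toggle global time dilation between normal speed and fast-forward or slow motion, respectively.
; C runs the console command that shows collision.
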(event EventBeginPlay
  (Development|ExecuteConsoleCommand "ai.debug.DrawPaths 1" 0))

(event Collision|EventActorBeginOverlap
  (params (OtherActor :type Actor%20Object%20Reference)))

(event EventTick
  (params (DeltaSeconds :type Float%20%28single-precision%29)))

(event Input|KeyboardEvents|DebugKeyX
  (params (Key :type Key%20Structure :default "None") (ActionValue :type Input%20Action%20Value%20Structure))
  (:Pressed
    (bind _isa (Utilities|FlowControl|FlipFlop)
      (:A
        _)
      (:B
        _))
    (Utilities|Time|SetGlobalTimeDilation (Math|Float|SelectFloat 5.0 1.0 _isa))))

(event Input|KeyboardEvents|DebugKeyZ
  (params (Key :type Key%20Structure :default "None") (ActionValue :type Input%20Action%20Value%20Structure))
  (:Pressed
    (bind _isa (Utilities|FlowControl|FlipFlop)
      (:A
        _)
      (:B
        _))
    (Utilities|Time|SetGlobalTimeDilation (Math|Float|SelectFloat 0.25 1.0 _isa))))

(event Input|KeyboardEvents|DebugKeyC
  (params (Key :type Key%20Structure :default "None") (ActionValue :type Input%20Action%20Value%20Structure))
  (:Pressed
    (Development|ExecuteConsoleCommand "show COLLISION" 0)))

(fn ConstructionScript)