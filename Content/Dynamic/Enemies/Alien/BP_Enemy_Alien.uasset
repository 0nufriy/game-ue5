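; Alien enemy Blueprint with a ground-smash area attack and sight taken from its head socket.
; An attack notify makes the server spawn a blast AOE at the main-hand socket, covering the smash radius.
; Each overlapped actor gets a multicast knockback with fixed lift and sideways push easing to half strength at the edge.
; Only hostile targets also take physical damage, without stun.
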(event Custom|AttackNotifyBegin
  (params (NotifyName :type Name))
  (Networking|SwitchHasAuthority
    (:Authority
      (switch name NotifyName
        (:Smash
          (bind _output_get (Variables|Attacks|Smash|SetSmashHitLocation (Transformation|GetSocketLocation (Variables|Character|GetMesh) "MainHandEnd_Socket")))
          (bind _returnvalue (Game|SpawnActorfromClass "/Game/Dynamic/Combat/Attacks/AOE/BP_AOE_BlastBase.BP_AOE_BlastBase_C" (Math|Transform|MakeTransform _output_get "0, 0, 0" "1.000000,1.000000,1.000000") "Undefined" "MultiplyWithRoot" 0 true false false (Utilities|Array|MakeArray "ObjectTypeQuery3" "ObjectTypeQuery2") 0))
          (Variables|/Game/Dynamic/Combat/Attacks/AOE/BP_AOE_Base.BP_AOE_Base_C|SetRadius _returnvalue (Variables|Attacks|Smash|GetSmashRadius))
          (EventDispatchers|BindEventtoOnAOEOverlapActor _returnvalue (EventDispatchers|CreateEvent :!event OnSmashHit))
          (Default|Trigger _returnvalue))))))

(event Custom|ApplayImpilseMulticast
  (params (Target :type Object%20Object%20Reference) (Impulse :type Vector))
  (Class|BPIMoveable|ApplyImpulse(Message) Target Impulse))

(fn ConstructionScript
  (|CallParentFunction)
  (EventDispatchers|BindEventtoOnAttackNotifyBegin (EventDispatchers|CreateEvent :!event Custom|AttackNotifyBegin)))

(fn OnSmashHit
  (params (Target :type Actor%20Object%20Reference))
  (bind _smashradius (Variables|Attacks|Smash|GetSmashRadius))
  (bind _smashhitlocation (Variables|Attacks|Smash|GetSmashHitLocation))
  (bind _smashsideknockbackpower (Variables|Attacks|Smash|GetSmashSideKnockbackPower))
  (bind _returnvalue (Transformation|GetActorLocation Target))
  (bind _returnvalue_2 (* _smashsideknockbackpower 0.5))
  (bind _returnvalue_3 (Math|Rotator|FindLookatRotation _smashhitlocation _returnvalue))
  (bind _returnvalue_4 (Math|Vector|Distance(Vector) _returnvalue _smashhitlocation))
  (bind _returnvalue_5 (Math|Vector|GetForwardVector _returnvalue_3))
  (bind _returnvalue_6 (/ _returnvalue_4 _smashradius))
  (bind _returnvalue_7 (Math|Float|Clamp(Float) _returnvalue_6))
  (bind _result (Math|Interpolation|Ease "EaseIn" _returnvalue_7 _smashsideknockbackpower _returnvalue_2 4.0))
  (bind _returnvalue_8 (* (Math|Vector2D|MakeVector2D (.x _returnvalue_5) (.y _returnvalue_5)) _result))
  (Networking|SwitchHasAuthority
    (:Authority
      (Utilities|FlowControl|Sequence
        (:then_0
          (if (Default|IsHostileTarget (Variables|Default|GetAIController) Target)
            (CallFunction|ApplayAttackMulticast Target (Utilities|Struct|MakeS_DamageInfo 5.0 "/Game/Dynamic/Blueprints/DamageTypes/BP_PhysicalDamage.BP_PhysicalDamage_C" false))))
        (:then_1
          (CallFunction|ApplayImpilseMulticast Target (Math|Vector|MakeVector (.x _returnvalue_8) (.y _returnvalue_8) (Variables|Attacks|Smash|GetSmashUpKnockbackPower))))))))

(fn GetSightLocation
  (return (Transformation|GetSocketLocation (Variables|Character|GetMesh) "Head")))