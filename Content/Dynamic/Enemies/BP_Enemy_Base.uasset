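; Base enemy character Blueprint that handles movement states, health, death and data-table-driven melee attacks, driven by its AI controller.
; Attack montages and per-hit damage come from AttacksDT, with trace component hits applying damage through an authority-checked multicast.
; Attacks reserve tokens from the target and return them on attack end or death.
; Abort requests wait until the attack is interruptible, and collision traces pause target focus.
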(event OnAllTracesEnd(AttackCollisionTrace)
  ;[1 1 1] Start/End events of Attack Collision Trace Component
  (Networking|SwitchHasAuthority
    (:Authority
      (bind _aicontroller (Variables|AI|GetAIController)
        (:then
          (Default|FocusonAttackTarget _aicontroller))
        (:else)))))

(event OnFirstTraceStart(AttackCollisionTrace)
  ;[1 1 1] Start/End events of Attack Collision Trace Component
  (Networking|SwitchHasAuthority
    (:Authority
      (AI|ClearFocus (AI|GetAIController self)))))

(event OnHit(AttackCollisionTrace)
  (params (HitResult :type Hit%20Result%20Structure) (AttackIndex :type Integer))
  ;[1 1 1] On Hit by Collision Trace Component
  (CallFunction|ApplyDamagetoHittedActor HitResult AttackIndex))

(event OnDeath(HealthSystem)
  ;[1 1 1] Death
  (Utilities|FlowControl|Sequence
    (:then_0
      (bind _output_get (Variables|Default|SetCurrentMontage (Variables|Montages|GetDeathMontage)))
      (Animation|Montage|PlayMontage (Variables|Character|GetMesh) _output_get
        (:then
          (Utilities|Time|SetTimerbyEvent (delegate Custom|DestroyActor) (Variables|Death|GetSelfDestroyTime)))
        (:OnCompleted
          (Collision|SetCollisionResponsetoChannel (Variables|Default|GetCapsuleComponent) "ECC_Pawn" "ECR_Ignore" :!label _label)
          (Variables|Default|SetCurrentMontage 0))
        (:OnInterrupted
          (goto _label))))
    (:then_1
      (bind _aicontroller (Variables|AI|GetAIController)
        (:then
          (Default|TrySetState _aicontroller "NewEnumerator5"))
        (:else)))
    (:then_2
      (Default|ReturnAllTokens (Variables|Default|GetBPC_AttackTokenTheft)))))

(event Custom|InterruptAttack
  ;[1 1 1] Try Abort Attack
  (Utilities|FlowControl|Sequence
    (:then_0
      (bind _currentmontage (Variables|Default|GetCurrentMontage)
        (:then
          (Animation|StopAnimMontage _currentmontage))
        (:else)))
    (:then_1
      (bind _aicontroller (Variables|AI|GetAIController)
        (:then
          (Default|OnStateAborted _aicontroller))
        (:else)))
    (:then_2
      (Variables|Default|SetShouldInterruptAttack false))))

(event Custom|DestroyActor
  ;[1 1 1] Death
  (Actor|DestroyActor))

(event Custom|AttackMulticast
  (params (MontageToPlay :type Anim%20Montage%20Object%20Reference))
  ;[1 1 1] Attack
  (bind _notifyname (Animation|Montage|PlayMontage (Variables|Character|GetMesh) MontageToPlay)
    (:then
      (bind _aicontroller (Variables|AI|GetAIController)
        (:then
          (Default|StartFollowAttackTarget _aicontroller))
        (:else)))
    (:OnCompleted
      (Variables|Default|SetCurrentMontage 0 :!label _label)
      (Default|SetIsAttacking (Variables|Default|GetCombat%20System) false)
      (Default|CallOnAttackEnd)
      (Utilities|FlowControl|Sequence
        (:then_0
          (Default|ReturnAllTokens (Variables|Default|GetBPC_AttackTokenTheft)))
        (:then_1
          (bind _aicontroller_2 (Variables|AI|GetAIController)
            (:then
              (Default|StopFollowAttackTarget _aicontroller_2))
            (:else)))
        (:then_2
          (CallFunction|SetCanInterruptAttack true))))
    (:OnInterrupted
      (goto _label))
    (:OnNotifyBegin
      (Default|CallOnAttackNotifyBegin _notifyname))))

(event Custom|ApplayAttackMulticast
  (params (Target :type Object%20Object%20Reference) (DamageInfo :type S%20Damage%20Info%20Structure))
  ;[1 1 1] Attack
  (Class|BPIDamagable|TakeDamage(Message) Target DamageInfo))

(event Custom|OnDeathAnimationEnd
  ;[1 1 1] Death
  (Collision|SetCollisionResponsetoChannel (Variables|Default|GetCapsuleComponent) "ECC_Pawn" "ECR_Ignore")
  (Variables|Default|SetCurrentMontage 0))

(event Custom|CallStateChangeMulticast
  (params (NewMovementState :type E_AIMovementSpeed%20Enum :default "NewEnumerator0"))
  ;[1 1 1] On Set Movement Speed
  (Default|CallOnMovementStateChange NewMovementState))

(event Custom|PerformAttack
  (params (AttackName :type Name))
  (bind _returnvalue (Utilities|String|ToString(Name) AttackName))
  ;[1 1 1] Attack
  (bind _returnvalue_2 (Utilities|GetDataTableRow (Variables|Default|GetAttacksDT) AttackName)
    (:then
      (Utilities|IsValid (.Animation (Utilities|Struct|BreakS_AIAttackInfo _returnvalue_2))
        (:Is%20Valid
          (Animation|StopAnimMontage (Variables|Default|GetCurrentMontage))
          (bind _output_get (Variables|Default|SetCurrentMontage (.Animation (Utilities|Struct|BreakS_AIAttackInfo _returnvalue_2))))
          (Variables|Default|SetCurrent%20Attack AttackName)
          (Default|SetIsAttacking (Variables|Default|GetCombat%20System) true)
          (CallFunction|SetCanInterruptAttack false)
          (CallFunction|AttackMulticast _output_get))
        (:Is%20Not%20Valid
          (Utilities|String|LogString (Utilities|String|Append "Warning: " "Missing attack  montage for " _returnvalue)))))
    (:RowNotFound
      (Utilities|String|LogString (Utilities|String|Append "Warning: " "Missing AttackInfo for attack " _returnvalue)))))

(event EventSetMovementSpeed
  (params (NewMovementState :type E_AIMovementSpeed%20Enum :default "NewEnumerator0"))
  ;[1 1 1] On Set Movement Speed
  (bind _output_get (Variables|Movement|SetMovement%20State NewMovementState))
  (CallFunction|CallStateChangeMulticast _output_get)
  (Variables|/Script/Engine.CharacterMovementComponent|SetMaxWalkSpeed (Variables|Character|GetCharacterMovement) (CallFunction|GetSpeedbyMovementState _output_get)))

(event EventBeginPlay
  ;[1 1 1] Begin Play
  (bind _asbp_aicontroller_enemy_base (Utilities|Casting|CastToBP_AIController_Enemy_Base (AI|GetAIController self)))
  (Variables|AI|SetAIController _asbp_aicontroller_enemy_base))

(event Collision|EventHit
  (params (MyComp :type Primitive%20Component%20Object%20Reference) (Other :type Actor%20Object%20Reference) (OtherComp :type Primitive%20Component%20Object%20Reference) (bSelfMoved :type Boolean) (HitLocation :type Vector :default "0, 0, 0") (HitNormal :type Vector :default "0, 0, 0") (NormalImpulse :type Vector :default "0, 0, 0") (Hit :type Hit%20Result%20Structure%20%28by%20ref%29))
  ;[0.01042 0.01042 0.01042] Displace enemy on hit
  (if (not (Math|Vector|VectorIsZero (Transformation|GetVelocity Other)))
    (Physics|AddForce (Variables|Character|GetCharacterMovement) (* (Transformation|GetActorForwardVector Other) 1e+06))))

(event EventSetMovementEnabled
  (params (Enabled :type Boolean))
  ;[1 1 1] Continuously Follow Attack Target
  (if Enabled
    (bind _aicontroller (Variables|AI|GetAIController)
      (:then
        (Default|StartFollowAttackTarget _aicontroller))
      (:else))
    (else
      (bind _aicontroller_2 (Variables|AI|GetAIController)
        (:then
          (Default|StopFollowAttackTarget _aicontroller_2))
        (:else)))))

(event EventSetCanInterruptAttack
  (params (Value :type Boolean))
  ;[1 1 1] Try Abort Attack
  (bind _output_get (Variables|Default|SetbCanBeInterrupted Value))
  (if (and _output_get (Variables|Default|GetShouldInterruptAttack))
    (CallFunction|InterruptAttack)))

(fn ConstructionScript
  (bind _capsulecomponent (Variables|Default|GetCapsuleComponent))
  (bind _stats_system (Variables|Default|GetStats%20System))
  (bind _returnvalue (Components|Capsule|GetScaledCapsuleRadius _capsulecomponent))
  (|CallParentFunction)
  (Variables|/Game/Dynamic/Blueprints/Components/StatsSystemComponent/Enemy/BPC_Enemy_StatsSystem.BPC_Enemy_StatsSystem_C|SetAttackRadius _stats_system _returnvalue)
  (Variables|/Game/Dynamic/Blueprints/Components/StatsSystemComponent/Enemy/BPC_Enemy_StatsSystem.BPC_Enemy_StatsSystem_C|SetIdealRange _stats_system _returnvalue))

(fn GetCurrentAttackDamageInfo
  (params (AttackIndex :type Integer))
  (bind _returnvalue (Utilities|GetDataTableRow (Variables|Default|GetAttacksDT) (Variables|Default|GetCurrent%20Attack))
    (:then
      (if (< AttackIndex (Utilities|Array|Length (.Damages (Utilities|Struct|BreakS_AIAttackInfo _returnvalue))))
        (return (Utilities|Array|Get(acopy) (.Damages (Utilities|Struct|BreakS_AIAttackInfo _returnvalue)) AttackIndex))
        (else
          (Development|PrintString (Utilities|String|Append "Warning: " "Attack damage not found for attack with index " (Utilities|String|ToString(Integer) AttackIndex))))))))

(fn GetMovementState
  (return (Variables|Movement|GetMovement%20State)))

(fn GetSpeedbyMovementState
  (params (MovementState :type E_AIMovementSpeed%20Enum :default "NewEnumerator0"))
  (return (Utilities|Select :Index MovementState :NewEnumerator0 0.0 :NewEnumerator1 (Variables|/Game/Dynamic/Blueprints/Components/StatsSystemComponent/Enemy/BPC_Enemy_StatsSystem.BPC_Enemy_StatsSystem_C|GetWalkSpeed (Variables|Default|GetStats%20System)) :NewEnumerator3 (Variables|/Game/Dynamic/Blueprints/Components/StatsSystemComponent/Enemy/BPC_Enemy_StatsSystem.BPC_Enemy_StatsSystem_C|GetJoggingSpeed (Variables|Default|GetStats%20System)) :NewEnumerator2 (Variables|/Game/Dynamic/Blueprints/Components/StatsSystemComponent/Enemy/BPC_Enemy_StatsSystem.BPC_Enemy_StatsSystem_C|GetRunningSpeed (Variables|Default|GetStats%20System)))))

(fn GetAttackTokensCost
  (params (Attack :type Name))
  (bind _returnvalue (Utilities|GetDataTableRow (Variables|Default|GetAttacksDT) Attack)
    (:then
      (return true (.AttackTokenCost (Utilities|Struct|BreakS_AIAttackInfo _returnvalue))))
    (:RowNotFound
      (return false 0))))

(fn ApplyDamagetoHittedActor
  (params (Hit :type Hit%20Result%20Structure%20%28by%20ref%29) (AttackIndex :type Integer))
  (Networking|SwitchHasAuthority
    (:Authority
      (CallFunction|ApplayAttackMulticast (.HitActor (Collision|BreakHitResult Hit)) (CallFunction|GetCurrentAttackDamageInfo AttackIndex)))))

(fn GetCanbeInterrupted
  (return (Variables|Default|GetbCanBeInterrupted)))

(fn GetCurrentHealth
  (return (Default|GetCurrentHealth (Variables|Default|GetHealth%20System))))

(fn GetMaxHealth
  (return (Default|GetMaxHealth (Variables|Default|GetHealth%20System))))

(fn GetSightLocation
  (return "0, 0, 0"))

(fn GetSocketsOwningComponent
  (return (Variables|Character|GetMesh)))

(fn Heal
  (params (HealAmount :type Float%20%28double-precision%29))
  (bind _newhealth (Default|Heal (Variables|Default|GetHealth%20System) HealAmount))
  (return _newhealth))

(fn IsDead
  (return (Default|IsDead (Variables|Default|GetHealth%20System))))

(fn IsUsingBigDoorsOnly
  (return false))

(fn ReserveAttackTokens
  (params (Amount :type Integer))
  (return false))

(fn TakeDamage
  (params (DamageInfo :type S%20Damage%20Info%20Structure))
  (bind _currenthealth (Default|TakeDamage (Variables|Default|GetHealth%20System) DamageInfo))
  (return _currenthealth))

(fn TryAbortAttack
  (Utilities|FlowControl|Sequence
    (:then_0
      (if (Variables|Default|GetbCanBeInterrupted)
        (if (Default|IsAttacking (Variables|Default|GetCombat%20System))
          (bind _currentmontage (Variables|Default|GetCurrentMontage)
            (:then
              (Animation|StopAnimMontage _currentmontage))
            (:else)))
        (else
          (Variables|Default|SetShouldInterruptAttack true))))
    (:then_1
      (return (Variables|Default|GetbCanBeInterrupted)))))

(fn TryPrepareAttack
  (params (AttackTarget :type Actor%20Object%20Reference) (AttackName :type Name :default "None"))
  (bind (_attackexist _attacktokencost) (CallFunction|GetAttackTokensCost AttackName))
  (if _attackexist
    (if (> _attacktokencost 0)
      (bind _success (Class|BPIDamagable|ReserveAttackTokens(Message) AttackTarget _attacktokencost))
      (if _success
        (Default|ReserveTokens (Variables|Default|GetBPC_AttackTokenTheft) AttackTarget _attacktokencost)
        (return true)
        (else
          (return false)))
      (else
        (return true)))
    (else
      (return false))))