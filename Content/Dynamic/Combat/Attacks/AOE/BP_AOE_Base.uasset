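; Base area-of-effect attack actor that finds actors within a radius of its location and broadcasts each one.
; Trigger runs on BeginPlay when flagged or can be called separately, and performs a single sphere overlap with optional debug drawing.
; The query defaults to Pawns when no object types are set, can ignore the instigator, and calls the OnAOEOverlapActor dispatcher per hit, leaving the effect to listeners.
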(event Custom|SpawnAOE
  (bind _overlapobject_types (Variables|Default|GetOverlapObject%20Types))
  (if (Variables|Default|GetDrawDebugSphere)
    (Rendering|Debug|DrawDebugSphere (Transformation|GetActorLocation) (Variables|Default|GetRadius) 12 "(R=0.000000,G=0.040111,B=1.000000,A=1.000000)" 3.0 1.0))
  (bind _outactors (Collision|SphereOverlapActors (Transformation|GetActorLocation) (Variables|Default|GetRadius) (select (Utilities|Array|IsNotEmpty _overlapobject_types) _overlapobject_types (Utilities|Array|MakeArray "ObjectTypeQuery3")) 0 (select (Variables|Default|GetIgnoreInstigator) (Utilities|Array|MakeArray (Game|GetInstigator)) 0)))
  (for _array_element _outactors
    (Default|CallOnAOEOverlapActor _array_element)))

(event Custom|Trigger
  (CallFunction|SpawnAOE))

(event EventBeginPlay
  (if (Variables|Default|GetTriggerOnBegin)
    (CallFunction|Trigger)))

(fn ConstructionScript)