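; Base Blueprint for blast-style area-of-effect combat attacks, adding one-shot visual and audio feedback to the parent's Trigger logic.
; On Trigger it calls the parent, spawns BlastEffect attached to the root and plays BlastSound at world origin rather than the actor's location.
; The actor destroys itself when the particle system finishes, or during effect spawning if no valid effect is set.
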(event Custom|OnSystemFinished_Event
  (params (PSystem :type Particle%20System%20Component%20Object%20Reference))
  (Actor|DestroyActor))

(event Custom|SpawnBlastEffect
  (bind _blasteffect (Variables|Default|GetBlastEffect)
    (:then
      (bind _returnvalue (Effects|SpawnEmitterAttached _blasteffect (Variables|Default|GetDefaultSceneRoot) "None"))
      (EventDispatchers|AssignOnSystemFinished _returnvalue (delegate Custom|OnSystemFinished_Event)))
    (:else
      (Actor|DestroyActor))))

(event Custom|PlayBlastSound
  (Audio|PlaySoundatLocation (Variables|Default|GetBlastSound) "0, 0, 0" "0, 0, 0" 1.0 1.0 0.0 0 0 0 0))

(event EventTrigger
  (|CallParentFunction)
  (CallFunction|SpawnBlastEffect)
  (CallFunction|PlayBlastSound))

(fn ConstructionScript
  (|CallParentFunction))