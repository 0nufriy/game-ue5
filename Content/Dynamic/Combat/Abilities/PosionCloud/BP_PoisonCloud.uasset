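; Poison cloud ability actor that deals periodic, non-stunning physical damage to players inside a spreading area.
; On authority, a timer widens the Cylinder collision over the spread duration, and its overlaps track actors tagged as damageable players.
; A looping timer damages tracked actors through the TakeDamage message.
; The construction script passes durations to the VFX and sets a lifespan that outlasts the collision, which is destroyed first.
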(event OnComponentBeginOverlap(Cylinder)
  (params (OverlappedComponent :type Primitive%20Component%20Object%20Reference) (OtherActor :type Actor%20Object%20Reference) (OtherComp :type Primitive%20Component%20Object%20Reference) (OtherBodyIndex :type Integer) (bFromSweep :type Boolean) (SweepResult :type Hit%20Result%20Structure%20%28by%20ref%29))
  ;[0.01042 0.01042 0.01042] Collision
  (Networking|SwitchHasAuthority
    (:Authority
      (bind _returnvalue (GameplayTags|HasMatchingGameplayTag(Message) OtherActor "(TagName=\"Damageable.Character.Player\")"))
      (if _returnvalue
        (Utilities|Array|Add (Variables|Default|GetActorsToHit) OtherActor)))))

(event OnComponentEndOverlap(Cylinder)
  (params (OverlappedComponent :type Primitive%20Component%20Object%20Reference) (OtherActor :type Actor%20Object%20Reference) (OtherComp :type Primitive%20Component%20Object%20Reference) (OtherBodyIndex :type Integer))
  ;[0.01042 0.01042 0.01042] Collision
  (Networking|SwitchHasAuthority
    (:Authority
      (Utilities|Array|RemoveItem (Variables|Default|GetActorsToHit) OtherActor))))

(event Custom|ApplyDamage
  ;[0.01042 0.01042 0.01042] Apply Damage
  (CallFunction|ApplayDamageMulticast (Variables|Default|GetActorsToHit) (Variables|Default|GetDamage%20Amount)))

(event Custom|ApplayDamageMulticast
  (params (ActorsTo%20hit :type Array%20of%20Actor%20Object%20References) (DamageAmount :type Float%20%28double-precision%29))
  (for _array_element ActorsTo%20hit
    (Class|BPIDamagable|TakeDamage(Message) _array_element (Utilities|Struct|MakeS_DamageInfo DamageAmount "/Game/Dynamic/Blueprints/DamageTypes/BP_PhysicalDamage.BP_PhysicalDamage_C" false))))

(event Custom|OnDestroyed_Event
  (params (DestroyedActor :type Actor%20Object%20Reference))
  ;[0.01042 0.01042 0.01042] On Destroy
  (Utilities|Time|ClearandInvalidateTimerbyHandle (Variables|Default|GetCollisionScaleTimer))
  (Utilities|Time|ClearandInvalidateTimerbyHandle (Variables|Default|GetDamageTimer)))

(event EventBeginPlay
  (Networking|SwitchHasAuthority
    (:Authority
      (bind _returnvalue (Utilities|Time|SetTimerbyEvent (EventDispatchers|CreateEvent :!event Custom|ApplyDamage) (Variables|Default|GetDamageDelay) true))
      (Variables|Default|SetDamageTimer _returnvalue)
      (EventDispatchers|BindEventtoOnDestroyed (EventDispatchers|CreateEvent :!event Custom|OnDestroyed_Event))
      (bind _returnvalue_2 (Utilities|Time|SetTimerbyFunctionName 0 "ScaleCollision" 0.1 true))
      (Variables|Default|SetCollisionScaleTimer _returnvalue_2)
      ;[0.01042 0.01042 0.01042] Kill Collision after Delay
      (Utilities|FlowControl|Delay (+ (Variables|Default|GetCloudDuration) (Variables|Default|GetSpreadDuration)))
      (Components|DestroyComponent (Variables|Default|GetCylinder)))))

(fn ConstructionScript
  (bind _cloudvfx (Variables|Default|GetCloudVFX))
  (|CallParentFunction)
  (Effects|Components|ParticleSystem|SetFloatParameter _cloudvfx "CloudDuration" (Variables|Default|GetCloudDuration))
  (Effects|Components|ParticleSystem|SetFloatParameter _cloudvfx "SpreadDuration" (Variables|Default|GetSpreadDuration))
  (Actor|SetLifeSpan (+ (Variables|Default|GetCloudDuration) (Variables|Default|GetSpreadDuration) 3.0)))

(fn ScaleCollision
  (bind _cylinder (Variables|Default|GetCylinder))
  (bind _output_get (LocalVariables|SetNormalizedSize (Math|Float|Clamp(Float) (/ (Actor|GetGameTimeSinceCreation) (Variables|Default|GetSpreadDuration)))))
  (Transformation|SetWorldScale3D _cylinder (Math|Vector|MakeVector (Math|Float|Lerp 0.0 4.1 _output_get) (Math|Float|Lerp 0.0 4.1 _output_get) (.z (Transformation|GetWorldScale _cylinder))))
  (if (== (LocalVariables|GetNormalizedSize) 1.0)
    (Utilities|Time|ClearandInvalidateTimerbyHandle (Variables|Default|GetCollisionScaleTimer))))