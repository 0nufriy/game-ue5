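; BP_LocalSettingsSave holds local input settings for mouse sensitivity and separate gamepad X and Y sensitivities, with getters for each device.
; UpdateSettings compares incoming values to stored ones, assigns them, then fires the mouse or gamepad change dispatcher only if that device's values differed.
; A reused Dispatch flag carries each comparison past the assignment, so listeners are notified after the new value is stored.
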(fn UpdateSettings
  (params (MouseSensitivity :type Float%20%28double-precision%29) (GamepadXSensitivity :type Float%20%28double-precision%29) (GamepadYSensitivity :type Float%20%28double-precision%29))
  (Utilities|FlowControl|Sequence
    (:then_0
      (if (!= (Variables|Default|GetMouseSensitivity) MouseSensitivity)
        (LocalVariables|SetDispatch true)))
    (:then_1
      (Variables|Default|SetMouseSensitivity MouseSensitivity)
      (Utilities|FlowControl|Sequence
        (:then_0
          (if (LocalVariables|GetDispatch)
            (Default|CallOnMouseSensitivityChanged (Variables|Default|GetMouseSensitivity))
            (LocalVariables|SetDispatch false)))
        (:then_1
          (if (or (!= (Variables|Default|GetGamepadXSensitivity) GamepadXSensitivity) (!= (Variables|Default|GetGamepadYSensitivity) GamepadYSensitivity))
            (LocalVariables|SetDispatch true)))
        (:then_2
          (Variables|Default|SetGamepadXSensitivity GamepadXSensitivity)
          (Variables|Default|SetGamepadYSensitivity GamepadYSensitivity)
          (Utilities|FlowControl|Sequence
            (:then_0
              (if (LocalVariables|GetDispatch)
                (Default|CallOnGamepadSensitivityChanged (Variables|Default|GetGamepadXSensitivity) (Variables|Default|GetGamepadYSensitivity))
                (LocalVariables|SetDispatch false)))))))))

(fn GetMouseSensitivity
  (return (Variables|Default|GetMouseSensitivity)))

(fn GetGamepadSensitivity
  (return (Variables|Default|GetGamepadXSensitivity) (Variables|Default|GetGamepadYSensitivity)))