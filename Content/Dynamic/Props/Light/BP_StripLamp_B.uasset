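; BP_StripLamp_B is a strip lamp prop that extends a parent light Blueprint with a rect light and a glowing mesh.
; On BeginPlay it sets the RectLight as the parent's light component and puts a dynamic material instance on the mesh's second material slot.
; LightOn and LightOff call the parent logic, then set that material's Intensity parameter so the emissive surface matches the light state.
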(event EventBeginPlay
  (bind _staticmesh (Variables|Default|GetStaticMesh))
  (Variables|Default|SetLightComponent (Variables|Default|GetRectLight))
  (|CallParentFunction)
  (bind _returnvalue (Rendering|Material|CreateDynamicMaterialInstance _staticmesh 1 (Rendering|Material|GetMaterial _staticmesh 1) "None" :!class /Script/Engine.PrimitiveComponent))
  (Variables|Default|SetLightMaterial _returnvalue)
  (Rendering|Material|SetMaterial _staticmesh 1 _returnvalue))

(fn ConstructionScript)

(fn LightOff
  (|CallParentFunction)
  (Rendering|Material|SetScalarParameterValue (Variables|Default|GetLightMaterial) "Intensity" 0.0 :!class /Script/Engine.MaterialInstanceDynamic))

(fn Lighton
  (|CallParentFunction)
  (Rendering|Material|SetScalarParameterValue (Variables|Default|GetLightMaterial) "Intensity" 5.5 :!class /Script/Engine.MaterialInstanceDynamic))