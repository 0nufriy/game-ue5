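; Anim notify state that marks the consume window in an animation and reports it to the mesh component's owner.
; Begin sends ConsumeBeginMessage with the window's total duration, and each tick sends ConsumeTickMessage.
; End sends ConsumeEndMessage with whether the notify state reached its end, letting the owner tell completion from interruption.
; The notify holds no consume logic itself and leaves the response to the owner.
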(fn ReceivedNotifyEnd
  (params (MeshComp :type Skeletal%20Mesh%20Component%20Object%20Reference) (Animation :type Anim%20Sequence%20Base%20Object%20Reference) (EventReference :type Anim%20Notify%20Event%20Reference%20Structure%20%28by%20ref%29))
  (Class|BPIConsumer|ConsumeEnd(Message) (Components|GetOwner MeshComp) (Class|AnimNotifyLibrary|NotifyStateReachedEnd EventReference))
  (return true))

(fn ReceivedNotifyBegin
  (params (MeshComp :type Skeletal%20Mesh%20Component%20Object%20Reference) (Animation :type Anim%20Sequence%20Base%20Object%20Reference) (TotalDuration :type Float%20%28single-precision%29) (EventReference :type Anim%20Notify%20Event%20Reference%20Structure%20%28by%20ref%29))
  (Class|BPIConsumer|ConsumeBegin(Message) (Components|GetOwner MeshComp) TotalDuration)
  (return true))

(fn ReceivedNotifyTick
  (params (MeshComp :type Skeletal%20Mesh%20Component%20Object%20Reference) (Animation :type Anim%20Sequence%20Base%20Object%20Reference) (FrameDeltaTime :type Float%20%28single-precision%29) (EventReference :type Anim%20Notify%20Event%20Reference%20Structure%20%28by%20ref%29))
  (Class|BPIConsumer|ConsumeTick(Message) (Components|GetOwner MeshComp))
  (return true))