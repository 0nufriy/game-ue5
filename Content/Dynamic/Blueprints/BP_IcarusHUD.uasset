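; Per-player HUD for Icarus that creates and owns the UI_BaseHUD widget, scaling it for split-screen by player count and controller ID.
; On possession it builds the widget and binds to the pawn's health component.
; Once all characters load, it binds to other players' class-set events for teammate widgets.
; Events forward death, shop, result and input updates to the widget, some polling each tick until it exists.
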(event Custom|OnPossessedPawnChanged_Event
  (params (OldPawn :type Pawn%20Object%20Reference) (NewPawn :type Pawn%20Object%20Reference))
  (bind _returnvalue (Class|HUD|GetOwningPawn))
  (bind _returnvalue_2 (Actor|GetComponentbyClass _returnvalue "/Game/Dynamic/Blueprints/Components/HealthSystem/BPC_HealthSystem.BPC_HealthSystem_C"))
  (Utilities|FlowControl|Sequence
    (:then_0
      (CallFunction|SetResizeHud))
    (:then_1
      (CallFunction|SetHUD)
      (Utilities|IsValid _returnvalue
        (:Is%20Valid
          (Utilities|IsValid _returnvalue_2
            (:Is%20Valid
              (bind _output_get (Variables|Default|SetHealthComponent _returnvalue_2))
              (EventDispatchers|BindEventtoOnHealthUpdated _returnvalue_2 (EventDispatchers|CreateEvent (Variables|Default|GetBaseWidget) :!event SetCurrentHealth))
              (EventDispatchers|BindEventtoOnMaxHeathUpdated _returnvalue_2 (delegate Custom|OnMaxHealthChanged)))))))))

(event Custom|OnAllCharactersLoaded_Event
  (params (Characters :type Array%20of%20BP%20Player%20Character%20Object%20References))
  ;[0 0 0] Setup for All characters load
  (CallFunction|SetupforPlayerClassChange Characters)
  (EventDispatchers|UnbindEventfromOnCharactersUpdated (Variables|Default|GetGame%20State) (EventDispatchers|CreateEvent :!event SetupforPlayerClassChange)))

(event Custom|OnMaxHealthChanged
  (params (NewMaxHealth :type Float%20%28double-precision%29))
  (Default|SetMaxHealth (Variables|Default|GetBaseWidget) (Default|GetCurrentHealth (Variables|Default|GetHealthComponent)) NewMaxHealth))

(event EventBeginPlay
  (bind _returnvalue (Class|HUD|GetOwningPawn))
  (bind _ismultiplayer (Class|BPIMultiplayer|GetIsMultiplayer(Message) (Game|GetGameInstance)))
  (Variables|Default|SetIsMultiplayer _ismultiplayer)
  (bind _asbp_main_game_state (Utilities|Casting|CastToBP_MainGameState (Game|GetGameState)))
  (Variables|Default|SetGame%20State _asbp_main_game_state)
  (Utilities|FlowControl|Sequence
    (:then_0
      ;[0 0 0] Setup for All characters load
      (bind _returnvalue_2 (Default|AllPlayersLoaded (Variables|Default|GetGame%20State)))
      (if _returnvalue_2
        (CallFunction|SetupforPlayerClassChange (Variables|/Game/Dynamic/Blueprints/BP_MainGameState.BP_MainGameState_C|GetPlayerCharacters (Variables|Default|GetGame%20State)))
        (else
          (EventDispatchers|AssignOnAllCharactersLoaded (Variables|Default|GetGame%20State) (delegate Custom|OnAllCharactersLoaded_Event)))))
    (:then_1
      (Utilities|IsValid _returnvalue
        (:Is%20Valid
          (CallFunction|OnPossessedPawnChangedEvent 0 _returnvalue))
        (:Is%20Not%20Valid
          (EventDispatchers|AssignOnPossessedPawnChanged (Game|Player|GetOwningPlayerController) (delegate Custom|OnPossessedPawnChanged_Event)))))))

(event EventAddCrewWidgets
  (params (OtherCharacters :type Array%20of%20BP%20Player%20Character%20Object%20References))
  (bind _basewidget (Variables|Default|GetBaseWidget))
  (Utilities|IsValid _basewidget :!label _label
    (:Is%20Valid
      (Default|InitializeTeammateWidgets _basewidget OtherCharacters))
    (:Is%20Not%20Valid
      (Utilities|FlowControl|DelayUntilNextTick)
      (goto _label))))

(event EventSetResult
  (params (Percent :type Float%20%28double-precision%29))
  (Default|SetResult (Variables|Default|GetBaseWidget) Percent))

(event EventWidgetAdded
  (params (Widget :type Widget%20Object%20Reference) (LocalPlayer :type Local%20Player%20Object%20Reference))
  (if (Variables|Default|GetbResizeHud)
    (if (not (Variables|Default|GetIsMultiplayer))
      (bind _asbp_player_character (Utilities|Casting|CastToBP_PlayerCharacter (Class|HUD|GetOwningPawn)))
      (if (== LocalPlayer (Class|GetLocalPlayer|GetLocalPlayerfromController (Variables|/Game/Dynamic/Blueprints/BP_PlayerCharacter.BP_PlayerCharacter_C|GetGetLocalPlayer _asbp_player_character) (Game|Player|GetOwningPlayerController)))
        (Class|BPIResizableUI|SetScale(Message) Widget (Variables|Default|GetScreen%20Size))))))

(event EventSetIsDead
  (params (Dead :type Boolean))
  (Default|SetDeath (Variables|Default|GetBaseWidget) Dead)
  (Variables|Default|SetDead Dead))

(event EventSetInput
  (params (BPC_Input :type BPC%20Input%20Object%20Reference))
  (bind _basewidget (Variables|Default|GetBaseWidget))
  (Utilities|IsValid _basewidget
    (:Is%20Valid
      (Utilities|FlowControl|DoOnce false
        (:Completed
          (Default|SetInput _basewidget BPC_Input))))))

(event EventRefreshDeathCam
  (bind _basewidget (Variables|Default|GetBaseWidget))
  (if (Variables|Default|GetDead)
    (Utilities|IsValid _basewidget
      (:Is%20Valid
        (Default|RefreshDeathCam _basewidget)))))

(event EventUnwait
  (bind _basewidget (Variables|Default|GetBaseWidget))
  (Utilities|IsValid _basewidget :!label _label
    (:Is%20Valid
      (Default|Unwait _basewidget))
    (:Is%20Not%20Valid
      (Utilities|FlowControl|DelayUntilNextTick)
      (goto _label))))

(event EventSetShopTime
  (params (Seconds :type Integer))
  (Default|SetShopTime (Variables|Default|GetBaseWidget) Seconds))

(event EventChangeResultShop
  (params (Shop :type Boolean))
  (Default|ChangeResulrBar (Variables|Default|GetBaseWidget) Shop))

(fn ConstructionScript)

(fn SetHUD
  (bind _returnvalue (Class|HUD|GetOwningPawn))
  (bind _maxhealth (Class|BPIDamagable|GetMaxHealth(Message) _returnvalue))
  (bind _currenthealth (Class|BPIDamagable|GetCurrentHealth(Message) _returnvalue))
  (bind _returnvalue_2 (UserInterface|CreateWidget "/Game/Dynamic/Blueprints/UI/BaseHUD/UI_BaseHUD.UI_BaseHUD_C" (Game|Player|GetOwningPlayerController) _currenthealth _maxhealth (Class|HUD|GetOwningPawn)))
  (Variables|Default|SetBaseWidget _returnvalue_2)
  (Utilities|FlowControl|Sequence
    (:then_0
      (if (Pawn|IsLocalController (Game|Player|GetOwningPlayerController))
        (UserInterface|Viewport|AddtoPlayerScreen (Variables|Default|GetBaseWidget))))
    (:then_1
      (if (Variables|Default|GetbResizeHud)
        (Default|SetScale (Variables|Default|GetBaseWidget) (Variables|Default|GetScreen%20Size))))))

(fn ResizeHurtandResult
  (bind _returnvalue (Class|WidgetLayoutLibrary|GetPlayerScreenWidgetGeometry (select (Variables|Default|GetIsMultiplayer) (Game|GetPlayerController 0) 0)))
  (Default|SetHurtSize (Variables|Default|GetBaseWidget) (Class|SlateBlueprintLibrary|GetAbsoluteSize _returnvalue))
  (Default|ResizeResult (Variables|Default|GetBaseWidget) (Class|SlateBlueprintLibrary|GetAbsoluteSize _returnvalue)))

(fn ShouldUIbeResized
  (params (PlayerIndex :type Integer) (PlayersNumber :type Integer))
  (return (or (== PlayersNumber 4) (and (!= PlayerIndex 0) (== PlayersNumber 3)))))

(fn SetResizeHud
  (Utilities|FlowControl|Sequence
    (:then_0
      (bind _count (Class|BPIMultiplayer|GetMultiplayerPlayerCount(Message) (Game|GetGameInstance)))
      (if (== _count 1)
        (Variables|Default|SetScreen%20Size "NewEnumerator0")
        (elif (or (== _count 2) (and (== _count 3) (== (Class|GameplayStatics|GetPlayerControllerID (Game|Player|GetOwningPlayerController)) 0)))
          (Variables|Default|SetScreen%20Size "NewEnumerator1")
          (else
            (Variables|Default|SetScreen%20Size "NewEnumerator2")))))
    (:then_1
      (Variables|Default|SetbResizeHud (Utilities|Enum|NotEqual(Enum) (Variables|Default|GetScreen%20Size) "NewEnumerator0")))))

(fn SetupforPlayerClassChange
  (params (Characters :type Array%20of%20BP%20Player%20Character%20Object%20References))
  (bind _players (CallFunction|CopyPlayersArrayWithoutOne Characters (Class|HUD|GetOwningPawn)))
  (for _array_element _players
    (EventDispatchers|BindEventtoOnClassSet _array_element (EventDispatchers|CreateEvent :!event InitializeTeammateWidget))))

(fn InitializeTeammateWidget
  (params (Character :type BP%20Player%20Character%20Object%20Reference))
  (Development|PrintString "Hello")
  (Default|InitializeTeammateWidget (Variables|Default|GetBaseWidget) Character)
  (EventDispatchers|UnbindEventfromOnClassSet Character (EventDispatchers|CreateEvent :!event InitializeTeammateWidget)))