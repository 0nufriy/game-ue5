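; Actor component that detects attack hits by box tracing between socket pairs on the owner's socket component, destroying itself if none exists.
; Added trace data runs on a looping timer, which stops when the last entry is removed.
; Hit actors are stored in wrapper objects keyed by attack index, created only for the first active trace, so each actor reports once.
; Callbacks signal first trace start, hits and all traces ending.
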(event EventBeginPlay
  (bind _scenecomponent (Class|BPIHitTracer|GetSocketsOwningComponent(Message) (Components|GetOwner)))
  (Utilities|IsValid _scenecomponent
    (:Is%20Valid
      (Variables|Default|SetSocketsComponent _scenecomponent))
    (:Is%20Not%20Valid
      (Components|DestroyComponent))))

(event EventEndPlay
  (params (EndPlayReason :type EEndPlayReason%20Enum :default "Destroyed"))
  ;[1 1 1] On End Play
  (Utilities|Time|ClearandInvalidateTimerbyHandle (Variables|Default|GetDataTracedTimer)))

(fn CollisionTrace
  (params (traceData :type S%20Hit%20Trace%20Data%20Structure))
  (bind (_attackindex _firstsocket _secondsocket _boxsize) (Utilities|Struct|BreakS_HitTraceData traceData))
  (bind _socketscomponent (Variables|Default|GetSocketsComponent))
  (LocalVariables|SetAttackIndex _attackindex)
  (bind (_outhits _returnvalue) (Class|KismetSystemLibrary|BoxTraceMulti (Transformation|GetSocketLocation _socketscomponent _firstsocket) (Transformation|GetSocketLocation _socketscomponent _secondsocket) _boxsize (Transformation|GetActorRotation (Components|GetOwner)) (Variables|Default|GetTrace%20Channel) false (Variables|Default|GetActorsToIgnore) (Variables|Debug|GetDraw%20Debug%20Type) (Variables|Default|GetbIgnoreSelf) "(R=1.000000,G=0.000000,B=0.000000,A=1.000000)" "(R=0.000000,G=1.000000,B=0.000000,A=1.000000)" (Variables|Debug|GetDrawTime)))
  (if _returnvalue
    (CallFunction|ProcessHitResults (LocalVariables|GetAttackIndex) _outhits)))

(fn MultiPartsTrace
  (for _array_element (Variables|Default|GetTracePointsArray)
    (CallFunction|CollisionTrace _array_element)))

(fn AddTraceData
  (params (TraceData :type S%20Hit%20Trace%20Data%20Structure%20%28by%20ref%29))
  (bind _tracepointsarray (Variables|Default|GetTracePointsArray))
  (bind _returnvalue (Utilities|Array|AddUnique _tracepointsarray TraceData))
  (if (and (>= _returnvalue 0) (== (Utilities|Array|Length _tracepointsarray) 1))
    (bind _returnvalue_2 (Game|ConstructObjectfromClass "/Game/Dynamic/Blueprints/Objects/BP_ActorArray.BP_ActorArray_C"))
    (Utilities|Map|Add (Variables|Default|GetAttackHittedActors) (.AttackIndex (Utilities|Struct|BreakS_HitTraceData TraceData)) _returnvalue_2)
    (Default|CallOnFirstTraceStart)
    (bind _returnvalue_3 (Utilities|Time|SetTimerbyFunctionName 0 "MultiPartsTrace" (Variables|Default|GetUpdateTime) true))
    (Variables|Default|SetDataTracedTimer _returnvalue_3)))

(fn RemoveTraceData
  (params (AttackIndex :type Integer%20%28by%20ref%29))
  (bind _tracepointsarray (Variables|Default|GetTracePointsArray))
  (Utilities|FlowControl|Sequence
    (:then_0
      (bind _array_element (Utilities|Array|ForEachLoopwithBreak _tracepointsarray :!label _label)
        (:LoopBody
          (if (== (.AttackIndex (Utilities|Struct|BreakS_HitTraceData _array_element)) AttackIndex)
            (bind _returnvalue (Utilities|Array|RemoveItem _tracepointsarray _array_element))
            (LocalVariables|SetRemoved _returnvalue)
            (goto _label Break)))))
    (:then_1
      (Utilities|Map|Remove (Variables|Default|GetAttackHittedActors) AttackIndex))
    (:then_2
      (if (and (LocalVariables|GetRemoved) (Utilities|Array|IsEmpty (Variables|Default|GetTracePointsArray)))
        (Utilities|Time|ClearandInvalidateTimerbyHandle (Variables|Default|GetDataTracedTimer))
        (Default|CallOnAllTracesEnd)))))

(fn IsTracing
  (return (Utilities|Array|IsNotEmpty (Variables|Default|GetTracePointsArray))))

(fn ProcessHitResults
  (params (AttackIndex :type Integer) (HitResults :type Array%20of%20Hit%20Result%20Structures))
  (bind _attackhittedactors (Variables|Default|GetAttackHittedActors))
  (bind (_value _returnvalue) (Utilities|Map|Find _attackhittedactors AttackIndex))
  (if _returnvalue
    (LocalVariables|SetWrapper _value)
    (for _array_element HitResults
      (bind _returnvalue_2 (Utilities|Array|AddUnique (Variables|/Game/Dynamic/Blueprints/Objects/BP_ActorArray.BP_ActorArray_C|GetArray (LocalVariables|GetWrapper)) (.HitActor (Collision|BreakHitResult _array_element))))
      (if (>= _returnvalue_2 0)
        (Default|CallOnHit _array_element AttackIndex)))))