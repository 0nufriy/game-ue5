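; BPC_CombatSystem is a combat component that holds combo and attack state for its owner.
; It keeps an attack counter with functions to increment, reset and read it, plus an Attacking flag with a getter and setter.
; It contains no combat logic of its own: BeginPlay and Tick are empty, so state changes only when its functions are called.
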(event EventBeginPlay)

(event EventTick
  (params (DeltaSeconds :type Float%20%28single-precision%29)))

(fn IncrementCombo
  (Variables|Combo|SetAttacksCounter (+ (Variables|Combo|GetAttacksCounter) 1)))

(fn ResetComboCounter
  (Variables|Combo|SetAttacksCounter 0))

(fn GetAttacksCounter
  (return (Variables|Combo|GetAttacksCounter)))

(fn IsAttacking
  (return (Variables|Default|GetbAttacking)))

(fn SetIsAttacking
  (params (bAttacking :type Boolean))
  (Variables|Default|SetbAttacking bAttacking))