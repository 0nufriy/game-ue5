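; Combat component that keeps a ledger of attack tokens its owner holds from other targets so they can be given back.
; ReserveTokens accumulates positive amounts per target in the ReservedAttackTokens map; it only records them and does not deduct from the target.
; ReturnAllTokens sends each target its stored total through ReturnAttackTokensMessage, then clears the map.
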(event EventBeginPlay)

(event EventTick
  (params (DeltaSeconds :type Float%20%28single-precision%29)))

(fn ReserveTokens
  (params (Target :type Actor%20Object%20Reference%20%28by%20ref%29) (TokenAmount :type Integer))
  (bind _reservedattacktokens (Variables|Default|GetReservedAttackTokens))
  (bind (_value _returnvalue) (Utilities|Map|Find _reservedattacktokens Target))
  (if (> TokenAmount 0)
    (Utilities|Map|Add (Variables|Default|GetReservedAttackTokens) Target (Math|Integer|SelectInt (+ _value TokenAmount) TokenAmount _returnvalue))))

(fn ReturnAllTokens
  (bind _keys (Utilities|Map|Keys (Variables|Default|GetReservedAttackTokens)))
  (for _array_element _keys
    (Class|BPIDamagable|ReturnAttackTokens(Message) _array_element (.Value (Utilities|Map|Find (Variables|Default|GetReservedAttackTokens) _array_element))))
  (Utilities|Map|Clear (Variables|Default|GetReservedAttackTokens)))