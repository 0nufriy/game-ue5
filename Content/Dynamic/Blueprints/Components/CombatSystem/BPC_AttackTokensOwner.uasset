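; BPC_AttackTokensOwner is a combat-system component that holds a pool of attack tokens for its owner.
; ReserveAttackTokens deducts the requested amount from AttackTokenCount and returns true, or returns false when too few tokens remain.
; ReturnAttackTokens adds positive amounts back to the pool, with no upper cap.
; The component only keeps the count, with no event logic and no record of who holds tokens.
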(event EventBeginPlay)

(event EventTick
  (params (DeltaSeconds :type Float%20%28single-precision%29)))

(fn ReserveAttackTokens
  (params (Amount :type Integer))
  (if (<= Amount (Variables|Tokens|GetAttackTokenCount))
    (Variables|Tokens|SetAttackTokenCount (- (Variables|Tokens|GetAttackTokenCount) Amount))
    (return true)
    (else
      (return false))))

(fn ReturnAttackTokens
  (params (Amount :type Integer))
  (if (> Amount 0)
    (Variables|Tokens|SetAttackTokenCount (+ Amount (Variables|Tokens|GetAttackTokenCount)))))