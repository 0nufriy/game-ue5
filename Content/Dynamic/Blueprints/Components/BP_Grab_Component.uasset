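; Scene component that runs forward-vector traces for player interactions: grabbing items, fixing, taping, extinguishing and short-range wall checks.
; Each function traces on demand and returns hits or actors, with grabbing refining a line hit by a sphere trace.
; AimToTape builds a plane from three offset sphere traces to return a surface-aligned transform.
; Its rotation is found by testing pitch and yaw sign combinations against the normal.
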(event EventBeginPlay)

(event EventTick
  (params (DeltaSeconds :type Float%20%28single-precision%29)))

(fn AimtoFix
  (bind _returnvalue (Transformation|GetWorldLocation))
  (bind _outhit (Collision|LineTraceByChannel _returnvalue (+ _returnvalue (* (Math|Vector|GetForwardVector) (Variables|Default|GetAimFix%20Distance))) "TraceTypeQuery3" false 0 "None" true "(R=1.000000,G=0.000000,B=0.000000,A=1.000000)" "(R=0.000000,G=1.000000,B=0.000000,A=1.000000)" 1.0))
  (return _outhit))

(fn TraceforGrabableItem
  (bind _returnvalue (Transformation|GetWorldLocation))
  (bind (_outhit _returnvalue_2) (Collision|LineTraceByChannel _returnvalue (+ _returnvalue (* (Math|Vector|GetForwardVector) (Variables|Default|GetGrab%20Distance))) "TraceTypeQuery1" false 0 "None"))
  (if _returnvalue_2
    (bind (_outhit_2 _returnvalue_3) (Collision|SphereTraceByChannel (.ImpactPoint (Collision|BreakHitResult _outhit)) (.ImpactPoint (Collision|BreakHitResult _outhit)) (Variables|Default|GetGrab%20Radius) "TraceTypeQuery4" false 0 "None"))
    (return _outhit_2 _returnvalue_3)
    (else
      (return "" false))))

(fn AimtoTape
  (bind _returnvalue (Math|Vector|GetForwardVector))
  (bind _returnvalue_2 (Transformation|GetWorldLocation))
  (bind _returnvalue_3 (Math|Vector|GetForwardVector))
  (bind _returnvalue_4 (Transformation|GetWorldLocation))
  (bind _returnvalue_5 (Math|Vector|GetForwardVector))
  (bind _returnvalue_6 (Transformation|GetWorldLocation))
  (bind _returnvalue_7 (* _returnvalue 80))
  (bind _returnvalue_8 (* _returnvalue_3 80))
  (bind _returnvalue_9 (* _returnvalue_5 80))
  (bind _returnvalue_10 (- _returnvalue_6 _returnvalue_7))
  (bind _returnvalue_11 (- _returnvalue_2 _returnvalue_8))
  (bind _returnvalue_12 (- _returnvalue_4 _returnvalue_9))
  (bind _returnvalue_13 (+ _returnvalue_11 "2.000000,0.000000,0.000000"))
  (bind _returnvalue_14 (+ _returnvalue_10 "0.000000,0.000000,2.000000"))
  (bind _returnvalue_15 (+ _returnvalue_12 "0.000000,0.000000,-2.000000"))
  (Utilities|FlowControl|Sequence
    (:then_0
      (bind (_outhit _returnvalue_16) (Collision|SphereTraceByChannel _returnvalue_14 (+ _returnvalue_14 (* (Math|Vector|GetForwardVector) (Variables|Default|GetTapeDistance))) 0.0 "TraceTypeQuery3" false 0 "None" true "(R=1.000000,G=0.000000,B=0.000000,A=1.000000)" "(R=0.000000,G=1.000000,B=0.000000,A=1.000000)" 2e+01))
      (if _returnvalue_16
        (LocalVariables|SetActor (.HitActor (Collision|BreakHitResult _outhit)))
        (LocalVariables|SetPoint1 (.ImpactPoint (Collision|BreakHitResult _outhit)))
        (else
          (return 0 ""))))
    (:then_1
      (bind (_outhit_2 _returnvalue_17) (Collision|SphereTraceByChannel _returnvalue_15 (+ _returnvalue_15 (* (Math|Vector|GetForwardVector) (Variables|Default|GetTapeDistance))) 0.0 "TraceTypeQuery3" false 0 "None"))
      (if _returnvalue_17
        (LocalVariables|SetPoint2 (.ImpactPoint (Collision|BreakHitResult _outhit_2)))
        (else
          (return 0 ""))))
    (:then_2
      (bind (_outhit_3 _returnvalue_18) (Collision|SphereTraceByChannel _returnvalue_13 (+ _returnvalue_13 (* (Math|Vector|GetForwardVector) (Variables|Default|GetTapeDistance))) 0.0 "TraceTypeQuery3" false 0 "None"))
      (if _returnvalue_18
        (LocalVariables|SetPoint3 (.ImpactPoint (Collision|BreakHitResult _outhit_3)))
        (else
          (return 0 ""))))
    (:then_3
      (LocalVariables|SetPlane (CallFunction|GetPlanefromPoints (LocalVariables|GetPoint1) (LocalVariables|GetPoint2) (LocalVariables|GetPoint3)))
      (LocalVariables|SetRotation (Math|Rotator|MakeRotator 0.0 (CallFunction|Angel (LocalVariables|GetPlane) (Math|Vector4|MakeVector4 0.0 0.0 1.0 0.0) 9e+01) (CallFunction|Angel (LocalVariables|GetPlane) (Math|Vector4|MakeVector4 1.0 0.0 0.0 0.0) 0.0)))
      (return (LocalVariables|GetActor) (Math|Transform|MakeTransform (+ (/ (+ (LocalVariables|GetPoint1) (LocalVariables|GetPoint2) (LocalVariables|GetPoint3)) 3) (* (Math|Vector|MakeVector (.X (Math|Vector4|BreakVector4 (LocalVariables|GetPlane))) (.Y (Math|Vector4|BreakVector4 (LocalVariables|GetPlane))) (.Z (Math|Vector4|BreakVector4 (LocalVariables|GetPlane)))) 0.5)) (CallFunction|RotationVectortoGetSame (LocalVariables|GetRotation) (Math|Vector|MakeVector 1.0 0.0 0.0) (Math|Vector|MakeVector (.X (Math|Vector4|BreakVector4 (LocalVariables|GetPlane))) (.Y (Math|Vector4|BreakVector4 (LocalVariables|GetPlane))) (.Z (Math|Vector4|BreakVector4 (LocalVariables|GetPlane)))) (CallFunction|Angel (LocalVariables|GetPlane) (Math|Vector4|MakeVector4 0.0 1.0 0.0 0.0) -9e+01)))))))

(fn GetPlanefromPoints
  (params (P0 :type Vector) (P1 :type Vector) (P2 :type Vector))
  (bind (_x _y _z) (Math|Vector|BreakVector P1))
  (bind _returnvalue (- P2 P0))
  (bind _returnvalue_2 (- P1 P0))
  (bind _returnvalue_3 (Math|Vector|CrossProduct _returnvalue_2 _returnvalue))
  (bind _returnvalue_4 (Math|Vector|Normalize _returnvalue_3))
  (bind _output_get (LocalVariables|SetNormal (* _returnvalue_4 (Math|Integer|SelectInt -1 1 (> (Math|Vector|DotProduct _returnvalue_4 (Math|Vector|GetForwardVector)) 0.0)))))
  (return (Math|Vector4|MakeVector4 (.X (Math|Vector|BreakVector _output_get)) (.Y (Math|Vector|BreakVector _output_get)) (.Z (Math|Vector|BreakVector _output_get)) (Utilities|Operators|Subtract 0.0 (* (.X (Math|Vector|BreakVector (LocalVariables|GetNormal))) _x) (* (.Y (Math|Vector|BreakVector (LocalVariables|GetNormal))) _y) (* (.Z (Math|Vector|BreakVector (LocalVariables|GetNormal))) _z)))))

(fn Angel
  (params (Plane1 :type Vector%204%20Structure) (Plane2 :type Vector%204%20Structure) (Add%20to%20angel :type Float%20%28double-precision%29))
  (bind (_x _y _z) (Math|Vector4|BreakVector4 Plane1))
  (bind (_x_2 _y_2 _z_2) (Math|Vector4|BreakVector4 Plane2))
  (bind (_x_3 _y_3 _z_3) (Math|Vector4|BreakVector4 Plane1))
  (bind (_x_4 _y_4 _z_4) (Math|Vector4|BreakVector4 Plane2))
  (bind _returnvalue (Math|Float|Square _x))
  (bind _returnvalue_2 (Math|Float|Square _z_2))
  (bind _returnvalue_3 (Math|Float|Square _x_2))
  (bind _returnvalue_4 (Math|Float|Square _y_2))
  (bind _returnvalue_5 (Math|Float|Square _y))
  (bind _returnvalue_6 (Math|Float|Square _z))
  (bind _returnvalue_7 (* _z_3 _z_4))
  (bind _returnvalue_8 (* _x_3 _x_4))
  (bind _returnvalue_9 (* _y_3 _y_4))
  (bind _returnvalue_10 (+ _returnvalue_8 _returnvalue_9 _returnvalue_7))
  (bind _returnvalue_11 (+ _returnvalue_3 _returnvalue_4 _returnvalue_2))
  (bind _returnvalue_12 (+ _returnvalue _returnvalue_5 _returnvalue_6))
  (bind _returnvalue_13 (Math|Float|Sqrt _returnvalue_11))
  (bind _returnvalue_14 (Math|Float|Sqrt _returnvalue_12))
  (bind _returnvalue_15 (* _returnvalue_14 _returnvalue_13))
  (bind _returnvalue_16 (/ _returnvalue_10 _returnvalue_15))
  (bind _returnvalue_17 (Class|KismetMathLibrary|DegAcos _returnvalue_16))
  (bind _returnvalue_18 (+ Add%20to%20angel _returnvalue_17))
  (return (Math|Float|SelectFloat 1.8e+02 _returnvalue_18 (or (and (< _returnvalue_18 0.0) (> _returnvalue_18 -0.1)) (and (< _returnvalue_18 0.1) (> _returnvalue_18 0.0))))))

(fn AimtoExtinguish
  (bind _returnvalue (Transformation|GetWorldLocation))
  (bind (_outhits _returnvalue_2) (Collision|MultiSphereTraceByChannel _returnvalue (+ _returnvalue (* (Math|Vector|GetForwardVector) (Variables|Default|GetExtingushDistance))) 5e+01 "TraceTypeQuery5" false 0 "None"))
  (if _returnvalue_2
    (for _array_element _outhits
      (Utilities|Array|Add (LocalVariables|GetActorArray) (.HitActor (Collision|BreakHitResult _array_element))))
    (return (LocalVariables|GetActorArray))
    (else
      (return 0))))

(fn RotationVectortoGetSame
  (params (Rotator :type Rotator) (V1 :type Vector) (V2 :type Vector) (OtherYaw :type Float%20%28double-precision%29))
  (bind (_roll _pitch) (Math|Rotator|BreakRotator Rotator))
  (bind (_x _y _z) (Math|Vector|BreakVector V2))
  (bind (_x_2 _y_2 _z_2) (Math|Vector|BreakVector V2))
  (bind (_roll_2 _pitch_2 _yaw) (Math|Rotator|BreakRotator Rotator))
  (bind (_x_3 _y_3 _z_3) (Math|Vector|BreakVector V2))
  (bind (_roll_3 _pitch_3 _yaw_2) (Math|Rotator|BreakRotator Rotator))
  (bind (_x_4 _y_4 _z_4) (Math|Vector|BreakVector V2))
  (bind _returnvalue (Math|Vector|RotateVector V1 Rotator))
  (bind (_x_5 _y_5 _z_5) (Math|Vector|BreakVector V2))
  (bind (_x_6 _y_6 _z_6) (Math|Vector|BreakVector V2))
  (bind (_roll_4 _pitch_4 _yaw_3) (Math|Rotator|BreakRotator Rotator))
  (bind (_x_7 _y_7 _z_7) (Math|Vector|BreakVector V2))
  (bind _returnvalue_2 (* _yaw 1.0))
  (bind _returnvalue_3 (* _pitch_3 1.0))
  (bind _returnvalue_4 (* _yaw_2 -1.0))
  (bind _returnvalue_5 (* _returnvalue -1))
  (bind _returnvalue_6 (* _pitch_4 -1.0))
  (bind _returnvalue_7 (* _yaw_3 -1.0))
  (bind _returnvalue_8 (* _pitch_2 -1.0))
  (bind _returnvalue_9 (Math|Rotator|MakeRotator _roll_2 _returnvalue_8 _returnvalue_2))
  (bind _returnvalue_10 (Math|Rotator|MakeRotator _roll_3 _returnvalue_3 _returnvalue_4))
  (bind (_x_8 _y_8 _z_8) (Math|Vector|BreakVector _returnvalue_5))
  (bind _returnvalue_11 (Math|Rotator|MakeRotator _roll_4 _returnvalue_6 _returnvalue_7))
  (bind _returnvalue_12 (Math|Vector|RotateVector V1 _returnvalue_9))
  (bind _returnvalue_13 (Math|Vector|RotateVector V1 _returnvalue_10))
  (bind _returnvalue_14 (Math|Vector|RotateVector V1 _returnvalue_11))
  (bind _returnvalue_15 (* _returnvalue_13 -1))
  (bind _returnvalue_16 (* _returnvalue_14 -1))
  (bind _returnvalue_17 (* _returnvalue_12 -1))
  (bind (_x_9 _y_9 _z_9) (Math|Vector|BreakVector _returnvalue_17))
  (bind (_x_10 _y_10 _z_10) (Math|Vector|BreakVector _returnvalue_15))
  (bind (_x_11 _y_11 _z_11) (Math|Vector|BreakVector _returnvalue_16))
  (Utilities|FlowControl|Sequence
    (:then_0
      (Utilities|FlowControl|Sequence
        (:then_0
          (if (Math|Boolean|ANDBoolean (Math|Float|NearlyEqual(Float) _x_3 _x_9 0.2) (Math|Float|NearlyEqual(Float) _y_3 _y_9 0.2) (Math|Float|NearlyEqual(Float) _z_3 _z_9 0.2))
            (return _returnvalue_9)))
        (:then_1
          (if (Math|Boolean|ANDBoolean (Math|Float|NearlyEqual(Float) _x_4 _x_10 0.2) (Math|Float|NearlyEqual(Float) _y_4 _y_10 0.2) (Math|Float|NearlyEqual(Float) _z_4 _z_10 0.2))
            (return _returnvalue_10)))
        (:then_2
          (if (Math|Boolean|ANDBoolean (Math|Float|NearlyEqual(Float) _x_7 _x_11 0.2) (Math|Float|NearlyEqual(Float) _y_7 _y_11 0.2) (Math|Float|NearlyEqual(Float) _z_7 _z_11 0.2))
            (return _returnvalue_11)))
        (:then_3
          (if (Math|Boolean|ANDBoolean (Math|Float|NearlyEqual(Float) _x_6 _x_8 0.2) (Math|Float|NearlyEqual(Float) _y_6 _y_8 0.2) (Math|Float|NearlyEqual(Float) _z_6 _z_8 0.2))
            (return Rotator)))))
    (:then_1
      (LocalVariables|SetRotatorNew (Math|Rotator|MakeRotator _roll _pitch OtherYaw))
      (Utilities|FlowControl|Sequence
        (:then_0
          (if (Math|Boolean|ANDBoolean (Math|Float|NearlyEqual(Float) _x (.X (Math|Vector|BreakVector (* (Math|Vector|RotateVector V1 (Math|Rotator|MakeRotator (.Roll (Math|Rotator|BreakRotator (LocalVariables|GetRotatorNew))) (* (.Pitch (Math|Rotator|BreakRotator (LocalVariables|GetRotatorNew))) -1.0) (* (.Yaw (Math|Rotator|BreakRotator (LocalVariables|GetRotatorNew))) 1.0))) -1))) 0.2) (Math|Float|NearlyEqual(Float) _y (.Y (Math|Vector|BreakVector (* (Math|Vector|RotateVector V1 (Math|Rotator|MakeRotator (.Roll (Math|Rotator|BreakRotator (LocalVariables|GetRotatorNew))) (* (.Pitch (Math|Rotator|BreakRotator (LocalVariables|GetRotatorNew))) -1.0) (* (.Yaw (Math|Rotator|BreakRotator (LocalVariables|GetRotatorNew))) 1.0))) -1))) 0.2) (Math|Float|NearlyEqual(Float) _z (.Z (Math|Vector|BreakVector (* (Math|Vector|RotateVector V1 (Math|Rotator|MakeRotator (.Roll (Math|Rotator|BreakRotator (LocalVariables|GetRotatorNew))) (* (.Pitch (Math|Rotator|BreakRotator (LocalVariables|GetRotatorNew))) -1.0) (* (.Yaw (Math|Rotator|BreakRotator (LocalVariables|GetRotatorNew))) 1.0))) -1))) 0.2))
            (return (Math|Rotator|MakeRotator (.Roll (Math|Rotator|BreakRotator (LocalVariables|GetRotatorNew))) (* (.Pitch (Math|Rotator|BreakRotator (LocalVariables|GetRotatorNew))) -1.0) (* (.Yaw (Math|Rotator|BreakRotator (LocalVariables|GetRotatorNew))) 1.0)))))
        (:then_1
          (if (Math|Boolean|ANDBoolean (Math|Float|NearlyEqual(Float) _x_2 (.X (Math|Vector|BreakVector (* (Math|Vector|RotateVector V1 (Math|Rotator|MakeRotator (.Roll (Math|Rotator|BreakRotator (LocalVariables|GetRotatorNew))) (* (.Pitch (Math|Rotator|BreakRotator (LocalVariables|GetRotatorNew))) 1.0) (* (.Yaw (Math|Rotator|BreakRotator (LocalVariables|GetRotatorNew))) -1.0))) -1))) 0.2) (Math|Float|NearlyEqual(Float) _y_2 (.Y (Math|Vector|BreakVector (* (Math|Vector|RotateVector V1 (Math|Rotator|MakeRotator (.Roll (Math|Rotator|BreakRotator (LocalVariables|GetRotatorNew))) (* (.Pitch (Math|Rotator|BreakRotator (LocalVariables|GetRotatorNew))) 1.0) (* (.Yaw (Math|Rotator|BreakRotator (LocalVariables|GetRotatorNew))) -1.0))) -1))) 0.2) (Math|Float|NearlyEqual(Float) _z_2 (.Z (Math|Vector|BreakVector (* (Math|Vector|RotateVector V1 (Math|Rotator|MakeRotator (.Roll (Math|Rotator|BreakRotator (LocalVariables|GetRotatorNew))) (* (.Pitch (Math|Rotator|BreakRotator (LocalVariables|GetRotatorNew))) 1.0) (* (.Yaw (Math|Rotator|BreakRotator (LocalVariables|GetRotatorNew))) -1.0))) -1))) 0.2))
            (return (Math|Rotator|MakeRotator (.Roll (Math|Rotator|BreakRotator (LocalVariables|GetRotatorNew))) (* (.Pitch (Math|Rotator|BreakRotator (LocalVariables|GetRotatorNew))) 1.0) (* (.Yaw (Math|Rotator|BreakRotator (LocalVariables|GetRotatorNew))) -1.0)))))
        (:then_2
          (if (Math|Boolean|ANDBoolean (Math|Float|NearlyEqual(Float) _x_5 (.X (Math|Vector|BreakVector (* (Math|Vector|RotateVector V1 (Math|Rotator|MakeRotator (.Roll (Math|Rotator|BreakRotator (LocalVariables|GetRotatorNew))) (* (.Pitch (Math|Rotator|BreakRotator (LocalVariables|GetRotatorNew))) -1.0) (* (.Yaw (Math|Rotator|BreakRotator (LocalVariables|GetRotatorNew))) -1.0))) -1))) 0.2) (Math|Float|NearlyEqual(Float) _y_5 (.Y (Math|Vector|BreakVector (* (Math|Vector|RotateVector V1 (Math|Rotator|MakeRotator (.Roll (Math|Rotator|BreakRotator (LocalVariables|GetRotatorNew))) (* (.Pitch (Math|Rotator|BreakRotator (LocalVariables|GetRotatorNew))) -1.0) (* (.Yaw (Math|Rotator|BreakRotator (LocalVariables|GetRotatorNew))) -1.0))) -1))) 0.2) (Math|Float|NearlyEqual(Float) _z_5 (.Z (Math|Vector|BreakVector (* (Math|Vector|RotateVector V1 (Math|Rotator|MakeRotator (.Roll (Math|Rotator|BreakRotator (LocalVariables|GetRotatorNew))) (* (.Pitch (Math|Rotator|BreakRotator (LocalVariables|GetRotatorNew))) -1.0) (* (.Yaw (Math|Rotator|BreakRotator (LocalVariables|GetRotatorNew))) -1.0))) -1))) 0.2))
            (return (Math|Rotator|MakeRotator (.Roll (Math|Rotator|BreakRotator (LocalVariables|GetRotatorNew))) (* (.Pitch (Math|Rotator|BreakRotator (LocalVariables|GetRotatorNew))) -1.0) (* (.Yaw (Math|Rotator|BreakRotator (LocalVariables|GetRotatorNew))) -1.0)))))))
    (:then_2
      (return (LocalVariables|GetRotatorNew)))))

(fn AimtoDamageFix
  (bind _returnvalue (Transformation|GetWorldLocation))
  (bind (_outhits _returnvalue_2) (Collision|MultiSphereTraceByChannel _returnvalue (+ _returnvalue (* (Math|Vector|GetForwardVector) (Variables|Default|GetAimFix%20Distance))) 0.0 "TraceTypeQuery1" false 0 "None"))
  (if _returnvalue_2
    (return _outhits)
    (else
      (return 0))))

(fn TraceWall
  (bind _returnvalue (Transformation|GetWorldLocation))
  (bind (_outhit _returnvalue_2) (Collision|LineTraceByChannel _returnvalue (+ _returnvalue (* (Math|Vector|GetForwardVector) 7e+01)) "TraceTypeQuery1" false 0 "None" true "(R=1.000000,G=0.000000,B=0.000000,A=1.000000)" "(R=0.000000,G=1.000000,B=0.000000,A=1.000000)" 1.0))
  (return _outhit _returnvalue_2))