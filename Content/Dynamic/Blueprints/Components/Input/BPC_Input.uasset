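; Input component that tracks whether the player is using keyboard and mouse or gamepad and supplies matching button prompts.
; Any key press or noticeable mouse movement updates the device state, firing OnInputSwitch and a debug print on change.
; GetKeyImage and GetKeyText map logical actions to the current device's icon or label, using Xbox glyphs for PSGamepad.
; A helper macro caches the owning pawn's PlayerController; cursor repositioning on switch is disabled.
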(event Input|KeyboardEvents|AnyKey
  (params (Key :type Key%20Structure :default "None"))
  (:Pressed
    (CallFunction|SetIsGamepad (Class|KismetInputLibrary|KeyIsGamepadKey Key))))

(event Input|MouseEvents|Mouse2D
  (params (AxisValue :type Vector :default "0, 0, 0"))
  (bind _playercontroller (Utilities|GetController)
    (:Valid
      (if (Utilities|Operators|NotEqual(!=) :B (Math|Vector2D|MakeVector2D (.DeltaX (Class|PlayerController|GetInputMouseDelta _playercontroller)) (.DeltaY (Class|PlayerController|GetInputMouseDelta _playercontroller))) :ErrorTolerance 0.1)
        (CallFunction|SetIsGamepad false)))))

(fn IsGamepad
  (return (Variables|Default|GetbIsGamepad)))

(fn SetIsGamepad
  (params (bIsGamepad :type Boolean))
  (if (!= bIsGamepad (Variables|Default|GetbIsGamepad))
    (bind _output_get (Variables|Default|SetbIsGamepad bIsGamepad))
    (Variables|Default|SetInputType (select _output_get "NewEnumerator1" "NewEnumerator0"))
    (Default|CallOnInputSwitch)
    (Development|PrintString (Utilities|String|SelectString "Gamepad" "Mouse" _output_get))))

(fn GetKeyImage
  (params (InputKey :type E_IAType%20Enum :default "NewEnumerator0"))
  (switch Utilities|FlowControl|Switch|SwitchonE_IAType InputKey
    (:NewEnumerator0
      (return (Utilities|Select :Index (Variables|Default|GetInputType) :NewEnumerator0 "/Game/Dynamic/Blueprints/UI/Map/Keyboard/E-Key.E-Key" :NewEnumerator1 "/Game/Dynamic/Blueprints/UI/Map/Gamepad/Digital_Buttons/ABXY/button_xbox_digital_x_10.button_xbox_digital_x_10")))
    (:NewEnumerator2
      (return (Utilities|Select :Index (Variables|Default|GetInputType) :NewEnumerator0 "/Game/Dynamic/Blueprints/UI/Map/Keyboard/Space-Key.Space-Key" :NewEnumerator1 "/Game/Dynamic/Blueprints/UI/Map/Gamepad/Digital_Buttons/ABXY/button_xbox_digital_a_10.button_xbox_digital_a_10")))
    (:NewEnumerator3
      (return (Utilities|Select :Index (Variables|Default|GetInputType) :NewEnumerator0 "/Game/Dynamic/Blueprints/UI/Map/Keyboard/Esc-Key.Esc-Key" :NewEnumerator1 "/Game/Dynamic/Blueprints/UI/Map/Gamepad/Digital_Buttons/ABXY/button_xbox_digital_b_10.button_xbox_digital_b_10")))
    (:NewEnumerator4
      (return (Utilities|Select :Index (Variables|Default|GetInputType) :NewEnumerator0 "/Game/Dynamic/Blueprints/UI/Map/Keyboard/Tab-Key.Tab-Key" :NewEnumerator1 "/Game/Dynamic/Blueprints/UI/Map/Gamepad/Digital_Buttons/System/button_xbox_digital_start_2.button_xbox_digital_start_2")))
    (:NewEnumerator5
      (return (Utilities|Select :Index (Variables|Default|GetInputType) :NewEnumerator0 "/Game/Dynamic/Blueprints/UI/Map/Keyboard/R-Key.R-Key" :NewEnumerator1 "/Game/Dynamic/Blueprints/UI/Map/Gamepad/Digital_Buttons/ABXY/button_xbox_digital_y_10.button_xbox_digital_y_10")))))

(fn GetKeyText
  (params (InputKey :type E_IAType%20Enum :default "NewEnumerator0"))
  (switch Utilities|FlowControl|Switch|SwitchonE_IAType InputKey
    (:NewEnumerator0
      (return (Utilities|Select :Index (Variables|Default|GetInputType) :NewEnumerator0 "E" :NewEnumerator1 "X")))
    (:NewEnumerator2
      (return (Utilities|Select :Index (Variables|Default|GetInputType) :NewEnumerator0 "Space" :NewEnumerator1 "A")))
    (:NewEnumerator3
      (return (Utilities|Select :Index (Variables|Default|GetInputType) :NewEnumerator0 "Esc" :NewEnumerator1 "B")))
    (:NewEnumerator4
      (return (Utilities|Select :Index (Variables|Default|GetInputType) :NewEnumerator0 "Tab" :NewEnumerator1 "Start")))
    (:NewEnumerator5
      (return (Utilities|Select :Index (Variables|Default|GetInputType) :NewEnumerator0 "R" :NewEnumerator1 "Y")))))