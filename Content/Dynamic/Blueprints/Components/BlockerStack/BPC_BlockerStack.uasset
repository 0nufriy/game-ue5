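; BPC_BlockerStack is a component that tracks how many blockers are currently active on its owner as a simple counter.
; Add and Remove functions raise or lower the count, with removal clamped at zero, and Reset clears it.
; HasNoBlockers and GetBlockerCount expose the state for queries, so several independent sources can block the same thing without tracking each other.
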(event EventBeginPlay)

(event EventTick
  (params (DeltaSeconds :type Float%20%28single-precision%29)))

(fn AddBlocker
  (Variables|Default|SetBlockerCount (+ (Variables|Default|GetBlockerCount) 1)))

(fn HasNoBlockers
  (return (<= (Variables|Default|GetBlockerCount) 0)))

(fn RemoveBlocker
  (Variables|Default|SetBlockerCount (Math|Integer|Max(Integer) 0 (- (Variables|Default|GetBlockerCount) 1))))

(fn ResetBlockers
  (Variables|Default|SetBlockerCount 0))

(fn GetBlockerCount
  (return (Variables|Default|GetBlockerCount)))