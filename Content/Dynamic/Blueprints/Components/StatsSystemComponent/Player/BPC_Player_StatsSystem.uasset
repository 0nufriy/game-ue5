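; Player stats component that manages oxygen supplied by an attachable tank.
; Attaching a tank sets current and max oxygen, detaching zeroes both, and each fires an event dispatcher.
; Healing and draining clamp the value and broadcast changes, with drain scaled by a modifier and signalling when oxygen runs out.
; Draining at zero oxygen instead damages the owner for half the drain amount, without stun.
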(fn OxHeal
  (params (OxToHeal :type Float%20%28double-precision%29))
  (bind _output_get (Variables|Stats|SetOxCurent (Math|Float|Clamp(Float) (+ (Variables|Stats|GetOxCurent) OxToHeal) 0.0 (Variables|Stats|GetOxMax))))
  (Default|CallOnOxChange _output_get)
  (return (Variables|Stats|GetOxCurent)))

(fn OxFall
  (params (OxFall :type Float%20%28double-precision%29))
  (if (!= (Variables|Stats|GetOxCurent) 0.0)
    (bind _output_get (Variables|Stats|SetOxCurent (Math|Float|Clamp(Float) (- (Variables|Stats|GetOxCurent) (* OxFall (Variables|Default|GetOxygenFallModifier))) 0.0 (Variables|Stats|GetOxMax))))
    (Default|CallOnOxChange _output_get)
    (Utilities|FlowControl|Sequence
      (:then_0
        (if (== (Variables|Stats|GetOxCurent) 0.0)
          (Default|CallOnOxRunOut)))
      (:then_1
        (return (Variables|Stats|GetOxCurent))))
    (else
      (Class|BPIDamagable|TakeDamage(Message) (Components|GetOwner) (Utilities|Struct|MakeS_DamageInfo (* OxFall 0.5) 0 false)))))

(fn AttachTank
  (params (CurrentOxygen :type Float%20%28double-precision%29) (MaxOxygen :type Float%20%28double-precision%29))
  (Variables|Stats|SetOxCurent CurrentOxygen)
  (Variables|Stats|SetOxMax MaxOxygen)
  (Variables|Default|SetbHasOxygenTank true)
  (Default|CallOnOxTankAttached (Variables|Stats|GetOxCurent) (Variables|Stats|GetOxMax)))

(fn DetachTank
  (Variables|Stats|SetOxCurent 0.0)
  (Variables|Stats|SetOxMax 0.0)
  (Variables|Default|SetbHasOxygenTank false)
  (Default|CallOnOxTankDetached))

(fn HasOxygenTank
  (return (Variables|Default|GetbHasOxygenTank)))