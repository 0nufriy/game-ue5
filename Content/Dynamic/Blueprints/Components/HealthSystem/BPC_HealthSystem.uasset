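; Actor component that tracks health, damage, healing, death and revival for its owner.
; Health starts at max, and damage, heals and optional max-health resets go through a clamped setter that broadcasts changes.
; Damage passes a macro gate for invincibility and death (reusing the CanBeHealedDead flag), firing damage and death dispatchers.
; Revive clears the dead flag and heals by max health, still subject to CanHeal.
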(event EventBeginPlay
  (Variables|Default|SetCurrentHealth (Variables|Default|GetMaxHealth)))

(event EventTick
  (params (DeltaSeconds :type Float%20%28single-precision%29)))

(fn GetMaxHealth
  (return (Variables|Default|GetMaxHealth)))

(fn GetCurrentHealth
  (return (Variables|Default|GetCurrentHealth)))

(fn Heal
  (params (HealAmount :type Float%20%28double-precision%29))
  (Utilities|FlowControl|Sequence
    (:then_0
      (if (and (Variables|Default|GetbCanHeal) (or (not (Variables|Default|GetbIsDead)) (Variables|Default|GetbCanBeHealedDead)))
        (Variables|Default|SetbIsDead false)
        (CallFunction|SetHealth (+ HealAmount (Variables|Default|GetCurrentHealth)))))
    (:then_1
      (return (Variables|Default|GetCurrentHealth)))))

(fn TakeDamage
  (params (DamageInfo :type S%20Damage%20Info%20Structure))
  (bind _damageamount (Utilities|Struct|BreakS_DamageInfo DamageInfo))
  (if (>= _damageamount 0.0)
    (Utilities|FlowControl|Sequence
      (:then_0
        (Utilities|CanbeDamaged
          (:Yes
            (CallFunction|SetHealth (- (Variables|Default|GetCurrentHealth) _damageamount))
            (Default|CallOnTakeDamage)
            (if (== (Variables|Default|GetCurrentHealth) 0.0)
              (Variables|Default|SetbIsDead true)
              (Default|CallOnDeath)))))
      (:then_1
        (return (Variables|Default|GetCurrentHealth))))))

(fn IsDead
  (return (Variables|Default|GetbIsDead)))

(fn IsInvinsible
  (return (Variables|Default|GetbIsInvincible)))

(fn SetMaxHealth
  (params (NewMaxHealth :type Float%20%28double-precision%29) (ResetCurrentHealth :type Boolean))
  (bind _output_get (Variables|Default|SetMaxHealth NewMaxHealth))
  (Default|CallOnMaxHeathUpdated _output_get)
  (if ResetCurrentHealth
    (CallFunction|SetHealth (Variables|Default|GetMaxHealth))))

(fn Revive
  (Variables|Default|SetbIsDead false)
  (CallFunction|Heal (Variables|Default|GetMaxHealth)))

(fn IsFullHP
  (return (== (Variables|Default|GetCurrentHealth) (Variables|Default|GetMaxHealth))))

(fn IsNotFullHP
  (return (not (Helpers|IsFullHP))))

(fn GetPercent
  (return (/ (Variables|Default|GetCurrentHealth) (Variables|Default|GetMaxHealth))))

(fn SetHealth
  (params (Value :type Float%20%28double-precision%29))
  (bind _maxhealth (Variables|Default|GetMaxHealth))
  (bind _returnvalue (Math|Float|Clamp(Float) Value 0.0 _maxhealth))
  (if (!= (Variables|Default|GetCurrentHealth) _returnvalue)
    (Variables|Default|SetCurrentHealth _returnvalue)
    (Default|CallOnHealthUpdated (Variables|Default|GetCurrentHealth))))