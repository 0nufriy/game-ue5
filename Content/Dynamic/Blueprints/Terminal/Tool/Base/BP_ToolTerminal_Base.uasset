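; Base tool terminal that recharges tools of a matching ammo type from the ship's shared tool ammo resource.
; Tick runs only during reload; the authority charges the item by delta time and drains the same amount from the resource manager while enough remains.
; The server multicasts resource updates and max-ammo resets to the slider UI, retrying each tick until the widget is valid.
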(event Custom|UpdateResurceMulticast
  (params (CurrentCharge :type Float%20%28double-precision%29))
  (bind _maxammo (Variables|Default|GetMaxAmmo))
  (Utilities|IsValid (Variables|Default|GetSliderTerminal) :!label _label
    (:Is%20Valid
      (if (> _maxammo 0.0)
        (Default|SetStock (Variables|Default|GetSliderTerminal) CurrentCharge _maxammo)))
    (:Is%20Not%20Valid
      (Utilities|FlowControl|DelayUntilNextTick)
      (goto _label))))

(event Custom|UpdateResource
  (params (NewAmount :type Float%20%28single-precision%29))
  (Networking|SwitchHasAuthority
    (:Authority
      (CallFunction|UpdateResurceMulticast NewAmount))))

(event Custom|ResetMaxAmmo
  (if (and (Networking|IsServer) (Ability|HasAuthority))
    (CallFunction|SetMaxAmmoMulticast (Class|FloatResourceManager|GetResource (Variables|Default|GetResourceManager)))))

(event Custom|SetMaxAmmoMulticast
  (params (MaxAmmo :type Float%20%28double-precision%29))
  (bind _sliderterminal (Variables|Default|GetSliderTerminal))
  (Variables|Default|SetMaxAmmo MaxAmmo)
  (Utilities|IsValid _sliderterminal :!label _label
    (:Is%20Valid
      (Default|SetStock _sliderterminal (Variables|Default|GetMaxAmmo) (Variables|Default|GetMaxAmmo)))
    (:Is%20Not%20Valid
      (Utilities|FlowControl|DelayUntilNextTick)
      (goto _label))))

(event EventStartItemReload
  (|CallParentFunction)
  (Actor|Tick|SetActorTickEnabled true))

(event EventStopItemReload
  (|CallParentFunction)
  (Actor|Tick|SetActorTickEnabled false))

(event EventBeginPlay
  (|CallParentFunction)
  (bind _asui_slider_terminal (Utilities|Casting|CastToUI_SliderTerminal (UserInterface|GetWidget (Variables|Default|GetTerminal%20UI))))
  (Variables|Default|SetSliderTerminal _asui_slider_terminal)
  (if (Networking|IsServer)
    (Variables|Default|SetResourceManager (Class|ShipResourcesSubsystem|GetToolAmmoManager (Subsystems|GetShipResourcesSubsystem) (Variables|Default|GetToolAmmoType)))
    (EventDispatchers|AssignOnResourceUpdated (Variables|Default|GetResourceManager) (EventDispatchers|CreateEvent :!event Custom|UpdateResource))
    (CallFunction|UpdateResource (Class|FloatResourceManager|GetResource (Variables|Default|GetResourceManager)))))

(event EventTick
  (params (DeltaSeconds :type Float%20%28single-precision%29))
  (Networking|SwitchHasAuthority
    (:Authority
      (|CallParentFunction DeltaSeconds)
      (Variables|Default|SetDelta%20Seconds DeltaSeconds)
      (CallFunction|TryCharge))))

(fn ConstructionScript)

(fn Charge
  (params (ReloadableItem :type BPI%20Reloadable%20Item%20Interface))
  (Default|AddCurrentCharge ReloadableItem (Variables|Default|GetDelta%20Seconds))
  (if (Networking|IsServer)
    (Class|FloatResourceManager|DecreaseResource (Variables|Default|GetResourceManager) (Variables|Default|GetDelta%20Seconds))))

(fn IsUsingProperAmmo
  (params (Item :type BP%20Grabbable%20Item%20Object%20Reference))
  (bind _asbp_tool (Utilities|Casting|CastToBP_Tool Item)
    (:then
      (return (Utilities|Enum|Equal(Enum) (Default|GetToolAmmoType _asbp_tool) (Variables|Default|GetToolAmmoType))))
    (:CastFailed
      (return false))))

(fn GetToolAmmoType
  (return (Variables|Default|GetToolAmmoType)))

(fn ShouldChargeItemServerOnly
  (params (Item :type BP%20Grabbable%20Item%20Object%20Reference))
  (if (>= (Class|FloatResourceManager|GetResource (Variables|Default|GetResourceManager)) (Variables|Default|GetDelta%20Seconds))
    (bind (_returnvalue _reloadableitem) (|CallParentFunction Item))
    (return _returnvalue _reloadableitem)
    (else
      (return false 0))))