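; Base weapon terminal that recharges weapons of a matching ammo type from the ship's shared ammo reserve.
; The server binds to the ammo manager for its weapon type and multicasts stock updates to the number widget, retrying next tick until the widget is valid.
; Reloading runs a looping timer, while overrides check ammo type and available stock, add charge, and deduct the reserve on the server.
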(event Custom|UpdateResurceMulticast
  (params (Ammo :type Integer))
  (bind _numberterminal (Variables|Default|GetNumberTerminal))
  (Utilities|IsValid _numberterminal :!label _label
    (:Is%20Valid
      (Default|SetStock _numberterminal Ammo))
    (:Is%20Not%20Valid
      (Utilities|FlowControl|DelayUntilNextTick)
      (goto _label))))

(event Custom|UpdateResource
  (params (NewAmount :type Integer))
  (Networking|SwitchHasAuthority
    (:Authority
      (CallFunction|UpdateResurceMulticast NewAmount))))

(event EventStartItemReload
  (|CallParentFunction)
  (bind _returnvalue (Utilities|Time|SetTimerbyEvent (EventDispatchers|CreateEvent :!event TryCharge) 0.2 true))
  (Variables|Default|SetReloadTimerHandle _returnvalue))

(event EventStopItemReload
  (|CallParentFunction)
  (Utilities|Time|ClearandInvalidateTimerbyHandle (Variables|Default|GetReloadTimerHandle)))

(event EventBeginPlay
  (|CallParentFunction)
  (bind _asui_number_terminal (Utilities|Casting|CastToUI_NumberTerminal (UserInterface|GetWidget (Variables|Default|GetTerminal%20UI))))
  (Variables|Default|SetNumberTerminal _asui_number_terminal)
  (if (Networking|IsServer)
    (Variables|Default|SetResourceManager (Class|ShipResourcesSubsystem|GetWeaponAmmoManager (Subsystems|GetShipResourcesSubsystem) (Variables|Default|GetWeapon)))
    (EventDispatchers|BindEventtoOnResourceUpdated (Variables|Default|GetResourceManager) (EventDispatchers|CreateEvent :!event Custom|UpdateResource))
    (CallFunction|UpdateResource (Class|ResourceManager|GetResource (Variables|Default|GetResourceManager)))))

(fn ConstructionScript)

(fn IsUsingProperAmmo
  (params (Item :type BP%20Grabbable%20Item%20Object%20Reference))
  (bind _asbp_weapon (Utilities|Casting|CastToBP_Weapon Item)
    (:then
      (return (Utilities|Enum|Equal(Enum) (Default|GetAmmoType _asbp_weapon) (Variables|Default|GetWeapon))))
    (:CastFailed
      (return false))))

(fn Charge
  (params (ReloadableItem :type BPI%20Reloadable%20Item%20Interface))
  (bind _rechargepower (Variables|Default|GetRechargePower))
  (Default|AddCurrentCharge ReloadableItem _rechargepower)
  (if (Networking|IsServer)
    (Class|ResourceManager|DecreaseResource (Variables|Default|GetResourceManager) (Math|Float|Truncate _rechargepower))))

(fn ShouldChargeItemServerOnly
  (params (Item :type BP%20Grabbable%20Item%20Object%20Reference))
  (if (>= (Class|ResourceManager|GetResource (Variables|Default|GetResourceManager)) (Variables|Default|GetRechargePower))
    (bind (_returnvalue _reloadableitem) (|CallParentFunction Item))
    (return _returnvalue _reloadableitem)))