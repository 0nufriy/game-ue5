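; Base wall or world terminal that recharges the reloadable item a nearby player is holding, with sound and blinking UI feedback.
; Use button events route through the player controller in multiplayer or run directly otherwise.
; TryCharge checks player range, ammo match and remaining capacity, then multicasts charge and sound.
; IsUsingProperAmmo returns false and StartItemReload is empty here; light-break events toggle UI blinking.
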(event Custom|TryCharge
  (bind _player (Class|BPIWidgetSetPlayer|GetPlayer(Message) (UserInterface|GetWidget (Variables|Default|GetTerminal%20UI))))
  (if (and (Utilities|IsValid _player) (CallFunction|IsinSuitableRange _player))
    (bind _grabbed_item (Variables|/Game/Dynamic/Blueprints/BP_PlayerCharacter.BP_PlayerCharacter_C|GetGrabbed%20Item _player)
      (:then
        (bind (_returnvalue _reloadableitem) (CallFunction|ShouldChargeItemServerOnly _grabbed_item))
        (if _returnvalue
          (if (Audio|Components|Audio|IsPlaying (Variables|Default|GetTerminalCharge))
            _
            (else
              (CallFunction|StartSoundMulticast)))
          (CallFunction|ChargeMulticast _reloadableitem)
          (else
            (CallFunction|StopSoundMulticast))))
      (:else))
    (else
      (CallFunction|StopSoundMulticast))))

(event Custom|StartItemReload)

(event Custom|StopItemReloadLocal
  (bind _ismultiplayer (Class|BPIMultiplayer|GetIsMultiplayer(Message) (Game|GetGameInstance)))
  (if _ismultiplayer
    (Class|BPIController|StopReload(Message) (Game|GetPlayerController 0) self)
    (else
      (CallFunction|StopItemReload))))

(event Custom|StopItemReload
  (CallFunction|StopSoundMulticast))

(event Custom|StopBlim
  ;[1 1 1] Blimming
  (Default|StopBlinking (Variables|Default|GetAs%20UI%20Terminal)))

(event Custom|StartBlim
  ;[1 1 1] Blimming
  (Default|StartBlinking (Variables|Default|GetAs%20UI%20Terminal) (Variables|Default|GetTerminalBlim)))

(event Custom|StopChargeSound
  (Audio|Components|Audio|Stop (Variables|Default|GetTerminalCharge)))

(event Custom|StopSoundMulticast
  (CallFunction|StopChargeSound))

(event Custom|StartSoundMulticast
  (Audio|Components|Audio|Play (Variables|Default|GetTerminalCharge) 0.0))

(event Custom|ChargeMulticast
  (params (ReloadableItem :type BPI%20Reloadable%20Item%20Interface))
  (CallFunction|Charge ReloadableItem))

(event Custom|StartItemRelodLocal
  (bind _ismultiplayer (Class|BPIMultiplayer|GetIsMultiplayer(Message) (Game|GetGameInstance)))
  (if _ismultiplayer
    (Class|BPIController|StartReload(Message) (Game|GetPlayerController 0) self)
    (else
      (CallFunction|StartItemReload))))

(event EventBeginPlay
  (bind _terminalui (Class|BPIHasTerminalUI|GetTerminalUI(Message) (UserInterface|GetWidget (Variables|Default|GetTerminal%20UI))))
  (Utilities|IsValid _terminalui
    (:Is%20Valid
      (bind _output_get (Variables|Default|SetAs%20UI%20Terminal _terminalui))
      (EventDispatchers|BindEventtoOnPressed (Variables|/Game/Dynamic/Blueprints/UI/InteractInWorld/Terminal/UI_Terminal.UI_Terminal_C|GetUseButton _output_get) (EventDispatchers|CreateEvent :!event Custom|StartItemRelodLocal))
      (EventDispatchers|BindEventtoOnReleased (Variables|/Game/Dynamic/Blueprints/UI/InteractInWorld/Terminal/UI_Terminal.UI_Terminal_C|GetUseButton _output_get) (EventDispatchers|CreateEvent :!event Custom|StopItemReloadLocal))
      (Variables|/Game/Dynamic/Blueprints/UI/InteractInWorld/Terminal/UI_Terminal.UI_Terminal_C|SetLight (Variables|Default|GetAs%20UI%20Terminal) (Variables|Default|GetDisplayLight))
      (Variables|/Game/Dynamic/Blueprints/UI/InteractInWorld/Terminal/UI_Terminal.UI_Terminal_C|SetResourceNameText (Variables|Default|GetAs%20UI%20Terminal) (Variables|Default|GetAmmoTypeName)))))

(event EventHugeLightBreakStart
  ;[1 1 1] Breaks
  (CallFunction|StartBlim))

(event EventHugeLightBreakStop
  ;[1 1 1] Breaks
  (CallFunction|StopBlim))

(event EventSmallLightBreakStop
  ;[1 1 1] Breaks
  (CallFunction|StopBlim))

(fn ConstructionScript)

(fn ShouldChargeItemServerOnly
  (params (Item :type BP%20Grabbable%20Item%20Object%20Reference))
  (if (CallFunction|IsUsingProperAmmo Item)
    (bind _asbpi_reloadable_item (Utilities|Casting|CastToBPI_ReloadableItem Item)
      (:then
        (LocalVariables|SetAs%20ReloadableItem _asbpi_reloadable_item)
        (bind _returnvalue (Default|GetMaxCharge (LocalVariables|GetAs%20ReloadableItem)))
        (bind _returnvalue_2 (Default|GetCurrentCharge (LocalVariables|GetAs%20ReloadableItem)))
        (return (< _returnvalue_2 _returnvalue) (LocalVariables|GetAs%20ReloadableItem)))
      (:CastFailed
        (return false 0)))
    (else
      (return false 0))))

(fn IsinSuitableRange
  (params (ItemToFind :type Actor%20Object%20Reference%20%28by%20ref%29))
  (return (Utilities|Array|ContainsItem (Collision|GetOverlappingActors (Variables|Default|GetCharacterCheckBox) 0 :!class /Script/Engine.PrimitiveComponent) ItemToFind)))

(fn IsUsingProperAmmo
  (params (Item :type BP%20Grabbable%20Item%20Object%20Reference))
  (return false))

(fn Charge
  (params (ReloadableItem :type BPI%20Reloadable%20Item%20Interface))
  (Default|AddCurrentCharge ReloadableItem 1.0))