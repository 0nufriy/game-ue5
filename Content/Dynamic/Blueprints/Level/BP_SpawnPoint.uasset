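; BP_SpawnPoint is a level marker for an enemy spawn, previewing the selected Enemy class with a skeletal mesh.
; The construction script picks a Kraken, Alien or default Raptor mesh and shrinks the whole actor for the Kraken.
; BeginPlay clears the mesh, so the preview is absent during play.
; GetEnemyTransform returns the mesh component's world transform, which carries that scale.
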(event EventBeginPlay
  (Variables|/Script/Engine.SkeletalMeshComponent|SetSkeletalMeshAsset (Variables|Default|GetSkeletalMesh) 0))

(fn ConstructionScript
  (bind _enemy (Variables|Enemy|GetEnemy))
  (bind _returnvalue (== _enemy "/Game/Dynamic/Enemies/Kraken/BP_Enemy_Kraken.BP_Enemy_Kraken_C"))
  (Variables|/Script/Engine.SkeletalMeshComponent|SetSkeletalMeshAsset (Variables|Default|GetSkeletalMesh) (select _returnvalue "/Game/Static/Enemies/Kraken/Meshes/KRAKEN.KRAKEN" (select (== (Variables|Enemy|GetEnemy) "/Game/Dynamic/Enemies/Alien/BP_Enemy_Alien.BP_Enemy_Alien_C") "/Game/Static/Enemies/Alien/Meshes/alien_RM.alien_RM" "/Game/Static/Enemies/Raptor/Meshes/SKM_Raptor.SKM_Raptor")))
  (Transformation|SetActorScale3D (Math|Vector|SelectVector "0.045000,0.045000,0.045000" "1.000000,1.000000,1.000000" _returnvalue)))

(fn GetEnemyTransform
  (return (Transformation|GetWorldTransform (Variables|Default|GetSkeletalMesh))))