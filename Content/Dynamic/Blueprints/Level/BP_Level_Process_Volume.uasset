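; Level manager that runs the ship's round loop, alternating timed shop breaks with rounds whose progress follows the two engines' speeds.
; During rounds the server randomly damages modules or opens holes, and spawns alien and raptor enemies as rounds start.
; Finishing the last round wins and all players dying loses, multicasting a results screen with run stats.
; Progress and shop countdown reach HUDs through RepNotifies or direct server updates.
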(event Custom|SetEngine
  (params (FirstEngine :type Boolean) (EngineMultiply :type Float%20%28double-precision%29))
  (if FirstEngine
    (Variables|Engine|SetEngine%201%20Speed EngineMultiply)
    (else
      (Variables|Engine|SetEngine%202%20Speed EngineMultiply))))

(event Custom|OnPlayerDeath
  (params (Player :type BP%20Player%20Character%20Object%20Reference))
  ;[0 0 0] Players Setup and Round Start
  (if (CallFunction|IsAllDead)
    (CallFunction|Win "lose!")))

(event Custom|Disconect
  (params (Player :type BP%20Player%20Character%20Object%20Reference))
  ;[0 0 0] Players Setup and Round Start
  (Utilities|Array|RemoveItem (Variables|Default|GetPlayers) Player)
  (if (CallFunction|IsAllDead)
    (CallFunction|Win "lose!")))

(event Custom|Start%20Round
  ;[0.01562 0.01562 0.01562] Rounds
  (Variables|Round|SetbIsRoundPlaying true)
  (Variables|Round|SetCurrent%20Round (+ (Variables|Round|GetCurrent%20Round) 1))
  (Default|CallOnRoundStart (Variables|Round|GetCurrent%20Round))
  (CallFunction|UpdateShoppingStateonUIMulticast false)
  (Actor|Tick|SetActorTickEnabled true)
  (Utilities|FlowControl|Delay (Variables|Breaks|GetRound%20Start%20Delay%20between%20Breaks))
  (if (Variables|Round|GetbIsRoundPlaying) :!label _label
    (if (Math|Random|RandomBool)
      (CallFunction|BreakModule)
      (else
        (CallFunction|CreateHole)))
    (Utilities|FlowControl|Delay (Math|Random|RandomFloatinRange (Variables|Breaks|GetMin%20Delay%20between%20Breaks) (Variables|Breaks|GetMax%20Delay%20between%20Breaks)))
    (goto _label)))

(event Custom|StartOnLessPlayer
  (Utilities|FlowControl|Delay 1.8e+02)
  (CallFunction|SetPlayerCountCurrent))

(event Custom|Win
  (params (Text :type Text))
  ;[0 0 0] WIN
  (CallFunction|WinMulticast Text (CallFunction|GetStats)))

(event Custom|ChangeTimeToSHop
  ;[0.01562 0.01562 0.01562] Rounds
  ;;[0 0 0] Shopping
  (Variables|Shop|SetTimeToShopCurrent (- (Variables|Shop|GetTimeToShopCurrent) 1))
  (bind _ismultiplayer (Class|BPIMultiplayer|GetIsMultiplayer(Message) (Game|GetGameInstance)))
  (if _ismultiplayer
    _
    (else
      (CallFunction|UpdateShoppingTimeonUiLocally)))
  (if (<= (Variables|Shop|GetTimeToShopCurrent) 0)
    (Utilities|Time|ClearandInvalidateTimerbyHandle (Variables|Shop|GetShopCounter))
    (CallFunction|StartRound)))

(event Custom|SetPlayerCountCurrent
  (bind _asbp_game_instance (Utilities|Casting|CastToBP_GameInstance (Game|GetGameInstance)))
  (bind _outactors (Actor|GetAllActorsOfClass "/Game/Dynamic/Blueprints/BP_PlayerCharacter.BP_PlayerCharacter_C"))
  (Default|SetPlayerCount _asbp_game_instance (Utilities|Array|Length _outactors))
  (Networking|SwitchHasAuthority
    (:Authority
      (bind _asbp_first_person_game_mode (Utilities|Casting|CastToBP_FirstPersonGameMode (Game|GetGameMode)))
      (Default|CheckControllersInitialized _asbp_first_person_game_mode))))

(event Custom|Update%20Shopping%20State%20on%20UI%20Multicast
  (params (Shop :type Boolean))
  ;[0.01562 0.01562 0.01562] Rounds
  ;;[0 0 0] Shopping
  (bind _ismultiplayer (Class|BPIMultiplayer|GetIsMultiplayer(Message) (Game|GetGameInstance)))
  (if _ismultiplayer
    (Class|BPIHUD|ChangeResultShop(Message) (HUD|GetHUD (Game|GetPlayerController 0)) Shop)
    (else
      (for _array_element (Variables|Default|GetPlayers)
        (bind _controller (Default|GetPlayerController _array_element))
        (Utilities|IsValid _controller
          (:Is%20Valid
            (Class|BPIHUD|ChangeResultShop(Message) (HUD|GetHUD _controller) Shop)))))))

(event Custom|Update%20Shopping%20Time%20on%20UI%20Locally
  ;[0.01562 0.01562 0.01562] Rounds
  ;;[0 0 0] Shopping
  (for _array_element (Variables|Default|GetPlayers)
    (bind _controller (Default|GetPlayerController _array_element))
    (Class|BPIHUD|SetShopTime(Message) (HUD|GetHUD _controller) (Variables|Shop|GetTimeToShopCurrent))))

(event Custom|WinMulticast
  (params (Text :type Text) (Stat :type S%20Result%20Stat%20Structure))
  ;[0 0 0] WIN
  (Utilities|FlowControl|DoOnce false
    (:Completed
      (bind _returnvalue (UserInterface|CreateWidget "/Game/Dynamic/Blueprints/UI/WinScreen/UI_Win.UI_Win_C" (Game|GetPlayerController 0) Text Stat))
      (UserInterface|Viewport|AddtoViewport _returnvalue 0))))

(event Custom|DeactivateShop
  (params (Round :type Integer))
  ;[0.01042 0.01042 0.01042] Setup Shop
  (Default|Deactivate (Variables|Shop|GetShop)))

(event Custom|ActivateShop
  (params (Round :type Integer))
  ;[0.01042 0.01042 0.01042] Setup Shop
  (Default|Activate (Variables|Shop|GetShop) Round))

(event Custom|TrySpawnAlien
  (params (Round :type Integer))
  ;[0.01042 0.01042 0.01042] EnemiesSpawn
  (if (>= Round 1)
    (Game|SpawnActorfromClass "/Game/Dynamic/Enemies/Alien/BP_Enemy_Alien.BP_Enemy_Alien_C" (Math|Transform|MakeTransform (Transformation|GetActorLocation (Variables|Enemies|GetAlienSpawnPoint)) "0, 0, 0" "1.000000,1.000000,1.000000") "Undefined" "MultiplyWithRoot" 0 0)))

(event Custom|TrySpawnRaptor
  (params (Round :type Integer))
  ;[0.01042 0.01042 0.01042] EnemiesSpawn
  (if (>= Round 2)
    (Game|SpawnActorfromClass "/Game/Dynamic/Enemies/Raptor/BP_Enemy_Raptor.BP_Enemy_Raptor_C" (Math|Transform|MakeTransform (Transformation|GetActorLocation (Variables|Enemies|GetRaptorSpawnPoint)) "0, 0, 0" "1.000000,1.000000,1.000000") "Undefined" "MultiplyWithRoot" 0 0)))

(event Custom|OnAllPlayersLoaded
  (params (Characters :type Array%20of%20BP%20Player%20Character%20Object%20References))
  ;[0 0 0] Players Setup and Round Start
  (CallFunction|SetupPlayers Characters)
  (EventDispatchers|UnbindEventfromOnAllCharactersLoaded (stale EventBeginPlay _asbp_main_game_state) (delegate Custom|OnAllPlayersLoaded))
  (CallFunction|StartRound))

(event Custom|SetupPlayers
  (params (Players :type Array%20of%20BP%20Player%20Character%20Object%20References))
  ;[0 0 0] Players Setup and Round Start
  (bind _output_get (Variables|Default|SetPlayers Players))
  (for _array_element _output_get
    (EventDispatchers|BindEventtoOnDeath _array_element (delegate Custom|OnPlayerDeath))
    (EventDispatchers|BindEventtoOnDisconect _array_element (delegate Custom|Disconect))))

(event Custom|Update%20Round%20Progress%20on%20HUD%20Locally
  (for _array_element (Variables|Default|GetPlayers)
    (bind _controller (Default|GetPlayerController _array_element))
    (Utilities|IsValid _controller
      (:Is%20Valid
        (Class|BPIHUD|SetResult(Message) (HUD|GetHUD _controller) (/ (Variables|Round|GetRound%20Progress) (Variables|Round|GetRound%20Length)))))))

(event Custom|Break%20Module
  (bind _moudls (CallFunction|GetAllAvaibleModuls))
  (bind _outitem (Utilities|Array|Random _moudls))
  ;[1 1 1] Breaks
  (Utilities|IsValid _outitem
    (:Is%20Valid
      (CallFunction|BrokenModulMulticast (Utilities|Struct|MakeS_DamageInfo (Math|Random|RandomFloatinRange (Variables|Breaks|GetMin%20Damage%20to%20Module) (Variables|Breaks|GetMax%20Damage%20to%20Module)) "/Engine/EngineDamageTypes/DmgTypeBP_Environmental.DmgTypeBP_Environmental_C" false) _outitem)
      (Variables|Stat|SetBreaksCount (+ (Variables|Stat|GetBreaksCount) 1)))))

(event Custom|Create%20Hole
  (bind _hole (CallFunction|GetAllAvaibleHole))
  (bind _outitem (Utilities|Array|Random _hole))
  ;[1 1 1] Breaks
  (Utilities|IsValid _outitem
    (:Is%20Valid
      (CallFunction|ActiveHoleMulticast _outitem)
      (Variables|Stat|SetBreaksCount (+ (Variables|Stat|GetBreaksCount) 1)))))

(event Custom|ActiveHoleMulticast
  (params (Hole :type BP%20Hole%20Object%20Reference))
  ;[1 1 1] Breaks
  (Default|SetActive Hole true))

(event Custom|BrokenModulMulticast
  (params (DamageInfo :type S%20Damage%20Info%20Structure) (Module :type BP%20Modul%20Base%20Object%20Reference))
  ;[1 1 1] Breaks
  (Default|TakeDamage Module DamageInfo))

(event Custom|End%20Round
  ;[0.01562 0.01562 0.01562] Rounds
  (Variables|Round|SetbIsRoundPlaying false)
  (Actor|Tick|SetActorTickEnabled false)
  (Variables|Round|SetRound%20Progress 0.0)
  (Default|CallOnRoundEnd (Variables|Round|GetCurrent%20Round))
  (if (== (Variables|Round|GetCurrent%20Round) (Variables|Round|GetRoundCount))
    (CallFunction|Win "win!")
    (else
      (CallFunction|UpdateShoppingStateonUIMulticast true)
      (Variables|Shop|SetTimeToShopCurrent (Variables|Shop|GetTimeToShopMax))
      (bind _returnvalue (Utilities|Time|SetTimerbyEvent (EventDispatchers|CreateEvent :!event Custom|ChangeTimeToSHop) 1.0 true))
      (Variables|Shop|SetShopCounter _returnvalue)
      (bind _ismultiplayer (Class|BPIMultiplayer|GetIsMultiplayer(Message) (Game|GetGameInstance)))
      (if (not _ismultiplayer)
        (CallFunction|UpdateShoppingTimeonUiLocally)))))

(event EventBeginPlay
  (Utilities|FlowControl|Sequence
    (:then_0
      ;[0.01042 0.01042 0.01042] Setup Shop
      (bind _returnvalue (Actor|GetActorOfClass "/Game/Dynamic/Shop/BP_Shop.BP_Shop_C"))
      (bind _output_get (Variables|Shop|SetShop _returnvalue))
      (Utilities|IsValid _output_get
        (:Is%20Valid
          (Networking|SwitchHasAuthority
            (:Authority
              (EventDispatchers|BindEventtoOnRoundStart (EventDispatchers|CreateEvent :!event Custom|DeactivateShop))
              (EventDispatchers|BindEventtoOnRoundEnd (EventDispatchers|CreateEvent :!event Custom|ActivateShop)))))))
    (:then_1
      (Networking|SwitchHasAuthority
        (:Authority
          (Utilities|FlowControl|Sequence
            (:then_0
              (bind _outactors (Actor|GetAllActorsOfClass "/Game/Dynamic/Blueprints/Mechanisms/Moduls/BP_Engine.BP_Engine_C"))
              (for _array_element _outactors
                (EventDispatchers|BindEventtoSetEngineonLevel _array_element (delegate Custom|SetEngine))))
            (:then_1
              (bind _outactors_2 (Actor|GetAllActorsOfClass "/Game/Dynamic/Blueprints/Mechanisms/Moduls/BP_ModulBase.BP_ModulBase_C"))
              (Variables|Default|SetModuls _outactors_2))
            (:then_2
              (bind _outactors_3 (Actor|GetAllActorsOfClass "/Game/Dynamic/Blueprints/Mechanisms/Hole/BP_Hole.BP_Hole_C"))
              (Variables|Default|SetHoles _outactors_3))
            (:then_3
              (Networking|SwitchHasAuthority
                (:Authority
                  (bind _asbp_first_person_game_mode (Utilities|Casting|CastToBP_FirstPersonGameMode (Game|GetGameMode)))
                  (EventDispatchers|BindEventtoOnRevive _asbp_first_person_game_mode (EventDispatchers|CreateEvent :!event IncrementReviveCount)))))
            (:then_4
              (CallFunction|StartonLessPlayer))
            (:then_5
              ;[0 0 0] Players Setup and Round Start
              (bind _asbp_main_game_state (Utilities|Casting|CastToBP_MainGameState (Game|GetGameState)))
              (bind _returnvalue_2 (Default|AllPlayersLoaded _asbp_main_game_state))
              (if _returnvalue_2
                (CallFunction|SetupPlayers (Variables|/Game/Dynamic/Blueprints/BP_MainGameState.BP_MainGameState_C|GetPlayerCharacters _asbp_main_game_state))
                (CallFunction|StartRound)
                (else
                  (EventDispatchers|BindEventtoOnAllCharactersLoaded _asbp_main_game_state (delegate Custom|OnAllPlayersLoaded)))))
            (:then_6
              ;[0.01042 0.01042 0.01042] EnemiesSpawn
              (Utilities|FlowControl|Sequence
                (:then_0
                  (Utilities|IsValid (Variables|Enemies|GetAlienSpawnPoint)
                    (:Is%20Valid
                      (EventDispatchers|BindEventtoOnRoundStart (EventDispatchers|CreateEvent :!event Custom|TrySpawnAlien)))))
                (:then_1
                  (Utilities|IsValid (Variables|Enemies|GetRaptorSpawnPoint)
                    (:Is%20Valid
                      (EventDispatchers|BindEventtoOnRoundStart (EventDispatchers|CreateEvent :!event Custom|TrySpawnRaptor)))))))))))))

(event EventTick
  (params (DeltaSeconds :type Float%20%28single-precision%29))
  ;[0 0 0] Tick
  (Networking|SwitchHasAuthority
    (:Authority
      (Variables|Round|SetRound%20Progress (+ (* (+ (Variables|Engine|GetEngine%201%20Speed) (Variables|Engine|GetEngine%202%20Speed)) (/ DeltaSeconds 2.0)) (Variables|Round|GetRound%20Progress)))
      (bind _ismultiplayer (Class|BPIMultiplayer|GetIsMultiplayer(Message) (Game|GetGameInstance)))
      (if _ismultiplayer
        (CallFunction|UpdateRoundProgressonHUDLocally))
      (if (>= (Variables|Round|GetRound%20Progress) (Variables|Round|GetRound%20Length))
        (CallFunction|EndRound)))))

(fn ConstructionScript
  (Variables|Shop|SetTimeToShopCurrent (Variables|Shop|GetTimeToShopMax)))

(fn GetAllAvaibleModuls
  (for _array_element (Variables|Default|GetModuls)
    (bind _isdead (Class|BPIDamagable|IsDead(Message) _array_element))
    (if (not (or _isdead (Variables|/Game/Dynamic/Blueprints/Mechanisms/Moduls/BP_ModulBase.BP_ModulBase_C|GetIsDrop _array_element)))
      (Utilities|Array|Add (LocalVariables|GetArray) _array_element)))
  (return (LocalVariables|GetArray)))

(fn GetAllAvaibleHole
  (for _array_element (Variables|Default|GetHoles)
    (if (not (Variables|/Game/Dynamic/Blueprints/Mechanisms/Hole/BP_Hole.BP_Hole_C|GetActive _array_element))
      (Utilities|Array|Add (LocalVariables|GetArray) _array_element)))
  (return (LocalVariables|GetArray)))

(fn OnRepTimetoShopCurrent
  (bind _returnvalue (Game|GetPlayerController 0))
  (Utilities|IsValid _returnvalue
    (:Is%20Valid
      (Class|BPIHUD|SetShopTime(Message) (HUD|GetHUD _returnvalue) (Variables|Shop|GetTimeToShopCurrent)))))

(fn IsAllDead
  (for _array_element (Variables|Default|GetPlayers)
    (bind _isdead (Default|IsDead _array_element))
    (if (not _isdead)
      (return false)))
  (return true))

(fn GetStats
  (Utilities|FlowControl|Sequence
    (:then_0
      (bind _outactors (Actor|GetAllActorsOfClass "/Game/Dynamic/Blueprints/Mechanisms/BoxColision/BP_ModulBoxColision.BP_ModulBoxColision_C"))
      (for _array_element _outactors
        (if (not (Variables|/Game/Dynamic/Blueprints/Mechanisms/BoxColision/BP_ModulBoxColision.BP_ModulBoxColision_C|GetIsDrop _array_element))
          (LocalVariables|SetShipModulBoxCoubt (+ (LocalVariables|GetShipModulBoxCoubt) 1)))))
    (:then_1
      (for _array_element_2 (Variables|Default|GetPlayers)
        (bind _isdead (Default|IsDead _array_element_2))
        (if (not _isdead)
          (LocalVariables|SetPlayer (+ (LocalVariables|GetPlayer) 1)))))
    (:then_2
      (return (Utilities|Struct|MakeS_ResultStat (Class|ResourceManager|GetResource (Class|ShipResourcesSubsystem|GetMoneyManager (Subsystems|GetShipResourcesSubsystem))) (LocalVariables|GetShipModulBoxCoubt) (Variables|Stat|GetBreaksCount) (LocalVariables|GetPlayer) (Variables|Stat|GetReviveCount) (Utilities|Array|Length (Variables|Default|GetPlayers)) (Variables|Round|GetCurrent%20Round))))))

(fn IncrementReviveCount
  (Variables|Stat|SetReviveCount (+ (Variables|Stat|GetReviveCount) 1)))

(fn OnRepRoundProgress
  (Class|BPIHUD|SetResult(Message) (HUD|GetHUD (Game|GetPlayerController 0)) (/ (Variables|Round|GetRound%20Progress) (Variables|Round|GetRound%20Length))))