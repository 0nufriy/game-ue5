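; Generated dynamic mesh actor that copies a static mesh and lets named holes be added, resized and removed at runtime.
; MakeHole subtracts a box from the main mesh and gives each hole its own component, holding a cached box-intersection cutout minus a low-poly hole shape.
; SetHoleRadius rebuilds only that hole's component from the cutout, avoiding a main-mesh rebuild.
; RemoveHole pools the component for reuse, then resets the main mesh and re-cuts the remaining holes.
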(event Custom|MAKE%20HOLES
  (CallFunction|RefreshMainDM)
  (bind _values (Utilities|Map|Values (Variables|Default|GetHoles)))
  (for _array_element _values
    (CallFunction|ApplyHoletoMainMesh (Utilities|Struct|BreakS_HoleData _array_element))))

(event Custom|RefreshMainDM
  (DynamicMesh|Reset (Variables|Default|GetMainDM))
  (CallFunction|AppendStaticMesh))

(event Events|EventOnRebuildGeneratedMesh
  (params (TargetMesh :type Dynamic%20Mesh%20Object%20Reference))
  (Variables|Default|SetMainDM TargetMesh)
  (bind _returnvalue (DynamicMeshActor|AllocateComputeMesh))
  (bind _returnvalue_2 (GeometryScript|StaticMesh|CopyMeshFromStaticMesh :FromStaticMeshAsset (Variables|Default|GetStaticMesh) :ToDynamicMesh _returnvalue :Debug 0)
    (:Success
      (Variables|Default|SetStaticMeshDM _returnvalue_2)
      (CallFunction|AppendStaticMesh))))

(event Collision|EventActorBeginOverlap
  (params (OtherActor :type Actor%20Object%20Reference)))

(event EventTick
  (params (DeltaSeconds :type Float%20%28single-precision%29)))

(event EventRemoveHole
  (params (HoleName :type String))
  (bind _holes (Variables|Default|GetHoles))
  (bind (_value _returnvalue) (Utilities|Map|Find _holes HoleName))
  (bind (_dynamicmeshcomponent _cutoutdm) (Utilities|Struct|BreakS_HoleData _value))
  (if _returnvalue
    (Utilities|Array|Add (Variables|Default|GetFreeHoleComponents) _dynamicmeshcomponent)
    (bind _returnvalue_2 (DynamicMeshComponent|GetDynamicMesh _dynamicmeshcomponent))
    (DynamicMesh|Reset _returnvalue_2)
    (Class|DynamicMeshActor|ReleaseComputeMesh _cutoutdm)
    (Utilities|Map|Remove (Variables|Default|GetHoles) HoleName)
    (CallFunction|RefreshMainDM)
    (CallFunction|ApplyHoles)))

(event EventMakeHole
  (params (HoleName :type String) (Info :type S%20Hole%20Info%20Structure))
  (bind (_holedm_component _cutoutdm) (CallFunction|CreateHoleDM Info))
  (Utilities|Map|Add (Variables|Default|GetHoles) HoleName (Utilities|Struct|MakeS_HoleData Info _holedm_component _cutoutdm))
  (CallFunction|ApplyHoletoMainMesh Info))

(event EventBeginPlay
  (Utilities|FlowControl|Sequence
    (:then_0
      (Class|DynamicMeshComponent|EnableComplexasSimpleCollision (Variables|DynamicMeshActor|GetDynamicMeshComponent))
      (Class|DynamicMeshComponent|ConfigureMaterialSet (Variables|DynamicMeshActor|GetDynamicMeshComponent) (Variables|Default|GetStaticMeshMaterials)))
    (:then_1
      (bind _returnvalue (DynamicMeshActor|AllocateComputeMesh))
      (bind _returnvalue_2 (GeometryScript|StaticMesh|CopyMeshFromStaticMesh :FromStaticMeshAsset "/Game/Dynamic/Blueprints/Mechanisms/Hole/SM_HoleLowPoly.SM_HoleLowPoly" :ToDynamicMesh _returnvalue :Debug 0)
        (:Success
          (Variables|Default|SetGeneralHoleDM _returnvalue_2))))
    (:then_2
      (if (Variables|Default|GetbAutoRebuild)
        (DynamicMeshActor|MarkforMeshRebuild true true)))
    (:then_3
      (bind _returnvalue_3 (DynamicMeshActor|AllocateComputeMesh))
      (bind _returnvalue_4 (GeometryScript|StaticMesh|CopyMeshFromStaticMesh :FromStaticMeshAsset "/Game/Dynamic/Blueprints/Mechanisms/Hole/SM_HoleBox.SM_HoleBox" :ToDynamicMesh _returnvalue_3 :Debug 0)
        (:Success
          (Variables|Default|SetCube%20Dynamic%20Mesh _returnvalue_4))))))

(event EventSetHoleRadius
  (params (HoleName :type String) (Radius :type Float%20%28double-precision%29))
  (bind _holes (Variables|Default|GetHoles))
  (bind (_value _returnvalue) (Utilities|Map|Find _holes HoleName))
  (if _returnvalue
    (bind _structout (Utilities|Struct|SetmembersinS_HoleInfo (Utilities|Struct|BreakS_HoleData _value) Radius))
    (bind _structout_2 (Utilities|Struct|SetmembersinS_HoleData _value _structout))
    (Utilities|Map|Add (Variables|Default|GetHoles) HoleName _structout_2)
    (bind _returnvalue_2 (DynamicMeshComponent|GetDynamicMesh (.DynamicMeshComponent (Utilities|Struct|BreakS_HoleData _structout_2))))
    (bind _returnvalue_3 (DynamicMesh|Reset _returnvalue_2))
    (CallFunction|UpdateHoleDM (.Info (Utilities|Struct|BreakS_HoleData _structout_2)) _returnvalue_3 (.CutoutDM (Utilities|Struct|BreakS_HoleData _structout_2)))))

(fn ConstructionScript)

(fn ApplyHoletoMainMesh
  (params (Info :type S%20Hole%20Info%20Structure))
  (bind (_radius _heightscale) (Utilities|Struct|BreakS_HoleInfo Info))
  (GeometryScript|Booleans|ApplyMeshBoolean :TargetMesh (Variables|Default|GetMainDM) :TargetTransform (Transformation|GetActorTransform) :ToolMesh (Variables|Default|GetCube%20Dynamic%20Mesh) :ToolTransform (Math|Transform|MakeTransform (Utilities|Struct|BreakS_HoleInfo Info) (CallFunction|GetHoleRotation Info) (Math|Vector|MakeVector _radius _radius _heightscale)) :Operation "Subtract" :Debug 0))

(fn AppendStaticMesh
  (GeometryScript|MeshEdits|AppendMesh :TargetMesh (Variables|Default|GetMainDM) :AppendMesh (Variables|Default|GetStaticMeshDM) :AppendOptions "(CombineMode=EnableAllMatching)" :Debug 0))

(fn ApplyHoles
  (bind _values (Utilities|Map|Values (Variables|Default|GetHoles)))
  (for _array_element _values
    (CallFunction|ApplyHoletoMainMesh (.Info (Utilities|Struct|BreakS_HoleData _array_element)))))

(fn CreateHoleDM
  (params (Info :type S%20Hole%20Info%20Structure%20%28by%20ref%29))
  (bind _returnvalue (Math|Float|MakeLiteralFloat 1.0))
  (bind _freeholecomponents (Variables|Default|GetFreeHoleComponents))
  (bind (_location _radius _heightscale) (Utilities|Struct|BreakS_HoleInfo Info))
  (if (Utilities|Array|IsEmpty _freeholecomponents)
    (bind _returnvalue_2 (AddComponent|AddDynamicMeshComponent false))
    (bind _output_get (LocalVariables|SetL_DM%20Component _returnvalue_2))
    (else
      (LocalVariables|SetL_DM%20Component (Utilities|Array|Get(acopy) _freeholecomponents))
      (Utilities|Array|RemoveIndex (Variables|Default|GetFreeHoleComponents))))
  (bind _returnvalue_3 (DynamicMeshComponent|GetDynamicMesh _output_get))
  (LocalVariables|SetL_HoleDM _returnvalue_3)
  (Class|DynamicMeshComponent|ConfigureMaterialSet (LocalVariables|GetL_DM%20Component) (Variables|Default|GetStaticMeshMaterials))
  (bind _returnvalue_4 (Game|ConstructObjectfromClass (LocalVariables|GetL_DM%20Component) "/Script/GeometryFramework.DynamicMesh"))
  (LocalVariables|SetL_CutoutDM _returnvalue_4)
  (GeometryScript|MeshEdits|AppendMesh :TargetMesh (LocalVariables|GetL_CutoutDM) :AppendMesh (Variables|Default|GetStaticMeshDM) :AppendOptions "(CombineMode=EnableAllMatching)" :Debug 0)
  (GeometryScript|Booleans|ApplyMeshBoolean :TargetMesh (LocalVariables|GetL_CutoutDM) :TargetTransform (Transformation|GetActorTransform) :ToolMesh (Variables|Default|GetCube%20Dynamic%20Mesh) :ToolTransform (Math|Transform|MakeTransform _location (CallFunction|GetHoleRotation Info) (Math|Vector|MakeVector _returnvalue _returnvalue _heightscale)) :Operation "Intersection" :Debug 0)
  (Utilities|FlowControl|Sequence
    (:then_0
      (CallFunction|UpdateHoleDM Info (LocalVariables|GetL_HoleDM) (LocalVariables|GetL_CutoutDM)))
    (:then_1
      (return (LocalVariables|GetL_DM%20Component) (LocalVariables|GetL_CutoutDM)))))

(fn GetHoleRotation
  (params (Info :type S%20Hole%20Info%20Structure%20%28by%20ref%29))
  (return (Math|Transform|TransformRotation (Math|Transform|MakeTransform "0, 0, 0" (Math|Transform|TransformRotation (Math|Transform|MakeTransform "0, 0, 0" (.rotation Info)) (Math|Rotator|MakeRotator 0.0 9e+01 0.0))) (Math|Rotator|MakeRotator 0.0 0.0 (.angle Info)))))

(fn UpdateHoleDM
  (params (Info :type S%20Hole%20Info%20Structure%20%28by%20ref%29) (HoleDM :type Dynamic%20Mesh%20Object%20Reference) (CutoutDM :type Dynamic%20Mesh%20Object%20Reference))
  (bind (_location _radius _heightscale) (Utilities|Struct|BreakS_HoleInfo Info))
  (GeometryScript|MeshEdits|AppendMesh :TargetMesh HoleDM :AppendMesh CutoutDM :AppendOptions "(CombineMode=EnableAllMatching)" :Debug 0)
  (GeometryScript|Booleans|ApplyMeshBoolean :TargetMesh HoleDM :TargetTransform (Transformation|GetActorTransform) :ToolMesh (Variables|Default|GetGeneralHoleDM) :ToolTransform (Math|Transform|MakeTransform _location (CallFunction|GetHoleRotation Info) (Math|Vector|MakeVector _radius _radius _heightscale)) :Operation "Subtract" :Debug 0))