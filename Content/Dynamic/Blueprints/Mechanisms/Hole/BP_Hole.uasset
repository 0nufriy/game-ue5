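; BP_Hole is a repairable breach that cuts holes into nearby meshes and may spawn a Kraken when activated.
; At BeginPlay it registers overlapping BP_HoleMesh actors and replaces overlapping StaticMeshActors with new ones.
; Breaking zeroes health and opens the hole via multicasts driving meshes and Niagara.
; Skill-scaled welding heals it, shrinking radius and refreshing decals until full health closes it, while tape only deactivates it temporarily.
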(event Custom|SetActiveMulticast
  (params (Active :type Boolean))
  (CallFunction|SetActive Active))

(event Custom|MakeHoleMulticast
  (params (HoleAngle :type Float%20%28double-precision%29))
  ;[0.01042 0.01042 0.01042] Hole Target
  (Variables|Default|SetHoleAngle HoleAngle)
  (Components|Activation|Activate (Variables|Default|GetNiagara) false)
  (for _array_element (Variables|Default|GetMeshManagers)
    (Default|MakeHole _array_element (CallFunction|GetName) (Utilities|Struct|MakeS_HoleInfo (Transformation|GetActorLocation) (Transformation|GetActorRotation) (Variables|Default|GetHoleAngle) (Variables|Default|GetHole%20Height%20Scale)))))

(event Custom|SetHoleRadiusMulticast
  ;[0.01042 0.01042 0.01042] Hole Target
  (Utilities|FlowControl|Sequence
    (:then_0
      (Niagara|SetNiagaraVariable(Float) (Variables|Default|GetNiagara) "RadiusPercent" (CallFunction|GetHoleRadius))
      (for _array_element (Variables|Default|GetMeshManagers)
        (Default|SetHoleRadius _array_element (CallFunction|GetName) (CallFunction|GetHoleRadius))))
    (:then_1
      (CallFunction|SpawnDecal (CallFunction|GetHoleRadius)))))

(event Custom|SetupHoleMesh
  (bind _sphere (Variables|Default|GetSphere))
  ;[0.01042 0.01042 0.01042] Hole Target
  (Utilities|FlowControl|DelayUntilNextTick)
  (bind _outactors (Collision|SphereOverlapActors (Transformation|GetWorldLocation _sphere) (Variables|/Script/Engine.SphereComponent|GetSphereRadius _sphere) (Utilities|Array|MakeArray "ObjectTypeQuery2") "/Game/Dynamic/Blueprints/Mechanisms/Hole/BP_HoleMesh.BP_HoleMesh_C"))
  (for _array_element _outactors
    (bind _asbpi_hole_target (Utilities|Casting|CastToBPI_HoleTarget _array_element))
    (Utilities|Array|AddUnique (Variables|Default|GetMeshManagers) _asbpi_hole_target))
  (for _array_element_2 (Collision|GetOverlappingActors (Variables|Default|GetSphere) "/Script/Engine.StaticMeshActor" :!class /Script/Engine.PrimitiveComponent)
    (Utilities|FlowControl|Sequence
      (:then_0
        (bind _returnvalue (Game|SpawnActorfromClass "/Game/Dynamic/Blueprints/Mechanisms/Hole/BP_HoleMesh.BP_HoleMesh_C" (Transformation|GetActorTransform _array_element_2) "Undefined" "MultiplyWithRoot" self (Variables|/Script/Engine.StaticMeshComponent|GetStaticMesh (Variables|/Script/Engine.StaticMeshActor|GetStaticMeshComponent (.AsStatic%20Mesh%20Actor (Utilities|Casting|CastToStaticMeshActor _array_element_2)))) true (Rendering|Material|GetMaterials (Variables|/Script/Engine.StaticMeshActor|GetStaticMeshComponent (.AsStatic%20Mesh%20Actor (Utilities|Casting|CastToStaticMeshActor _array_element_2)))) 0))
        (Utilities|Array|Add (Variables|Default|GetMeshManagers) _returnvalue))
      (:then_1
        (Actor|DestroyActor _array_element_2)))))

(event Custom|RemoveHoleMulticast
  ;[0.01042 0.01042 0.01042] Hole Target
  (for _array_element (Variables|Default|GetMeshManagers)
    (Default|RemoveHole _array_element (CallFunction|GetName))))

(event Custom|Set%20Active
  (params (Active :type Boolean))
  (Variables|Default|SetActive Active)
  (Networking|SwitchHasAuthority
    (:Authority
      (Utilities|FlowControl|Sequence
        (:then_0
          (Collision|SetCollisionResponsetoChannel (Variables|Default|GetSphere) "ECC_GameTraceChannel2" (select (Variables|Default|GetActive) "ECR_Block" "ECR_Ignore")))
        (:then_1
          (Utilities|ShouldSpawnKraken
            (:True
              (CallFunction|SpawnKraken))))
        (:then_2
          (if (Variables|Default|GetActive)
            (Default|CallOnActivated)
            (else
              (Default|CallOnDeactivated))))
        (:then_3
          (Components|Activation|SetActive (Variables|Default|GetNiagara) (Variables|Default|GetActive) false))))))

(event EventBeginPlay
  (CallFunction|SetupHoleMesh))

(event EventTapeFix
  (params (Time :type Float%20%28double-precision%29))
  (Variables|Default|SetIsTape true)
  (if (Variables|Default|GetActive)
    (CallFunction|SetActiveMulticast false)
    (Utilities|FlowControl|Delay Time)
    (Variables|Default|SetIsTape false)
    (CallFunction|SetActiveMulticast true)
    (else
      (Utilities|FlowControl|Delay 0.2)
      (Variables|Default|SetIsTape false))))

(event EventHugeBreakingStart
  (Default|SetHealth (Variables|Default|GetBPC_HealthSystem) 0.0)
  (CallFunction|SetActiveMulticast true)
  (CallFunction|MakeHoleMulticast (Math|Random|RandomFloatinRange 0.0 3.6e+02)))

(event EventHugeBreakingStop
  (CallFunction|SetActiveMulticast false)
  (CallFunction|RemoveHoleMulticast))

(event EventFix
  (params (FixValue :type Float%20%28double-precision%29) (PlayerStats :type BPC%20Player%20Stats%20System%20Object%20Reference) (ToolFixModulEfficiency :type Integer) (ToolFixHoleEfficiency :type Integer))
  (bind _bpc_healthsystem (Variables|Default|GetBPC_HealthSystem))
  (if (Variables|Default|GetActive)
    (bind _fix (CallFunction|CalculateFixEfficiency FixValue PlayerStats ToolFixHoleEfficiency))
    (Default|Heal _bpc_healthsystem _fix)
    (Utilities|FlowControl|Sequence
      (:then_0
        (CallFunction|SetHoleRadiusMulticast))
      (:then_1
        (if (Default|IsFullHP _bpc_healthsystem)
          (CallFunction|HugeBreakingStop))))))

(fn ConstructionScript)

(fn SpawnKraken
  (Game|SpawnActorfromClass "/Game/Dynamic/Enemies/Kraken/BP_Enemy_Kraken.BP_Enemy_Kraken_C" (Math|Transform|MakeTransform (+ (Transformation|GetActorLocation) (* (Math|Vector|GetForwardVector (Variables|Default|GetSpawnDirection)) 100)) (Math|Rotator|MakeRotator 0.0 0.0 (.yaw (Transformation|GetActorRotation))) "1.000000,1.000000,1.000000") "Undefined" "MultiplyWithRoot" 0 0))

(fn GetHoleRadius
  (return (Math|Float|Max(Float) (- 1.0 (Default|GetPercent (Variables|Default|GetBPC_HealthSystem))) (Variables|Default|GetMinHoleSize))))

(fn SpawnDecal
  (params (Radius :type Float%20%28double-precision%29))
  (bind _returnvalue (Math|Float|MakeLiteralFloat 1e+01))
  (bind _returnvalue_2 (* Radius 22.0))
  (bind _hole_height_scale (Variables|Default|GetHole%20Height%20Scale))
  (bind _returnvalue_3 (* _returnvalue _hole_height_scale))
  (Utilities|FlowControl|Sequence
    (:then_0
      (bind _decal (Variables|Default|GetDecal)
        (:then
          (Components|DestroyComponent _decal))
        (:else)))
    (:then_1
      (bind _returnvalue_4 (Class|GameplayStatics|SpawnDecalAttached "/Game/Dynamic/Blueprints/Mechanisms/Hole/Decal/M_HoleDecal.M_HoleDecal" (Math|Vector|MakeVector _returnvalue_3 _returnvalue_2 _returnvalue_2) (Variables|Default|GetSphere) "None" (Math|Vector|MakeVector (/ _returnvalue_3 -1.0) 0.0 0.0) (Math|Rotator|CombineRotators (Math|Rotator|MakeRotator 9e+01 0.0 1.8e+02) (Math|Rotator|MakeRotator (Variables|Default|GetHoleAngle) 0.0 0.0)) "KeepRelativeOffset" 4.0))
      (bind _output_get (Variables|Default|SetDecal _returnvalue_4))
      (Rendering|Components|Decal|SetFadeOut _output_get 0.0 4.0 false))))

(fn GetName
  (return (Utilities|GetObjectName self)))

(fn CalculateFixEfficiency
  (params (FixValue :type Float%20%28double-precision%29) (PlayerStat :type BPC%20Player%20Stats%20System%20Object%20Reference) (ToolFixEfficiency :type Integer))
  (return (* FixValue (Variables|/Game/Dynamic/Blueprints/Components/StatsSystemComponent/Player/BPC_Player_StatsSystem.BPC_Player_StatsSystem_C|GetWeldSkill PlayerStat) ToolFixEfficiency)))

(fn GetHealthPercent
  (return 0.0))

(fn GetIsTape
  (return (Variables|Default|GetIsTape)))