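; BP_Fire is a networked fire node that spreads to neighbors, damages characters, and needs oxygen from its collision box to burn.
; While burning, a server timer ignites random unlit overlapping fires, and tick deals damage scaled by remaining strength.
; Short-lived extinguish pulses drain that strength, which otherwise recovers and drives effect scale and volume.
; Multicast state changes toggle effects, tick and nav modifier; stopping makes burning neighbors re-check oxygen.
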(event OnComponentBeginOverlap(ExpandColision)
  (params (OverlappedComponent :type Primitive%20Component%20Object%20Reference) (OtherActor :type Actor%20Object%20Reference) (OtherComp :type Primitive%20Component%20Object%20Reference) (OtherBodyIndex :type Integer) (bFromSweep :type Boolean) (SweepResult :type Hit%20Result%20Structure%20%28by%20ref%29))
  (Networking|SwitchHasAuthority
    (:Authority
      (bind _returnvalue (GameplayTags|HasMatchingGameplayTag(Message) OtherActor "(TagName=\"Damageable.Character\")"))
      (if _returnvalue
        (Utilities|Array|Add (Variables|Default|GetActorsToDamage) OtherActor)))))

(event OnComponentEndOverlap(ExpandColision)
  (params (OverlappedComponent :type Primitive%20Component%20Object%20Reference) (OtherActor :type Actor%20Object%20Reference) (OtherComp :type Primitive%20Component%20Object%20Reference) (OtherBodyIndex :type Integer))
  (Networking|SwitchHasAuthority
    (:Authority
      (bind _returnvalue (GameplayTags|HasMatchingGameplayTag(Message) OtherActor "(TagName=\"Damageable.Character\")"))
      (if _returnvalue
        (Utilities|Array|RemoveItem (Variables|Default|GetActorsToDamage) OtherActor)))))

(event Custom|SetFireMulticast
  (params (IsFire :type Boolean))
  ;[1 1 1] SetFire
  (bind _ox (CallFunction|IsOx))
  (bind _output_get (Variables|Default|SetIsFire? (and _ox IsFire)))
  (Actor|Tick|SetActorTickEnabled _output_get)
  (Class|NavRelevantComponent|SetNavigationRelevancy (Variables|Default|GetNavModifier) _output_get)
  (if _output_get
    (CallFunction|StartFire)
    (else
      (CallFunction|StopFire))))

(event Custom|TakeDamageMulticast
  (params (Target :type Object%20Object%20Reference) (DamageInfo :type S%20Damage%20Info%20Structure))
  ;[1 1 1] DamageCharacter
  (Class|BPIDamagable|TakeDamage(Message) Target DamageInfo))

(event Custom|SetUnExtingush
  (Variables|Default|SetIsExtingush false))

(event EventBeginPlay
  (Utilities|FlowControl|DelayUntilNextTick)
  (bind _output (CallFunction|GetOverlappingCollisionBox (Variables|Default|GetExpandColision)))
  (Variables|Default|SetCollisionBox _output))

(event Collision|EventActorBeginOverlap
  (params (OtherActor :type Actor%20Object%20Reference)))

(event EventTick
  (params (DeltaSeconds :type Float%20%28single-precision%29))
  ;[1 1 1] DamageCharacter
  (Networking|SwitchHasAuthority
    (:Authority
      (Utilities|FlowControl|Sequence
        (:then_0
          (if (Variables|Default|GetIsExtingush)
            (if (Variables|Default|GetIsFire?)
              (bind _output_get (CallFunction|SetTimetoExtingush (- (Variables|Default|GetRemainTimeToExtingush) DeltaSeconds)))
              (if (<= _output_get 0.0)
                (CallFunction|SetFire false)))
            (elif (!= (Variables|Default|GetRemainTimeToExtingush) (Variables|Default|GetTimeToExtingush))
              (CallFunction|SetTimetoExtingush (+ (* DeltaSeconds 0.4) (Variables|Default|GetRemainTimeToExtingush))))))
        (:then_1
          (for _array_element (Variables|Default|GetActorsToDamage)
            (CallFunction|TakeDamageMulticast _array_element (Utilities|Struct|MakeS_DamageInfo (* DeltaSeconds 2.5 (Variables|Default|GetRemainTimeToExtingush)) "/Engine/EngineDamageTypes/DmgTypeBP_Environmental.DmgTypeBP_Environmental_C" false))))))))

(event EventExpand
  (bind _newparam (CallFunction|GetEnableFire))
  (bind _outitem (Utilities|Array|Random _newparam))
  (if (Variables|Default|GetIsFire?)
    (Utilities|IsValid _outitem
      (:Is%20Valid
        (Class|BPIFire|SetFire(Message) _outitem true)))))

(event EventSetFire
  (params (IsFire :type Boolean))
  ;[1 1 1] SetFire
  (CallFunction|SetFireMulticast IsFire))

(fn ConstructionScript
  (Class|NavRelevantComponent|SetNavigationRelevancy (Variables|Default|GetNavModifier) false)
  (if (!= (Variables|Default|GetModuleTag) "")
    (Variables|Default|SetTags (Utilities|Array|MakeArray (Variables|Default|GetModuleTag)))))

(fn NewFunction)

(fn StartFire
  (Components|Activation|Activate (Variables|Default|GetFireFX) true)
  (Audio|Components|Audio|Play (Variables|Default|GetFire) 0.0)
  (Networking|SwitchHasAuthority
    (:Authority
      (bind _returnvalue (Utilities|Time|SetTimerbyEvent (EventDispatchers|CreateEvent :!event Expand) (Variables|Default|GetFireExpandTime) true))
      (Variables|Default|SetFireHandler _returnvalue))))

(fn StopFire
  (Components|Activation|Deactivate (Variables|Default|GetFireFX))
  (Audio|Components|Audio|Stop (Variables|Default|GetFire))
  (Networking|SwitchHasAuthority
    (:Authority
      (Utilities|Time|ClearandInvalidateTimerbyHandle (Variables|Default|GetFireHandler))
      (for _array_element (CallFunction|GetAllFire)
        (bind _isfire (Class|BPIFire|IsFire(Message) _array_element))
        (if _isfire
          (Class|BPIFire|SetFire(Message) _array_element true))))))

(fn GetEnableFire
  (LocalVariables|SetNearFires (Collision|GetOverlappingActors (Variables|Default|GetExpandColision) "BP_Fire_C" :!class /Script/Engine.PrimitiveComponent))
  (Utilities|Array|RemoveItem (LocalVariables|GetNearFires) self)
  (for _array_element (LocalVariables|GetNearFires)
    (bind _isfire (Class|BPIFire|IsFire(Message) _array_element))
    (if (not _isfire)
      (Utilities|Array|Add (LocalVariables|GetEnableNearFires) _array_element)))
  (if (Utilities|Array|IsEmpty (LocalVariables|GetEnableNearFires))
    (Utilities|Time|ClearandInvalidateTimerbyHandle (Variables|Default|GetFireHandler)))
  (return (LocalVariables|GetEnableNearFires)))

(fn GetAllFire
  (LocalVariables|SetFireArray (Collision|GetOverlappingActors (Variables|Default|GetExpandColision) "BP_Fire_C" :!class /Script/Engine.PrimitiveComponent))
  (Utilities|Array|RemoveItem (LocalVariables|GetFireArray) self)
  (return (LocalVariables|GetFireArray)))

(fn SetTimetoExtingush
  (params (RemainTimeToExtingush :type Float%20%28double-precision%29))
  (bind _output_get (Variables|Default|SetRemainTimeToExtingush (Math|Float|Clamp(Float) RemainTimeToExtingush 0.0 (Variables|Default|GetTimeToExtingush))))
  (Audio|Components|Audio|SetVolumeMultiplier (Variables|Default|GetFire) _output_get :!class /Script/Engine.AudioComponent)
  (Transformation|SetRelativeScale3D (Variables|Default|GetFireFX) (Math|Vector|MakeVector _output_get _output_get _output_get))
  (return _output_get))

(fn IsOx
  (bind _ox (Class|BPIColisionHaveOx|HaveOx(Message) (Variables|Default|GetCollisionBox)))
  (return _ox))

(fn OnRepRemainTimetoExtingush
  (bind _remaintimetoextingush (Variables|Default|GetRemainTimeToExtingush))
  (Audio|Components|Audio|SetVolumeMultiplier (Variables|Default|GetFire) _remaintimetoextingush :!class /Script/Engine.AudioComponent)
  (Transformation|SetRelativeScale3D (Variables|Default|GetFireFX) (Math|Vector|MakeVector _remaintimetoextingush _remaintimetoextingush _remaintimetoextingush)))

(fn IsFire
  (return (Variables|Default|GetIsFire?)))

(fn SetIsExtingush
  (params (IsExtingush :type Boolean))
  (Utilities|Time|ClearandInvalidateTimerbyHandle (Variables|Default|GetExtingushtimer))
  (bind _output_get (Variables|Default|SetIsExtingush IsExtingush))
  (Utilities|FlowControl|Sequence
    (:then_0
      (if _output_get
        (bind _returnvalue (Utilities|Time|SetTimerbyEvent (EventDispatchers|CreateEvent :!event Custom|SetUnExtingush) 0.3))
        (Variables|Default|SetExtingushtimer _returnvalue)))
    (:then_1
      (return _output_get))))