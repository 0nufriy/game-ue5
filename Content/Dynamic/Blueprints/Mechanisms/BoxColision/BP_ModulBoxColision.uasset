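; Box volume for one module that manages its oxygen, visibility culling and destruction.
; Holes, permanent state, corridor air and drop state determine breathability; airless modules extinguish fires, drain players' oxygen on tick and propagate changes through permanently open doors.
; The server hides filtered contents when no pawns, open doors or camera viewing require them.
; Dropping breaks the camera, deals lethal damage to contents and cascades to droppable neighbours left without available doors.
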(event OnComponentBeginOverlap(Box)
  (params (OverlappedComponent :type Primitive%20Component%20Object%20Reference) (OtherActor :type Actor%20Object%20Reference) (OtherComp :type Primitive%20Component%20Object%20Reference) (OtherBodyIndex :type Integer) (bFromSweep :type Boolean) (SweepResult :type Hit%20Result%20Structure%20%28by%20ref%29))
  (Utilities|Casting|CastToPawn OtherActor)
  (Optimize|DoOptimize)
  (if (Utilities|DoesObjectImplementInterface OtherActor "/Game/Dynamic/Interfaces/BPI_Players.BPI_Players_C")
    (bind _player (Class|BPIPlayers|GetPlayer(Message) OtherActor))
    (Utilities|Array|Add (Variables|Default|GetPlayerToOx) _player)))

(event OnComponentEndOverlap(Box)
  (params (OverlappedComponent :type Primitive%20Component%20Object%20Reference) (OtherActor :type Actor%20Object%20Reference) (OtherComp :type Primitive%20Component%20Object%20Reference) (OtherBodyIndex :type Integer))
  (Utilities|Casting|CastToPawn OtherActor)
  (Optimize|DoOptimize)
  (if (Utilities|DoesObjectImplementInterface OtherActor "/Game/Dynamic/Interfaces/BPI_Players.BPI_Players_C")
    (bind _player (Class|BPIPlayers|GetPlayer(Message) OtherActor))
    (Utilities|Array|RemoveItem (Variables|Default|GetPlayerToOx) _player)))

(event Custom|AddHole
  (params (AddedHolesNumber :type Integer))
  (Networking|SwitchHasAuthority
    (:Authority
      (bind _output_get (Variables|Modul|SetHoleCount (+ AddedHolesNumber (Variables|Modul|GetHoleCount))))
      (Default|SetBreath (Variables|Modul|GetCamera) _output_get)
      (CallFunction|AddHoleMulticast))))

(event Custom|DropOxygenMulticast
  (params (DeltaTime :type Float%20%28double-precision%29))
  (for _array_element (Variables|Default|GetPlayerToOx)
    (Class|BPIHasOxygen|DecreaseOxygen(Message) _array_element (* DeltaTime 2.0))))

(event Custom|SetOxPermanent
  (params (CanBreath :type Boolean))
  (bind _nobreath (CallFunction|IsBreathEnable))
  (Variables|Default|SetCan%20Breath CanBreath)
  (if (!= (Variables|Modul|GetNo%20Breath) _nobreath)
    (Variables|Modul|SetNo%20Breath _nobreath)
    (Actor|Tick|SetActorTickEnabled _nobreath)
    (CallFunction|SetFire _nobreath)))

(event Custom|AddHoleMulticast
  (bind _nobreath (CallFunction|IsBreathEnable))
  (if (!= (Variables|Modul|GetNo%20Breath) _nobreath)
    (Variables|Modul|SetNo%20Breath _nobreath)
    (Actor|Tick|SetActorTickEnabled _nobreath)
    (CallFunction|SetFire _nobreath)))

(event Custom|SetCoridorOx
  (params (Door :type BP%20Door%20Object%20Reference) (CoridorOX :type Boolean))
  (bind _nobreath (CallFunction|IsBreathEnable))
  (Variables|Modul|SetCoridorOx CoridorOX)
  (if (!= (Variables|Modul|GetNo%20Breath) _nobreath)
    (Variables|Modul|SetNo%20Breath _nobreath)
    (Actor|Tick|SetActorTickEnabled _nobreath)
    (CallFunction|SetFire _nobreath)
    (for _array_element (CallFunction|GetPermanentOpenDoor)
      (if (!= _array_element Door)
        (bind _coridor (Class|BPIDoor|GetCoridor(Message) _array_element))
        (bind _door (Class|BPIDoor|GetSelf(Message) _array_element))
        (Default|RecountBreathPermanent _coridor self _door)))))

(event Custom|HoleActivated
  ;[0.01042 0.01042 0.01042] Setup cameras
  (CallFunction|AddHole 1))

(event Custom|OptimizeMulticast
  (params (Hide :type Boolean))
  (Optimize|Optimize Hide)
  (for _array_element (Collision|GetOverlappingActors (Variables|Default|GetBox) "/Game/Dynamic/Blueprints/Mechanisms/Door/BP_Door.BP_Door_C" :!class /Script/Engine.PrimitiveComponent)
    (Class|BPIDoor|OptimizeCoridor(Message) _array_element)))

(event Custom|HoleDeactivated
  ;[0.01042 0.01042 0.01042] Setup cameras
  (CallFunction|AddHole -1))

(event EventBeginPlay
  (|CallParentFunction)
  (Utilities|FlowControl|Sequence
    (:then_0
      (bind _outactors (Actor|GetAllActorsOfClasswithTag "/Game/Dynamic/Blueprints/Mechanisms/Moduls/Camera/BP_Camera.BP_Camera_C" (Variables|Modul|GetCameraTag)))
      (Variables|Modul|SetCamera (Utilities|Array|Get(acopy) _outactors)))
    (:then_1
      ;[0.01042 0.01042 0.01042] Setup cameras
      (for _array_element (Collision|GetOverlappingActors (Variables|Default|GetBox) "/Game/Dynamic/Blueprints/Mechanisms/Hole/BP_Hole.BP_Hole_C" :!class /Script/Engine.PrimitiveComponent)
        (bind _asbp_hole (Utilities|Casting|CastToBP_Hole _array_element))
        (EventDispatchers|BindEventtoOnActivated _asbp_hole (delegate Custom|HoleActivated))
        (EventDispatchers|AssignOnDeactivated _asbp_hole (delegate Custom|HoleDeactivated))))
    (:then_2
      (Utilities|FlowControl|Delay 0.2)
      (Optimize|DoOptimize))))

(event EventTick
  (params (DeltaSeconds :type Float%20%28single-precision%29))
  (|CallParentFunction DeltaSeconds)
  (Networking|SwitchHasAuthority
    (:Authority
      (CallFunction|DropOxygenMulticast DeltaSeconds))))

(fn ConstructionScript
  (if (Variables|Modul|GetOxLittleBreak)
    (Variables|Default|SetTags (Utilities|Array|MakeArray (Variables|Modul|GetCameraTag) "LittleOXBreak"))
    (else
      (Variables|Default|SetTags (Utilities|Array|MakeArray (Variables|Modul|GetCameraTag))))))

(fn SetFire
  (params (bEnabled :type Boolean))
  (if bEnabled
    (for _array_element (Collision|GetOverlappingActors (Variables|Default|GetBox) "/Game/Dynamic/Blueprints/Mechanisms/Fire/BP_Fire.BP_Fire_C" :!class /Script/Engine.PrimitiveComponent)
      (Class|BPIFire|SetFire(Message) _array_element false))))

(fn Optimize
  (params (Hide :type Boolean))
  (bind _outcomponents (Collision|BoxOverlapComponents (Transformation|GetWorldLocation (Variables|Default|GetBox)) (* (Transformation|GetWorldScale (Variables|Default|GetBox)) (Variables|/Script/Engine.BoxComponent|GetBoxExtent (Variables|Default|GetBox))) (Utilities|Array|MakeArray "ObjectTypeQuery1" "ObjectTypeQuery2" "ObjectTypeQuery4" "ObjectTypeQuery5" "ObjectTypeQuery6") 0 0 :!class /Script/Engine.KismetSystemLibrary))
  (for _array_element _outcomponents
    (if (Optimize|IsAvaible _array_element)
      (Development|SetHiddeninGame _array_element Hide true))))

(fn DoOptimize
  (bind _close (Optimize|AllDoorClose))
  (bind _is_camerawatch (Variables|Optimize|GetIs%20CameraWatch))
  (bind _isdrop (Variables|Modul|GetIsDrop))
  (bind _box (Variables|Default|GetBox))
  (bind _returnvalue (not _is_camerawatch))
  (bind _overlappingactors (Collision|GetOverlappingActors _box "/Script/Engine.Pawn" :!class /Script/Engine.PrimitiveComponent))
  (bind _returnvalue_2 (Utilities|Array|Length _overlappingactors))
  (bind _returnvalue_3 (== _returnvalue_2 0))
  (bind _returnvalue_4 (Math|Boolean|ANDBoolean _returnvalue_3 _close _returnvalue))
  (bind _returnvalue_5 (or _returnvalue_4 _isdrop))
  (if (Networking|IsServer)
    (if (!= (Variables|Optimize|GetIsHideNow) _returnvalue_5)
      (bind _output_get (Variables|Optimize|SetIsHideNow _returnvalue_5))
      (CallFunction|OptimizeMulticast _output_get))))

(fn IsBreathEnable
  (return (Math|Boolean|ORBoolean (> (Variables|Modul|GetHoleCount) 0) (not (Variables|Default|GetCan%20Breath)) (not (Variables|Modul|GetCoridorOx)) (Variables|Modul|GetIsDrop))))

(fn IsAvaible
  (params (ActorComponent :type Actor%20Component%20Object%20Reference))
  (bind _returnvalue (Components|GetOwner ActorComponent))
  (bind _returnvalue_2 (Utilities|GetClass _returnvalue))
  (return (Math|Boolean|ANDBoolean (!= _returnvalue_2 "BP_ModulBoxColision_C") (!= _returnvalue_2 "/Script/Engine.BlockingVolume") (!= _returnvalue_2 "/Script/Icarus.EnemyBase") (!= _returnvalue_2 "/Game/Dynamic/Blueprints/BP_PlayerCharacter.BP_PlayerCharacter_C") (!= _returnvalue_2 "/Game/Dynamic/Blueprints/Mechanisms/BoxColision/BP_CoridorBoxColision.BP_CoridorBoxColision_C") (!= _returnvalue_2 "/Game/Dynamic/Blueprints/Mechanisms/Door/BP_CoridorMash.BP_CoridorMash_C") (!= _returnvalue_2 "/Game/Dynamic/Blueprints/Mechanisms/Door/BP_Door.BP_Door_C") (!= _returnvalue_2 "/Game/Dynamic/Blueprints/Mechanisms/Door/BP_Stair.BP_Stair_C") (!= _returnvalue_2 "/Game/Dynamic/Blueprints/Mechanisms/Door/BP_CornerCoridorMash.BP_CornerCoridorMash_C") (!= _returnvalue_2 "/Game/Dynamic/Blueprints/Mechanisms/Moduls/Camera/BP_Camera.BP_Camera_C") (!= _returnvalue_2 "/Game/Dynamic/Blueprints/Mechanisms/Hole/BP_Hole.BP_Hole_C") (!= _returnvalue_2 "/Game/Dynamic/Blueprints/Mechanisms/Fire/BP_Fire.BP_Fire_C") (not (Utilities|ClassIsChildOf _returnvalue_2 "/Game/Dynamic/Blueprints/Items/BP_GrabbableItem.BP_GrabbableItem_C")) (not (Utilities|ClassIsChildOf _returnvalue_2 "/Game/Dynamic/Blueprints/Terminal/BP_Terminal_Base.BP_Terminal_Base_C")) (!= _returnvalue_2 "/Game/Dynamic/Shop/BP_Shop.BP_Shop_C"))))

(fn AllDoorClose
  (for _array_element (Collision|GetOverlappingActors (Variables|Default|GetBox) "/Game/Dynamic/Blueprints/Mechanisms/Door/BP_Door.BP_Door_C" :!class /Script/Engine.PrimitiveComponent)
    (bind _open (Class|BPIDoor|IsOpenDoor(Message) _array_element))
    (bind _permanentopen (Class|BPIDoor|GetPermanentOpen(Message) _array_element))
    (if (or _permanentopen _open)
      (return false)))
  (return true))

(fn GetPermanentOpenDoor
  (for _array_element (Collision|GetOverlappingActors (Variables|Default|GetBox) "/Game/Dynamic/Blueprints/Mechanisms/Door/BP_Door.BP_Door_C" :!class /Script/Engine.PrimitiveComponent)
    (bind _permanentopen (Class|BPIDoor|GetPermanentOpen(Message) _array_element))
    (if _permanentopen
      (Utilities|Array|Add (LocalVariables|GetDoors) _array_element)))
  (return (LocalVariables|GetDoors)))

(fn IsAllOfPermanentDoorCanBeath
  (for _array_element (CallFunction|GetPermanentOpenDoor)
    (bind _coridor (Class|BPIDoor|GetCoridor(Message) _array_element))
    (if (not (Variables|/Game/Dynamic/Blueprints/Mechanisms/BoxColision/BP_CoridorBoxColision.BP_CoridorBoxColision_C|GetCan%20Breath_0 _coridor))
      (return false)))
  (return true))

(fn GetIsDropAvaible
  (return (Variables|Modul|GetIsDropAvaible)))

(fn Drop
  (bind _camera (Variables|Modul|GetCamera))
  (bind _securitycenter (Variables|/Game/Dynamic/Blueprints/Mechanisms/Moduls/Camera/BP_Camera.BP_Camera_C|GetSecurityCenter _camera))
  (bind _camnum (Variables|/Game/Dynamic/Blueprints/Mechanisms/Moduls/Camera/BP_Camera.BP_Camera_C|GetCamNum _camera))
  (Utilities|FlowControl|Sequence
    (:then_0
      (Variables|Modul|SetIsDropAvaible false))
    (:then_1
      (Variables|Modul|SetIsDrop true))
    (:then_2
      (Utilities|IsValid _camera
        (:Is%20Valid
          (Variables|/Game/Dynamic/Blueprints/Mechanisms/Moduls/Camera/BP_Camera.BP_Camera_C|SetRenderMaterial _camera "/Game/Dynamic/Blueprints/Mechanisms/Moduls/Camera/Material/MI_VHS_BrokenCam.MI_VHS_BrokenCam")
          (if (== _camnum (Variables|/Game/Dynamic/Blueprints/Mechanisms/Moduls/Camera/BP_SecurityCenter.BP_SecurityCenter_C|GetCurCam _securitycenter))
            (Default|SetCamonScreenbyNum _securitycenter _camnum)))))
    (:then_3
      (if (Networking|IsServer)
        (for _array_element (Collision|GetOverlappingActors (Variables|Default|GetBox) "/Game/Dynamic/Blueprints/Mechanisms/Fire/BP_Fire.BP_Fire_C" :!class /Script/Engine.PrimitiveComponent)
          (bind _isfire (Class|BPIFire|IsFire(Message) _array_element))
          (if _isfire
            (Class|BPIFire|SetFire(Message) _array_element false)))))
    (:then_4
      (for _array_element_2 (Collision|GetOverlappingActors (Variables|Default|GetBox) "/Game/Dynamic/Blueprints/Mechanisms/Door/BP_Door.BP_Door_C" :!class /Script/Engine.PrimitiveComponent)
        (Class|BPIDoor|DropModule(Message) _array_element_2)
        (bind _door (Class|BPIDoor|GetAnotherDoor(Message) _array_element_2))
        (if (and (== (CallFunction|GetDoorAvaibleCount (Variables|/Game/Dynamic/Blueprints/Mechanisms/Door/BP_Door.BP_Door_C|GetModulBox _door)) 0) (and (Variables|BP_ModulBoxColision_C|GetIsDropAvaible (Variables|/Game/Dynamic/Blueprints/Mechanisms/Door/BP_Door.BP_Door_C|GetModulBox _door)) (not (Variables|BP_ModulBoxColision_C|GetIsDrop (Variables|/Game/Dynamic/Blueprints/Mechanisms/Door/BP_Door.BP_Door_C|GetModulBox _door)))))
          (CallFunction|Drop (Variables|/Game/Dynamic/Blueprints/Mechanisms/Door/BP_Door.BP_Door_C|GetModulBox _door)))))
    (:then_5
      (bind _outcomponents (Collision|BoxOverlapComponents (Transformation|GetWorldLocation (Variables|Default|GetBox)) (* (Transformation|GetWorldScale (Variables|Default|GetBox)) (Variables|/Script/Engine.BoxComponent|GetBoxExtent (Variables|Default|GetBox))) (Utilities|Array|MakeArray "ObjectTypeQuery1" "ObjectTypeQuery2" "ObjectTypeQuery4" "ObjectTypeQuery5" "ObjectTypeQuery6") 0 0 :!class /Script/Engine.KismetSystemLibrary))
      (for _array_element_3 _outcomponents
        (if (Utilities|DoesObjectImplementInterface (Components|GetOwner _array_element_3) "/Game/Dynamic/Blueprints/Components/HealthSystem/BPI_Damagable.BPI_Damagable_C")
          (bind _asbp_modul_base (Utilities|Casting|CastToBP_ModulBase (Components|GetOwner _array_element_3))
            (:then
              (Variables|/Game/Dynamic/Blueprints/Mechanisms/Moduls/BP_ModulBase.BP_ModulBase_C|SetIsDrop _asbp_modul_base true))
            (:CastFailed
              (Utilities|Casting|CastToBP_Door (Components|GetOwner _array_element_3)
                (:CastFailed
                  _))))
          (bind _maxhealth (Class|BPIDamagable|GetMaxHealth(Message) (Components|GetOwner _array_element_3)))
          (Class|BPIDamagable|TakeDamage(Message) (Components|GetOwner _array_element_3) (Utilities|Struct|MakeS_DamageInfo _maxhealth "/Engine/EngineDamageTypes/DmgTypeBP_Environmental.DmgTypeBP_Environmental_C" false)))))
    (:then_6
      (bind _outactors (Actor|GetAllActorswithInterface "/Game/Dynamic/Blueprints/Components/HealthSystem/BPI_Damagable.BPI_Damagable_C"))
      (for _array_element_4 _outactors
        (if (and (Collision|IsOverlappingActor _array_element_4 self :!class /Script/Engine.Actor) (not (Utilities|DoesObjectImplementInterface _array_element_4 "/Game/Dynamic/Interfaces/BPI_Door.BPI_Door_C")))
          (bind _maxhealth_2 (Class|BPIDamagable|GetMaxHealth(Message) _array_element_4))
          (Class|BPIDamagable|TakeDamage(Message) _array_element_4 (Utilities|Struct|MakeS_DamageInfo _maxhealth_2 "/Engine/EngineDamageTypes/DmgTypeBP_Environmental.DmgTypeBP_Environmental_C" false)))))))

(fn GetDoorAvaibleCount
  (for _array_element (Collision|GetOverlappingActors (Variables|Default|GetBox) "/Game/Dynamic/Blueprints/Mechanisms/Door/BP_Door.BP_Door_C" :!class /Script/Engine.PrimitiveComponent)
    (bind _drop (Class|BPIDoor|GetIsDrop(Message) _array_element))
    (bind _door (Class|BPIDoor|GetAnotherDoor(Message) _array_element))
    (bind _drop_2 (Class|BPIDoor|GetIsDrop(Message) _door))
    (if (and (not _drop) (not _drop_2))
      (LocalVariables|SetC (+ (LocalVariables|GetC) 1))))
  (return (LocalVariables|GetC)))

(fn HaveOx
  (return (not (CallFunction|IsBreathEnable))))