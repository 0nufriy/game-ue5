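; Corridor volume that manages oxygen and render culling for a connecting passage between modules.
; While ticking, the authority multicasts an oxygen drain for players inside who overlap no module box.
; Door events derive breathability from the module, toggle tick and propagate permanent air state through permanently open doors.
; Pawn overlaps trigger hiding of corridor meshes, doors and stairs when it is empty and modules behind its ID-tagged doors are hidden.
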(event OnComponentBeginOverlap(Box)
  (params (OverlappedComponent :type Primitive%20Component%20Object%20Reference) (OtherActor :type Actor%20Object%20Reference) (OtherComp :type Primitive%20Component%20Object%20Reference) (OtherBodyIndex :type Integer) (bFromSweep :type Boolean) (SweepResult :type Hit%20Result%20Structure%20%28by%20ref%29))
  (Utilities|Casting|CastToPawn OtherActor)
  (CallFunction|DoOptimize)
  (if (Utilities|DoesObjectImplementInterface OtherActor "/Game/Dynamic/Interfaces/BPI_Players.BPI_Players_C")
    (bind _player (Class|BPIPlayers|GetPlayer(Message) OtherActor))
    (Utilities|Array|Add (Variables|Default|GetPlayerToOx) _player)))

(event OnComponentEndOverlap(Box)
  (params (OverlappedComponent :type Primitive%20Component%20Object%20Reference) (OtherActor :type Actor%20Object%20Reference) (OtherComp :type Primitive%20Component%20Object%20Reference) (OtherBodyIndex :type Integer))
  (Utilities|Casting|CastToPawn OtherActor)
  (CallFunction|DoOptimize)
  (if (Utilities|DoesObjectImplementInterface OtherActor "/Game/Dynamic/Interfaces/BPI_Players.BPI_Players_C")
    (bind _player (Class|BPIPlayers|GetPlayer(Message) OtherActor))
    (Utilities|Array|RemoveItem (Variables|Default|GetPlayerToOx) _player)))

(event Custom|DoorOpen
  (params (ModulBox :type BP%20Modul%20Box%20Colision%20Object%20Reference))
  (bind _nobreath (Default|IsBreathEnable ModulBox))
  (bind _permanentbreath (Variables|Modul|GetPermanentBreath))
  (bind _returnvalue (not _permanentbreath))
  (bind _returnvalue_2 (or _nobreath _returnvalue))
  (Variables|Default|SetCan%20Breath (not _returnvalue_2))
  (Actor|Tick|SetActorTickEnabled _returnvalue_2))

(event Custom|DropOxygenMulticast
  (params (DeltaTime :type Float%20%28double-precision%29))
  (for _array_element (Variables|Default|GetPlayerToOx)
    (if (== (Utilities|Array|Length (Collision|GetOverlappingActors _array_element "/Game/Dynamic/Blueprints/Mechanisms/BoxColision/BP_ModulBoxColision.BP_ModulBoxColision_C" :!class /Script/Engine.Actor)) 0)
      (Class|BPIHasOxygen|DecreaseOxygen(Message) _array_element (* DeltaTime 2.0)))))

(event Custom|DoorOpenWhenPermanent
  (params (ModulBox :type BP%20Modul%20Box%20Colision%20Object%20Reference) (Door :type BP%20Door%20Object%20Reference))
  (bind _output_get (Variables|Default|SetCan%20Breath (not (or (Default|IsBreathEnable ModulBox) (not (Variables|Modul|GetPermanentBreath))))))
  (bind _output_get_2 (Variables|Modul|SetPermanentBreath _output_get))
  (Actor|Tick|SetActorTickEnabled (or (Default|IsBreathEnable ModulBox) (not (Variables|Modul|GetPermanentBreath))))
  (Default|SetCoridorOx ModulBox Door _output_get_2)
  (CallFunction|RecountBreathPermanent ModulBox Door))

(event Custom|RecountBreathPermanent
  (params (ModulBox :type BP%20Modul%20Box%20Colision%20Object%20Reference) (Door :type BP%20Door%20Object%20Reference))
  (bind _nobreath (Default|IsBreathEnable ModulBox))
  (bind _returnvalue (not _nobreath))
  (Variables|Modul|SetPermanentBreath _returnvalue)
  (Variables|Default|SetCan%20Breath _returnvalue)
  (Actor|Tick|SetActorTickEnabled _nobreath)
  (for _array_element (CallFunction|GetPermanentOpenDoor)
    (if (!= _array_element Door)
      (bind _module (Class|BPIDoor|GetModule(Message) _array_element))
      (bind _door (Class|BPIDoor|GetSelf(Message) _array_element))
      (Default|SetCoridorOx _module _door _returnvalue))))

(event EventBeginPlay
  (|CallParentFunction)
  (Utilities|FlowControl|Delay 0.2)
  (CallFunction|DoOptimize))

(event EventTick
  (params (DeltaSeconds :type Float%20%28single-precision%29))
  (|CallParentFunction DeltaSeconds)
  (Networking|SwitchHasAuthority
    (:Authority
      (CallFunction|DropOxygenMulticast DeltaSeconds))))

(fn ConstructionScript
  (Variables|Default|SetTags (Utilities|Array|MakeArray (CallFunction|IntIdtoTag (Variables|Door|GetDoorID)))))

(fn SetFire
  (params (bEnabled :type Boolean))
  (Actor|Tick|SetActorTickEnabled bEnabled)
  (if bEnabled
    (for _array_element (Collision|GetOverlappingActors (Variables|Default|GetBox) "/Game/Dynamic/Blueprints/Mechanisms/Fire/BP_Fire.BP_Fire_C" :!class /Script/Engine.PrimitiveComponent)
      (Class|BPIFire|SetFire(Message) _array_element false))))

(fn Optimize
  (params (Hide :type Boolean))
  (bind _outcomponents (Collision|BoxOverlapComponents (Transformation|GetWorldLocation (Variables|Default|GetBox)) (* (Transformation|GetWorldScale (Variables|Default|GetBox)) (Variables|/Script/Engine.BoxComponent|GetBoxExtent (Variables|Default|GetBox))) (Utilities|Array|MakeArray "ObjectTypeQuery1" "ObjectTypeQuery2" "ObjectTypeQuery4" "ObjectTypeQuery5" "ObjectTypeQuery6") 0 0 :!class /Script/Engine.KismetSystemLibrary))
  (for _array_element _outcomponents
    (if (CallFunction|IsAvaible _array_element)
      (Development|SetHiddeninGame _array_element Hide true))))

(fn DoOptimize
  (bind _open (CallFunction|IsOneOfEndRender?))
  (bind _box (Variables|Default|GetBox))
  (bind _overlappingactors (Collision|GetOverlappingActors _box "/Script/Engine.Pawn" :!class /Script/Engine.PrimitiveComponent))
  (bind _returnvalue (not _open))
  (bind _returnvalue_2 (Utilities|Array|Length _overlappingactors))
  (bind _returnvalue_3 (== _returnvalue_2 0))
  (bind _returnvalue_4 (and _returnvalue_3 _returnvalue))
  (if (!= (Variables|Optimize|GetIsHideNow) _returnvalue_4)
    (bind _output_get (Variables|Optimize|SetIsHideNow _returnvalue_4))
    (CallFunction|Optimize _output_get)))

(fn IntIdtoTag
  (params (InInt :type Integer))
  (return (Utilities|String|StringToName (Utilities|String|Append (Utilities|String|MakeLiteralString "Door") (Utilities|String|ToString(Integer) InInt)))))

(fn IsAvaible
  (params (ActorComponent :type Actor%20Component%20Object%20Reference))
  (bind _returnvalue (Components|GetOwner ActorComponent))
  (bind _returnvalue_2 (Utilities|GetClass _returnvalue))
  (return (Math|Boolean|ORBoolean (== _returnvalue_2 "/Game/Dynamic/Blueprints/Mechanisms/Door/BP_Door.BP_Door_C") (== _returnvalue_2 "/Game/Dynamic/Blueprints/Mechanisms/Door/BP_CoridorMash.BP_CoridorMash_C") (== _returnvalue_2 "/Game/Dynamic/Blueprints/Mechanisms/Door/BP_CornerCoridorMash.BP_CornerCoridorMash_C") (== _returnvalue_2 "/Game/Dynamic/Blueprints/Mechanisms/Door/BP_Stair.BP_Stair_C"))))

(fn IsOneOfEndRender?
  (bind _outactors (Actor|GetAllActorsOfClasswithTag "/Game/Dynamic/Blueprints/Mechanisms/Door/BP_Door.BP_Door_C" (CallFunction|IntIdtoTag (Variables|Door|GetDoorID))))
  (for _array_element _outactors
    (Utilities|IsValid (Variables|/Game/Dynamic/Blueprints/Mechanisms/Door/BP_Door.BP_Door_C|GetModulBox _array_element)
      (:Is%20Valid
        (if (not (Variables|/Game/Dynamic/Blueprints/Mechanisms/BoxColision/BP_ModulBoxColision.BP_ModulBoxColision_C|GetIsHideNow (Variables|/Game/Dynamic/Blueprints/Mechanisms/Door/BP_Door.BP_Door_C|GetModulBox _array_element)))
          (return true)))))
  (return false))

(fn GetPermanentOpenDoor
  (for _array_element (Collision|GetOverlappingActors (Variables|Default|GetBox) "/Game/Dynamic/Blueprints/Mechanisms/Door/BP_Door.BP_Door_C" :!class /Script/Engine.PrimitiveComponent)
    (bind _permanentopen (Class|BPIDoor|GetPermanentOpen(Message) _array_element))
    (if _permanentopen
      (Utilities|Array|Add (LocalVariables|GetDoors) _array_element)))
  (return (LocalVariables|GetDoors)))