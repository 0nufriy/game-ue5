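; BP_MechanismBase is a base Blueprint for mechanisms that can be damaged, healed and targeted through attack tokens.
; Health queries, healing and damage calls forward to a BPCHealthSystem component.
; Reserving and returning attack tokens forward to a BPCAttackTokensSystem component, so the actor holds no logic of its own beyond these pass-throughs.
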(event EventBeginPlay)

(event Collision|EventActorBeginOverlap
  (params (OtherActor :type Actor%20Object%20Reference)))

(event EventTick
  (params (DeltaSeconds :type Float%20%28single-precision%29)))

(event EventReturnAttackTokens
  (params (Amount :type Integer))
  (Default|ReturnAttackTokens (Variables|Default|GetBPC_AttackTokensSystem) Amount))

(fn ConstructionScript)

(fn GetCurrentHealth
  (return (Default|GetCurrentHealth (Variables|Default|GetBPC_HealthSystem))))

(fn GetMaxHealth
  (return (Default|GetMaxHealth (Variables|Default|GetBPC_HealthSystem))))

(fn Heal
  (params (HealAmount :type Float%20%28double-precision%29))
  (bind _newhealth (Default|Heal (Variables|Default|GetBPC_HealthSystem) HealAmount))
  (return _newhealth))

(fn IsDead
  (return (Default|IsDead (Variables|Default|GetBPC_HealthSystem))))

(fn ReserveAttackTokens
  (params (Amount :type Integer))
  (bind _success (Default|ReserveAttackTokens (Variables|Default|GetBPC_AttackTokensSystem) Amount))
  (return _success))

(fn TakeDamage
  (params (DamageInfo :type S%20Damage%20Info%20Structure))
  (bind _currenthealth (Default|TakeDamage (Variables|Default|GetBPC_HealthSystem) DamageInfo))
  (return _currenthealth))