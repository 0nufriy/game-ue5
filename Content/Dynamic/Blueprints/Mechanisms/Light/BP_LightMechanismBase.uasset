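; BP_LightMechanismBase is a base light mechanism that simulates small and huge breakages on its light component.
; It caches the starting intensity on BeginPlay, then toggles between that and zero.
; A small break runs a looping blink timer, with the delayed relight skipped once the timer is cleared.
; A huge break stops blinking and darkens the light; ending it relights and resumes the small-break blink.
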(event Custom|Blink
  (CallFunction|LightOff)
  (Utilities|FlowControl|Delay 1.4)
  (if (Utilities|Time|IsTimerActivebyHandle (Variables|Default|GetBlink%20Timer))
    (CallFunction|Lighton)))

(event EventBeginPlay
  (Variables|Default|SetIntensity (Variables|/Script/Engine.LightComponentBase|GetIntensity (Variables|Default|GetLightComponent))))

(event EventHugeLightBreakStop
  (CallFunction|Lighton)
  (CallFunction|SmallLightBreakStart))

(event EventHugeLightBreakStart
  (Utilities|Time|ClearandInvalidateTimerbyHandle (Variables|Default|GetBlink%20Timer))
  (CallFunction|LightOff))

(event EventSmallLightBreakStart
  (bind _returnvalue (Utilities|Time|SetTimerbyEvent (delegate Custom|Blink) 2.0 true))
  (Variables|Default|SetBlink%20Timer _returnvalue))

(event EventSmallLightBreakStop
  (Utilities|Time|ClearandInvalidateTimerbyHandle (Variables|Default|GetBlink%20Timer))
  (CallFunction|Lighton))

(fn ConstructionScript)

(fn OnLightChange
  (params (LightOn :type Boolean)))

(fn Lighton
  (Rendering|Components|Light|SetIntensity (Variables|Default|GetLightComponent) (Variables|Default|GetIntensity)))

(fn LightOff
  (Rendering|Components|Light|SetIntensity (Variables|Default|GetLightComponent) 0.0))