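; BP_ProjectorMech is a projector light prop, a child Blueprint that adds an emissive on/off look to its parent's light mechanism.
; On BeginPlay it creates a dynamic material instance on the SMPowerCellsWall mesh and stores it as LightMaterial.
; The LightOn and LightOff overrides call the parent, then set that material's Brightness parameter to glow or go dark.
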(event EventBeginPlay
  (bind _sm_powercells_wall (Variables|Default|GetSM_PowerCells_Wall))
  (|CallParentFunction)
  (bind _returnvalue (Rendering|Material|CreateDynamicMaterialInstance _sm_powercells_wall 0 (Rendering|Material|GetMaterial _sm_powercells_wall 0) "None" :!class /Script/Engine.PrimitiveComponent))
  (Variables|Default|SetLightMaterial _returnvalue)
  (Rendering|Material|SetMaterial _sm_powercells_wall 0 _returnvalue))

(event Collision|EventActorBeginOverlap
  (params (OtherActor :type Actor%20Object%20Reference)))

(event EventTick
  (params (DeltaSeconds :type Float%20%28single-precision%29))
  (|CallParentFunction DeltaSeconds) ; This node is disabled and will not be called.\nDrag off pins to build functionality.
)

(fn ConstructionScript
  (|CallParentFunction))

(fn Lighton
  (|CallParentFunction)
  (Rendering|Material|SetScalarParameterValue (Variables|Default|GetLightMaterial) "Brightness" 6.0 :!class /Script/Engine.MaterialInstanceDynamic))

(fn LightOff
  (|CallParentFunction)
  (Rendering|Material|SetScalarParameterValue (Variables|Default|GetLightMaterial) "Brightness" 0.0 :!class /Script/Engine.MaterialInstanceDynamic))