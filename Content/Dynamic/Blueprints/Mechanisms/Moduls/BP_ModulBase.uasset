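; Base Blueprint for damageable, repairable mechanism modules, with intact, small-break and huge-break states driven by health percentage thresholds.
; TakeDamage and Heal switch the state, toggling break VFX, calling the empty SetSoundAndLight hook and, on authority only, alerting a tag-matched camera.
; Fix heals by fix value scaled with tool efficiency and player WeldSkill, while TapeFix sets a timed IsTape flag.
; A tag-matched BP_Fire is cached but unused here.
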(event Custom|ModulSetAllert
  (bind _camera (Variables|Default|GetCamera)
    (:then
      (Default|CameraSetAllert _camera (Variables|Default|GetStatus)))
    (:else)))

(event EventBeginPlay
  (Utilities|FlowControl|Sequence
    (:then_0
      (bind _outactors (Actor|GetAllActorsOfClasswithTag "/Game/Dynamic/Blueprints/Mechanisms/Moduls/Camera/BP_Camera.BP_Camera_C" (Variables|Default|GetCameraTag)))
      (bind _array_element (Utilities|Array|ForEachLoopwithBreak _outactors :!label _label)
        (:LoopBody
          (Variables|Default|SetCamera _array_element)
          (goto _label Break))))
    (:then_1
      (bind _outactors_2 (Actor|GetAllActorsOfClasswithTag "/Game/Dynamic/Blueprints/Mechanisms/Fire/BP_Fire.BP_Fire_C" (Variables|Default|GetCameraTag)))
      (bind _array_element_2 (Utilities|Array|ForEachLoopwithBreak _outactors_2 :!label _label_2)
        (:LoopBody
          (Variables|Default|SetFire _array_element_2)
          (goto _label_2 Break))))))

(event Collision|EventActorBeginOverlap
  (params (OtherActor :type Actor%20Object%20Reference)))

(event EventHugeBreakingStart
  (Components|Activation|Activate (Variables|Default|GetHugeBreakVFX) false)
  (Components|Activation|Deactivate (Variables|Default|GetLittleBreakVFX))
  (Variables|Default|SetStatus "NewEnumerator2")
  (CallFunction|SetSoundandLight)
  (Networking|SwitchHasAuthority
    (:Authority
      (CallFunction|ModulSetAllert))))

(event EventFix
  (params (FixValue :type Float%20%28double-precision%29) (PlayerStats :type BPC%20Player%20Stats%20System%20Object%20Reference) (ToolFixModulEfficiency :type Integer) (ToolFixHoleEfficiency :type Integer))
  (bind _bpc_healthsystem (Variables|Default|GetBPC_HealthSystem))
  (if (!= (Default|GetMaxHealth _bpc_healthsystem) (Default|GetCurrentHealth _bpc_healthsystem))
    (bind _fix (CallFunction|CalculateFixEfficiency FixValue PlayerStats ToolFixModulEfficiency))
    (CallFunction|Heal _fix)))

(event EventTapeFix
  (params (Time :type Float%20%28double-precision%29))
  (Variables|Default|SetIsTape true)
  (Utilities|FlowControl|Delay Time)
  (Variables|Default|SetIsTape false))

(event EventSmallBreakingStart
  (Components|Activation|Activate (Variables|Default|GetLittleBreakVFX) false)
  (Components|Activation|Deactivate (Variables|Default|GetHugeBreakVFX))
  (Variables|Default|SetStatus "NewEnumerator1")
  (CallFunction|SetSoundandLight)
  (Networking|SwitchHasAuthority
    (:Authority
      (CallFunction|ModulSetAllert))))

(event EventHugeBreakingStop
  (Components|Activation|Deactivate (Variables|Default|GetHugeBreakVFX))
  (Variables|Default|SetStatus "NewEnumerator1")
  (CallFunction|SetSoundandLight)
  (Networking|SwitchHasAuthority
    (:Authority
      (CallFunction|ModulSetAllert))))

(event EventSmallBreakingStop
  (Components|Activation|Deactivate (Variables|Default|GetLittleBreakVFX))
  (Variables|Default|SetStatus "NewEnumerator0")
  (CallFunction|SetSoundandLight)
  (Networking|SwitchHasAuthority
    (:Authority
      (CallFunction|ModulSetAllert))))

(fn ConstructionScript)

(fn TakeDamage
  (params (DamageInfo :type S%20Damage%20Info%20Structure))
  (bind _status (Variables|Default|GetStatus))
  (bind _newhealth (|CallParentFunction DamageInfo))
  (Utilities|FlowControl|Sequence
    (:then_0
      (bind _maxhealth (CallFunction|GetMaxHealth))
      (bind _currenthealth (CallFunction|GetCurrentHealth))
      (if (and (<= (/ _currenthealth _maxhealth) (Variables|Default|GetPercentHpToHugeBrock)) (!= (Variables|Default|GetStatus) 2))
        (CallFunction|HugeBreakingStart)
        (elif (Math|Boolean|ANDBoolean (<= (/ _currenthealth _maxhealth) (Variables|Default|GetPercentHpToSmallBrock)) (!= _status 1) (!= _status 2))
          (CallFunction|SmallBreakingStart))))
    (:then_1
      (return _newhealth))))

(fn Heal
  (params (HealAmount :type Float%20%28double-precision%29))
  (bind _newhealth (Default|Heal (Variables|Default|GetBPC_HealthSystem) HealAmount))
  (Utilities|FlowControl|Sequence
    (:then_0
      (bind _maxhealth (CallFunction|GetMaxHealth))
      (bind _currenthealth (CallFunction|GetCurrentHealth))
      (if (and (> (/ _currenthealth _maxhealth) (Variables|Default|GetPercentHpToSmallBrock)) (!= (Variables|Default|GetStatus) 0))
        (CallFunction|SmallBreakingStop)
        (elif (and (> (/ _currenthealth _maxhealth) (Variables|Default|GetPercentHpToHugeBrock)) (== (Variables|Default|GetStatus) 2))
          (CallFunction|HugeBreakingStop))))
    (:then_1
      (return _newhealth))))

(fn GetCurrentHealth
  (return (Default|GetCurrentHealth (Variables|Default|GetBPC_HealthSystem))))

(fn GetMaxHealth
  (return (Default|GetMaxHealth (Variables|Default|GetBPC_HealthSystem))))

(fn IsDead
  (return (Default|IsDead (Variables|Default|GetBPC_HealthSystem))))

(fn SetSoundandLight)

(fn CalculateFixEfficiency
  (params (FixValue :type Float%20%28double-precision%29) (PlayerStat :type BPC%20Player%20Stats%20System%20Object%20Reference) (ToolFixEfficiency :type Integer))
  (return (* FixValue ToolFixEfficiency (Variables|/Game/Dynamic/Blueprints/Components/StatsSystemComponent/Player/BPC_Player_StatsSystem.BPC_Player_StatsSystem_C|GetWeldSkill PlayerStat))))

(fn GetHealthPercent
  (bind _bpc_healthsystem (Variables|Default|GetBPC_HealthSystem))
  (return (/ (Default|GetCurrentHealth _bpc_healthsystem) (Default|GetMaxHealth _bpc_healthsystem))))

(fn GetIsTape
  (return (Variables|Default|GetIsTape)))