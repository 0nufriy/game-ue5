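; Breakable generator mechanism that drives the level's lights according to its small or huge break state.
; It caches all BPI_Light actors on BeginPlay and relays break start and stop events to them, with huge breaks also igniting Fire on authority.
; TapeFix temporarily sends a small-break stop to the lights, then reapplies the current break after a delay.
; Status also selects the indicator material and running or broken sounds.
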(event EventBeginPlay
  (|CallParentFunction)
  (bind _outactors (Actor|GetAllActorswithInterface "/Game/Dynamic/Interfaces/BPI_Light.BPI_Light_C"))
  (Variables|Default|SetLights _outactors))

(event Collision|EventActorBeginOverlap
  (params (OtherActor :type Actor%20Object%20Reference))
  (|CallParentFunction OtherActor) ; This node is disabled and will not be called.\nDrag off pins to build functionality.
)

(event EventTick
  (params (DeltaSeconds :type Float%20%28single-precision%29))
  (|CallParentFunction DeltaSeconds) ; This node is disabled and will not be called.\nDrag off pins to build functionality.
)

(event EventSmallBreakingStop
  (|CallParentFunction)
  (for _array_element (Variables|Default|GetLights)
    (Class|BPILight|SmallLightBreakStop(Message) _array_element)))

(event EventHugeBreakingStop
  (|CallParentFunction)
  (if (not (Variables|Default|GetIsTape))
    (for _array_element (Variables|Default|GetLights)
      (Class|BPILight|HugeLightBreakStop(Message) _array_element))))

(event EventHugeBreakingStart
  (|CallParentFunction)
  (for _array_element (Variables|Default|GetLights)
    (Class|BPILight|HugeLightBreakStart(Message) _array_element))
  (Networking|SwitchHasAuthority
    (:Authority
      ;[1 1 1] Should Refactor
      (bind _fire (Variables|Default|GetFire)
        (:then
          (Default|SetFire _fire true))
        (:else)))))

(event EventSmallBreakingStart
  (|CallParentFunction)
  (for _array_element (Variables|Default|GetLights)
    (Class|BPILight|SmallLightBreakStart(Message) _array_element)))

(event EventTapeFix
  (params (Time :type Float%20%28double-precision%29))
  (bind _lights (Variables|Default|GetLights))
  (Variables|Default|SetIsTape true)
  (if (!= (Variables|Default|GetStatus) 0)
    (for _array_element _lights
      (Class|BPILight|SmallLightBreakStop(Message) _array_element))
    (Utilities|FlowControl|Delay Time)
    (Variables|Default|SetIsTape false)
    (switch Utilities|FlowControl|Switch|SwitchonE_ModuleStatus (Variables|Default|GetStatus)
      (:NewEnumerator1
        (for _array_element_2 _lights
          (Class|BPILight|SmallLightBreakStart(Message) _array_element_2)))
      (:NewEnumerator2
        (for _array_element_3 _lights
          (Class|BPILight|HugeLightBreakStart(Message) _array_element_3))))
    (else
      (Utilities|FlowControl|Delay Time)
      (Variables|Default|SetIsTape false))))

(fn ConstructionScript
  (|CallParentFunction))

(fn SetLightandSound
  (params (Status :type E_ModuleStatus%20Enum :default "NewEnumerator0"))
  (Rendering|Material|SetMaterial (Variables|Default|GetStaticMeshComponent) 1 (Utilities|Select :Index Status :NewEnumerator0 "/Game/Static/Moduls/Generator/Material/MI_ElectricalSupply_Details_Green.MI_ElectricalSupply_Details_Green" :NewEnumerator1 "/Game/Static/Moduls/Generator/Material/MI_ElectricalSupply_Details_Yellow.MI_ElectricalSupply_Details_Yellow" :NewEnumerator2 "/Game/Static/Moduls/Generator/Material/MI_ElectricalSupply_Details_Red.MI_ElectricalSupply_Details_Red"))
  (switch Utilities|FlowControl|Switch|SwitchonE_ModuleStatus Status
    (:NewEnumerator0
      (Audio|Components|Audio|Stop (Variables|Default|GetGeneratorBroken))
      (if (not (Audio|Components|Audio|IsPlaying (Variables|Default|GetGenerator)))
        (Audio|Components|Audio|Play (Variables|Default|GetGenerator) 0.0)))
    (:NewEnumerator1
      (Audio|Components|Audio|Play (Variables|Default|GetGeneratorBroken) 0.0)
      (if (not (Audio|Components|Audio|IsPlaying (Variables|Default|GetGenerator)))
        (Audio|Components|Audio|Play (Variables|Default|GetGenerator) 0.0)))
    (:NewEnumerator2
      (Audio|Components|Audio|Stop (Variables|Default|GetGeneratorBroken))
      (Audio|Components|Audio|Stop (Variables|Default|GetGenerator)))))

(fn SetSoundandLight
  (CallFunction|SetLightandSound (Variables|Default|GetStatus)))