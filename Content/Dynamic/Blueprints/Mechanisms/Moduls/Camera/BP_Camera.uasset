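; Security camera for a tagged module that renders its view into a runtime render target shown through a VHS-style material.
; It reports the higher of its set alert and hole-count alert to BP_SecurityCenter.
; When rotation is enabled, the head sweeps on authority, pausing and reversing at each angle limit.
; SetLight toggles capture visibility, head material and the camera-watch flag on matching module boxes, then triggers their optimization.
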(event Custom|CameraSetAllert
  (params (AllertLevl :type E_ModuleStatus%20Enum :default "NewEnumerator0"))
  (Variables|Default|SetAllert%20Levl AllertLevl)
  (bind _newparam (CallFunction|CalculateAllart))
  (Default|CenterSetAllert (Variables|Default|GetSecurityCenter) _newparam (Variables|Cam|GetCamNum)))

(event Custom|RotationDelay
  (Actor|Tick|SetActorTickEnabled false)
  (Utilities|FlowControl|Delay (Variables|Rotate|GetRotateDelay))
  (Actor|Tick|SetActorTickEnabled true))

(event Custom|SetBreath
  (params (HoleCount :type Integer))
  (Variables|Default|SetHoleCount HoleCount)
  (bind _newparam (CallFunction|CalculateAllart))
  (Default|CenterSetAllert (Variables|Default|GetSecurityCenter) _newparam (Variables|Cam|GetCamNum)))

(event Custom|SetLight
  (params (Light :type Boolean))
  (Rendering|SetVisibility (Variables|Default|GetSceneCaptureComponent2D) Light true)
  (Rendering|Material|SetMaterial (Variables|Default|Getcamera_head) 0 (select Light "/Game/Static/SomeMesh/Camera/Material/Cam.Cam" "/Game/Static/SomeMesh/Camera/Material/Cam_unlight.Cam_unlight"))
  (bind _outactors (Actor|GetAllActorsOfClasswithTag "/Game/Dynamic/Blueprints/Mechanisms/BoxColision/BP_ModulBoxColision.BP_ModulBoxColision_C" (Variables|Cam|GetModulTag)))
  (for _array_element _outactors
    (Variables|/Game/Dynamic/Blueprints/Mechanisms/BoxColision/BP_ModulBoxColision.BP_ModulBoxColision_C|SetIs%20CameraWatch _array_element Light)
    (Default|DoOptimize _array_element)))

(event EventBeginPlay
  (bind _returnvalue (Rendering|CreateRenderTarget2D 1024 576 "RTF_RGBA16f"))
  (bind _output_get (Variables|Cam|SetRenderTarget _returnvalue))
  (Variables|/Script/Engine.SceneCaptureComponent2D|SetTextureTarget (Variables|Default|GetSceneCaptureComponent2D) _output_get)
  (bind _returnvalue_2 (Rendering|Material|CreateDynamicMaterialInstance "/Game/Dynamic/Blueprints/Mechanisms/Moduls/Camera/Material/MI_VHS_Cam1.MI_VHS_Cam1" "None" "None" :!class /Script/Engine.KismetMaterialLibrary))
  (Rendering|Material|SetTextureParameterValue _returnvalue_2 "Camera" _output_get)
  (Variables|Cam|SetRenderMaterial _returnvalue_2)
  (Actor|Tick|SetActorTickEnabled (Variables|Rotate|GetShouldRotate))
  (Variables|Default|SetAllert%20Levl "NewEnumerator0")
  (Variables|Default|SetHoleCount 0)
  (CallFunction|CalculateAllart))

(event EventTick
  (params (DeltaSeconds :type Float%20%28single-precision%29))
  (Networking|SwitchHasAuthority
    (:Authority
      (CallFunction|Rotate DeltaSeconds))))

(fn ConstructionScript
  (Variables|Default|SetTags (Utilities|Array|MakeArray (Variables|Cam|GetModulTag)))
  (bind _returnvalue (Actor|GetActorOfClass "/Game/Dynamic/Blueprints/Mechanisms/Moduls/Camera/BP_SecurityCenter.BP_SecurityCenter_C"))
  (Variables|Default|SetSecurityCenter _returnvalue))

(fn GetMaterial
  (return (Variables|Cam|GetRenderMaterial)))

(fn Rotate
  (params (DeltaTime :type Float%20%28double-precision%29))
  (bind _rotateangle (Variables|Rotate|GetRotateAngle))
  (bind _rotateangle_2 (Variables|Rotate|GetRotateAngle))
  (bind _camera_head (Variables|Default|Getcamera_head))
  (bind _returnvalue (* _rotateangle -1.0))
  (bind _relativerotation (Variables|/Script/Engine.SceneComponent|GetRelativeRotation _camera_head))
  (bind (_roll _pitch _yaw) (Math|Rotator|BreakRotator _relativerotation))
  (bind _returnvalue_2 (<= _yaw _rotateangle_2))
  (Transformation|AddLocalRotation (Variables|Default|Getcamera_head) (Math|Rotator|MakeRotator 0.0 0.0 (* DeltaTime (Variables|Rotate|GetRotateSpeed))) false false)
  (if (not (and _returnvalue_2 (>= _yaw _returnvalue)))
    (Transformation|SetRelativeRotation (Variables|Default|Getcamera_head) (Math|Rotator|MakeRotator _roll _pitch (Math|Float|SelectFloat _returnvalue _rotateangle_2 _returnvalue_2)) false false)
    (Variables|Rotate|SetRotateSpeed (* (Variables|Rotate|GetRotateSpeed) -1.0))
    (CallFunction|RotationDelay)))

(fn CalculateAllart
  (switch int (Variables|Default|GetHoleCount)
    (:Default
      (LocalVariables|SetHoleAllert "NewEnumerator2"))
    (:0
      (LocalVariables|SetHoleAllert "NewEnumerator0"))
    (:1
      (LocalVariables|SetHoleAllert "NewEnumerator1")))
  (switch int (Math|Conversions|ToInteger(Byte) (Class|KismetMathLibrary|BMax (Variables|Default|GetAllert%20Levl) (LocalVariables|GetHoleAllert)))
    (:Default
      (return "NewEnumerator2"))
    (:0
      (return "NewEnumerator0"))
    (:1
      (return "NewEnumerator1"))))

(fn GetModule
  (bind _outactors (Actor|GetAllActorsOfClasswithTag "/Game/Dynamic/Blueprints/Mechanisms/BoxColision/BP_ModulBoxColision.BP_ModulBoxColision_C" (Variables|Cam|GetModulTag)))
  (return (Utilities|Array|Get(acopy) _outactors)))