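; BP_Button is a mechanism button with an embedded UI widget that drops its linked module when pressed.
; A press runs Click directly or, when the game instance flags multiplayer messaging, goes through the player controller's DropButtonMessage.
; Click deactivates the button and animates it along Z by timeline, then calls Drop on the module assigned through SetModul.
; Active and Disactive toggle its state through Multicast-named events with their own movement timelines.
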(event Custom|Active
  (CallFunction|ActiveMulticast))

(event Custom|Disactive
  (CallFunction|DisactiveMulticast))

(event Custom|ClickLocal
  (bind _ismultiplayer (Class|BPIMultiplayer|GetIsMultiplayer(Message) (Game|GetGameInstance)))
  (if _ismultiplayer
    (Class|BPIController|DropButton(Message) (Game|GetPlayerController 0) self)
    (else
      (CallFunction|Click))))

(event Custom|ActiveMulticast
  (if (not (Variables|Default|GetIsActive))
    (Variables|Default|SetIsActive true)
    (bind _buttonactive (Timeline|Timeline_1 PlayFromStart)
      (:Update
        (Transformation|SetRelativeLocation (Variables|Default|GetButton_Button) (Math|Vector|Lerp(Vector) "0, 0, 0" "0.000000,0.000000,-51.000000" _buttonactive) false false)))))

(event Custom|DisactiveMulticast
  (if (Variables|Default|GetIsActive)
    (Variables|Default|SetIsActive false)
    (bind _buttondisactive (Timeline|Timeline_0 PlayFromStart)
      (:Update
        (Transformation|SetRelativeLocation (Variables|Default|GetButton_Button) (Math|Vector|Lerp(Vector) "0, 0, 0" "0.000000,0.000000,-51.000000" _buttondisactive) false false)))))

(event Custom|ClickMulticast
  (params (Target :type BP%20Modul%20Box%20Colision%20Object%20Reference))
  (Variables|Default|SetIsActive false)
  (bind _button (Timeline|Timeline PlayFromStart)
    (:Update
      (Transformation|SetRelativeLocation (Variables|Default|GetButton_Button) (Math|Vector|Lerp(Vector) "0, 0, 0" "0.000000,0.000000,-51.000000" _button) false false))
    (:Finished
      (Default|Drop Target))))

(event Custom|Click
  (if (and (Variables|Default|GetIsActive) (Utilities|IsValid (Variables|Default|GetModule)))
    (CallFunction|ClickMulticast (Variables|Default|GetModule))))

(event EventBeginPlay
  (bind _asui_button (Utilities|Casting|CastToUI_Button (UserInterface|GetWidget (Variables|Default|GetWidget))))
  (EventDispatchers|BindEventtoOnPressed (Variables|/Game/Dynamic/Blueprints/UI/InteractInWorld/Camera/UI_Button.UI_Button_C|GetButton_41 _asui_button) (delegate Custom|ClickLocal)))

(fn ConstructionScript)

(fn SetModul
  (params (ModulBoxColision :type BP%20Modul%20Box%20Colision%20Object%20Reference))
  (bind _output_get (Variables|Default|SetModule ModulBoxColision))
  (return _output_get))