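; BP_SecurityCenter is a breakable security station module that shows the selected BP_Camera's feed on a monitor and camera alert levels on a UI_Map widget.
; Button presses, routed through the player controller in multiplayer, black out the screen, then after a delay light that camera and arm a button if its module allows dropping.
; Damage state drives blinking or static feeds and broken sounds via authority-gated multicasts, while tape temporarily lifts a huge break.
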(event Custom|CenterSetAllert
  (params (AllertLevel :type E_ModuleStatus%20Enum :default "NewEnumerator0") (CamNum :type Integer))
  (Default|SetAllert (Variables|Default|GetUI%20Map) (Utilities|Select :Index AllertLevel :NewEnumerator0 (Class|KismetSystemLibrary|MakeLiteralInteger) :NewEnumerator1 (Class|KismetSystemLibrary|MakeLiteralInteger 1) :NewEnumerator2 (Class|KismetSystemLibrary|MakeLiteralInteger 2)) CamNum))

(event Custom|SetMaterialByCammeraMulticast
  (params (Camera :type BP%20Camera%20Object%20Reference))
  (Rendering|Material|SetMaterial (Variables|Default|GetCube) 0 (Variables|/Game/Dynamic/Blueprints/Mechanisms/Moduls/Camera/BP_Camera.BP_Camera_C|GetRenderMaterial Camera)))

(event Custom|ButtonPressLocal
  (params (CamNum :type Integer))
  (bind _ismultiplayer (Class|BPIMultiplayer|GetIsMultiplayer(Message) (Game|GetGameInstance)))
  (if _ismultiplayer
    (Class|BPIController|CameraButton(Message) (Game|GetPlayerController 0) self CamNum)
    (else
      (CallFunction|ButtonPress CamNum))))

(event Custom|LitleBrakeBlink
  (Networking|SwitchHasAuthority
    (:Authority
      (CallFunction|SetMaterialbyCammeraMulticast (Variables|Default|GetCameraNow))
      (Utilities|FlowControl|Delay 0.1)
      (CallFunction|SetMaterialMulticast "/Game/Dynamic/Blueprints/Mechanisms/Moduls/Camera/Material/MI_VHS_BrokenCam.MI_VHS_BrokenCam"))))

(event Custom|StopSoundMulticast
  (Audio|Components|Audio|Stop (Variables|Default|GetCamera1)))

(event Custom|StartSoundMulticast
  (Audio|Components|Audio|Play (Variables|Default|GetCamera1) 0.0))

(event Custom|StartBrokenSoundMulticast
  (Audio|Components|Audio|Play (Variables|Default|GetCameraBroken) 0.0))

(event Custom|StopBrokenSoundMulticast
  (Audio|Components|Audio|Stop (Variables|Default|GetCameraBroken)))

(event Custom|SetMaterialMulticast
  (params (Material :type Material%20Interface%20Object%20Reference))
  (Rendering|Material|SetMaterial (Variables|Default|GetCube) 0 Material))

(event Custom|ButtonPress
  (params (CamNum :type Integer))
  (CallFunction|SetVoidScreen)
  (Utilities|FlowControl|Delay (Variables|Default|GetChangeCameraDelay))
  (CallFunction|SetCamonScreenbyNum CamNum))

(event EventBeginPlay
  (|CallParentFunction)
  (bind _outactors (Actor|GetAllActorsOfClass "/Game/Dynamic/Blueprints/Mechanisms/Moduls/Camera/BP_Camera.BP_Camera_C"))
  (Variables|Default|SetCamers _outactors)
  (bind _asbp_button (Utilities|Casting|CastToBP_Button (Variables|/Script/Engine.ChildActorComponent|GetChildActor (Variables|Default|GetBP_Button)))
    (:then
      (Variables|Default|SetBP%20Button _asbp_button))
    (:CastFailed
      _))
  (bind _asui_map (Utilities|Casting|CastToUI_Map (UserInterface|GetWidget (Variables|Default|GetWidget))))
  (bind _output_get (Variables|Default|SetUI%20Map _asui_map))
  (Default|SetSecurityCentr _output_get self))

(event Collision|EventActorBeginOverlap
  (params (OtherActor :type Actor%20Object%20Reference))
  (|CallParentFunction OtherActor) ; This node is disabled and will not be called.\nDrag off pins to build functionality.
)

(event EventTick
  (params (DeltaSeconds :type Float%20%28single-precision%29))
  (|CallParentFunction DeltaSeconds) ; This node is disabled and will not be called.\nDrag off pins to build functionality.
)

(event EventTapeFix
  (params (Time :type Float%20%28double-precision%29))
  (Variables|Default|SetIsTape true)
  (if (== (Variables|Default|GetStatus) 2)
    (CallFunction|HugeBreakingStop)
    (Utilities|FlowControl|Delay Time)
    (bind _currenthealth (CallFunction|GetCurrentHealth))
    (bind _maxhealth (CallFunction|GetMaxHealth))
    (Variables|Default|SetIsTape false)
    (if (<= (/ _currenthealth _maxhealth) (Variables|Default|GetPercentHpToHugeBrock))
      (CallFunction|HugeBreakingStart))
    (else
      (Utilities|FlowControl|Delay Time)
      (Variables|Default|SetIsTape false))))

(event EventSmallBreakingStop
  (|CallParentFunction)
  (Utilities|Time|ClearandInvalidateTimerbyHandle (Variables|Default|GetBlinkHandler))
  (Audio|Components|Audio|Stop (Variables|Default|GetCameraBroken))
  (Networking|SwitchHasAuthority
    (:Authority
      (CallFunction|SetCamonScreenbyNum (Variables|Default|GetCurCam)))))

(event EventHugeBreakingStop
  (|CallParentFunction)
  (CallFunction|SetCamonScreenbyNum (Variables|Default|GetCurCam)))

(event EventHugeBreakingStart
  (|CallParentFunction)
  (Utilities|Time|ClearandInvalidateTimerbyHandle (Variables|Default|GetBlinkHandler))
  (Networking|SwitchHasAuthority
    (:Authority
      (bind _fire (Variables|Default|GetFire)
        (:then
          (Default|SetFire _fire true))
        (:else
          _))
      (CallFunction|SetCamonScreenbyNum (Variables|Default|GetCurCam)))))

(event EventSmallBreakingStart
  (|CallParentFunction)
  (Audio|Components|Audio|Stop (Variables|Default|GetCamera1))
  (Networking|SwitchHasAuthority
    (:Authority
      (CallFunction|SetCamonScreenbyNum (Variables|Default|GetCurCam)))))

(fn ConstructionScript
  (|CallParentFunction))

(fn SetCamonScreenbyNum
  (params (Num :type Integer))
  (bind _bp_button (Variables|Default|GetBP%20Button))
  (Utilities|IsValid (Variables|Default|GetCameraNow)
    (:Is%20Valid
      (Default|SetLight (Variables|Default|GetCameraNow) false)
      (Variables|Default|SetCameraNow 0))
    (:Is%20Not%20Valid
      _))
  (Variables|Default|SetCurCam Num)
  (bind _array_element (Utilities|Array|ForEachLoopwithBreak (Variables|Default|GetCamers))
    (:LoopBody
      (if (== Num (Variables|/Game/Dynamic/Blueprints/Mechanisms/Moduls/Camera/BP_Camera.BP_Camera_C|GetCamNum _array_element))
        (bind _output_get (Variables|Default|SetCameraNow _array_element))
        (if (Default|GetIsDropAvaible (Default|GetModule _output_get))
          (Default|Active _bp_button)
          (Default|SetModul _bp_button (Default|GetModule _output_get))
          (else
            (Default|Disactive _bp_button)
            (Default|SetModul _bp_button)))
        (Default|SetLight _output_get true)
        (switch Utilities|FlowControl|Switch|SwitchonE_ModuleStatus (Variables|Default|GetStatus)
          (:NewEnumerator0
            (CallFunction|SetMaterialbyCammeraMulticast (Variables|Default|GetCameraNow))
            (CallFunction|StartSoundMulticast))
          (:NewEnumerator1
            (bind _returnvalue (Utilities|Time|SetTimerbyEvent (EventDispatchers|CreateEvent :!event Custom|LitleBrakeBlink) 0.5 true -0.5))
            (Variables|Default|SetBlinkHandler _returnvalue)
            (Variables|Default|SetTexture%20Render (Default|GetMaterial (Variables|Default|GetCameraNow)))
            (CallFunction|StartBrokenSoundMulticast :!label _label))
          (:NewEnumerator2
            (CallFunction|SetMaterialMulticast "/Game/Dynamic/Blueprints/Mechanisms/Moduls/Camera/Material/MI_VHS_BrokenCam.MI_VHS_BrokenCam")
            (goto _label)))
        (return true)))
    (:Completed
      (Variables|Default|SetTexture%20Render "/Engine/MapTemplates/Sky/M_BlackBackground.M_BlackBackground")
      (return false))))

(fn SetVoidScreen
  (CallFunction|SetMaterialMulticast "/Engine/MapTemplates/Sky/M_BlackBackground.M_BlackBackground")
  (CallFunction|StopSoundMulticast))