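; BP_Engine is a breakable engine mechanism, tagged first or second, that reports a speed multiplier to the level from reactor speed and damage status.
; Small breaks scale output and change rotor speed; huge breaks also stop motion and ignite fire, while tape temporarily boosts broken output.
; Authority-side Tick swings the mesh in pitch between random limits, pausing at each reversal, with sound volume following rotation speed.
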(event Custom|RotateDelay
  (Audio|Components|Audio|SetVolumeMultiplier (Variables|Default|GetEngine) 0.0 :!class /Script/Engine.AudioComponent)
  (Actor|Tick|SetActorTickEnabled false)
  (Utilities|FlowControl|Delay (Variables|Default|GetDelayRotate))
  (if (or (!= (Variables|Default|GetStatus) 2) (Variables|Default|GetIsTape))
    (Actor|Tick|SetActorTickEnabled true)
    (CallFunction|SetSound)))

(event Custom|Rotation
  (params (NewRotation :type Rotator) (RotateSpeed :type Float%20%28double-precision%29) (RotateAngel :type Float%20%28double-precision%29))
  (Transformation|SetRelativeRotation (Variables|Default|GetStaticMeshComponent) NewRotation false false)
  (Variables|Default|SetRotateSpeed RotateSpeed)
  (Variables|Default|SetRotateAngel RotateAngel))

(event Custom|AddRotation
  (params (DeltaRotation :type Rotator))
  (Transformation|AddRelativeRotation (Variables|Default|GetStaticMeshComponent) DeltaRotation false false))

(event EventBeginPlay
  (|CallParentFunction))

(event Collision|EventActorBeginOverlap
  (params (OtherActor :type Actor%20Object%20Reference))
  (|CallParentFunction OtherActor) ; This node is disabled and will not be called.\nDrag off pins to build functionality.
)

(event EventTick
  (params (DeltaSeconds :type Float%20%28single-precision%29))
  (Networking|SwitchHasAuthority
    (:Authority
      (|CallParentFunction DeltaSeconds)
      (CallFunction|Rotate DeltaSeconds))))

(event EventSmallBreakingStart
  (bind _breakrotatorspeed (Variables|Default|GetBreakRotatorSpeed))
  (|CallParentFunction)
  (Networking|SwitchHasAuthority
    (:Authority
      (Default|CallSetEngineonLevel (Variables|Engine|GetFirstEngine) (* (Variables|Engine|GetMultiplySmallBreak) (Variables|Engine|GetReactorSpeed)))
      (Variables|Default|SetRotateSpeed (Math|Float|SelectFloat _breakrotatorspeed (* _breakrotatorspeed -1.0) (>= (Variables|Default|GetRotateSpeed) 0.0)))
      (Variables|Default|SetDelayRotate (Variables|Default|GetBreakRotateDelay)))))

(event EventHugeBreakingStart
  (|CallParentFunction)
  (Networking|SwitchHasAuthority
    (:Authority
      (Default|CallSetEngineonLevel (Variables|Engine|GetFirstEngine) (* (Variables|Engine|GetMultiplayHugeBreak) (Variables|Engine|GetReactorSpeed)))
      (Actor|Tick|SetActorTickEnabled false)
      (bind _fire (Variables|Default|GetFire)
        (:then
          (Default|SetFire _fire true))
        (:else)))))

(event EventHugeBreakingStop
  (bind _breakrotatorspeed (Variables|Default|GetBreakRotatorSpeed))
  (|CallParentFunction)
  (Networking|SwitchHasAuthority
    (:Authority
      (Default|CallSetEngineonLevel (Variables|Engine|GetFirstEngine) (* (Variables|Engine|GetMultiplySmallBreak) (Variables|Engine|GetReactorSpeed)))
      (Actor|Tick|SetActorTickEnabled true)
      (Variables|Default|SetRotateSpeed (Math|Float|SelectFloat _breakrotatorspeed (* _breakrotatorspeed -1.0) (>= (Variables|Default|GetRotateSpeed) 0.0)))
      (Variables|Default|SetDelayRotate (Variables|Default|GetBreakRotateDelay)))))

(event EventSmallBreakingStop
  (bind _normalrotatorspeed (Variables|Default|GetNormalRotatorSpeed))
  (|CallParentFunction)
  (Networking|SwitchHasAuthority
    (:Authority
      (Default|CallSetEngineonLevel (Variables|Engine|GetFirstEngine) (Variables|Engine|GetReactorSpeed))
      (Variables|Default|SetRotateSpeed (Math|Float|SelectFloat _normalrotatorspeed (* _normalrotatorspeed -1.0) (>= (Variables|Default|GetRotateSpeed) 0.0)))
      (Variables|Default|SetDelayRotate (Variables|Default|GetBreakRotateDelay)))))

(event EventTapeFix
  (params (Time :type Float%20%28double-precision%29))
  (Variables|Default|SetIsTape true)
  (if (!= (Variables|Default|GetStatus) 0)
    (Default|CallSetEngineonLevel (Variables|Engine|GetFirstEngine) (Utilities|Select :Index (Variables|Default|GetStatus) :NewEnumerator0 0.0 :NewEnumerator1 (+ (* (Variables|Engine|GetMultiplySmallBreak) (Variables|Engine|GetReactorSpeed)) 0.1) :NewEnumerator2 (+ (* (Variables|Engine|GetMultiplayHugeBreak) (Variables|Engine|GetReactorSpeed)) 0.1)))
    (Actor|Tick|SetActorTickEnabled true)
    (Utilities|FlowControl|Delay Time)
    (Variables|Default|SetIsTape false)
    (Default|CallSetEngineonLevel (Variables|Engine|GetFirstEngine) (Utilities|Select :Index (Variables|Default|GetStatus) :NewEnumerator0 (Variables|Engine|GetReactorSpeed) :NewEnumerator1 (* (Variables|Engine|GetMultiplySmallBreak) (Variables|Engine|GetReactorSpeed)) :NewEnumerator2 (* (Variables|Engine|GetMultiplayHugeBreak) (Variables|Engine|GetReactorSpeed))))
    (if (== (Variables|Default|GetStatus) 2)
      (Actor|Tick|SetActorTickEnabled false)
      (Audio|Components|Audio|SetVolumeMultiplier (Variables|Default|GetEngine) 0.0 :!class /Script/Engine.AudioComponent))
    (else
      (Utilities|FlowControl|Delay Time)
      (Variables|Default|SetIsTape false))))

(fn ConstructionScript
  (|CallParentFunction)
  (Variables|Default|SetDelayRotate (Variables|Default|GetNormalRotatorDelay))
  (Variables|Default|SetRotateSpeed (Variables|Default|GetNormalRotatorSpeed))
  (if (Variables|Engine|GetFirstEngine)
    (Variables|Default|SetTags (Utilities|Array|MakeArray "EngineFirst"))
    (else
      (Variables|Default|SetTags (Utilities|Array|MakeArray "EngineSecond")))))

(fn SetReactorSpeed
  (params (Reactor%20speed :type Float%20%28double-precision%29) (IsAnotherReactor :type Boolean))
  (if IsAnotherReactor
    (Variables|Default|SetAnotherReactor true))
  (if (not (and (Variables|Default|GetAnotherReactor) (< Reactor%20speed (CallFunction|GetReactorSpeed IsAnotherReactor))))
    (bind _output_get (Variables|Engine|SetReactorSpeed Reactor%20speed))
    (CallFunction|SetSound)
    (Default|CallSetEngineonLevel (Variables|Engine|GetFirstEngine) (Utilities|Select :Index (Variables|Default|GetStatus) :NewEnumerator0 _output_get :NewEnumerator1 (* (Variables|Engine|GetMultiplySmallBreak) (Variables|Engine|GetReactorSpeed)) :NewEnumerator2 (* (Variables|Engine|GetReactorSpeed) (Variables|Engine|GetMultiplayHugeBreak))))))

(fn Rotate
  (params (DeltaTime :type Float%20%28double-precision%29))
  (bind _returnvalue (CallFunction|RotateSpeedCalculate))
  (bind _rotatespeed (Variables|Default|GetRotateSpeed))
  (bind _staticmeshcomponent (Variables|Default|GetStaticMeshComponent))
  (bind _rotateangel (Variables|Default|GetRotateAngel))
  (bind _rotateangel_2 (Variables|Default|GetRotateAngel))
  (bind _angelmin (Variables|Default|GetAngelMin))
  (bind _returnvalue_2 (* DeltaTime _returnvalue))
  (bind _returnvalue_3 (- _angelmin 1.0))
  (bind _returnvalue_4 (* _rotateangel_2 -1.0))
  (bind _relativerotation (Variables|/Script/Engine.SceneComponent|GetRelativeRotation _staticmeshcomponent))
  (bind (_roll _pitch _yaw) (Math|Rotator|BreakRotator _relativerotation))
  (bind _returnvalue_5 (Math|Float|Absolute(Float) _returnvalue_2))
  (bind _returnvalue_6 (Math|Float|Clamp(Float) _returnvalue_5 _returnvalue_2 _returnvalue_3))
  (bind _returnvalue_7 (<= _pitch _returnvalue_4))
  (CallFunction|AddRotation (Math|Rotator|MakeRotator 0.0 (select (< _returnvalue_2 0.0) (* _returnvalue_6 -1.0) _returnvalue_6) 0.0))
  (if (or (and (>= _rotatespeed 0.0) (>= _pitch _rotateangel)) (and (< _rotatespeed 0.0) _returnvalue_7))
    (CallFunction|Rotation (Math|Rotator|MakeRotator _roll (Math|Float|SelectFloat _returnvalue_4 _rotateangel _returnvalue_7) _yaw) (* (Variables|Default|GetRotateSpeed) -1.0) (Math|Random|RandomFloatinRange (Variables|Default|GetAngelMin) (Variables|Default|GetAngelMax)))
    (CallFunction|RotateDelay)))

(fn SetSound
  (Audio|Components|Audio|SetVolumeMultiplier (Variables|Default|GetEngine) (/ (Math|Float|Absolute(Float) (CallFunction|RotateSpeedCalculate)) 5.0) :!class /Script/Engine.AudioComponent))

(fn TakeDamage
  (params (DamageInfo :type S%20Damage%20Info%20Structure))
  (bind _newhealth (|CallParentFunction DamageInfo))
  (Utilities|FlowControl|Sequence
    (:then_0
      (if (Variables|Default|GetIsDrop)
        (bind _outactors (Actor|GetAllActorsOfClasswithTag "/Game/Dynamic/Blueprints/Mechanisms/Moduls/BP_Reactor.BP_Reactor_C" (select (Variables|Engine|GetFirstEngine) "ReactorFirst" "ReactorSecond")))
        (for _array_element _outactors
          (Networking|SwitchHasAuthority
            (:Authority
              (Default|ResendSpeed _array_element))))))
    (:then_1
      (return _newhealth))))

(fn RotateSpeedCalculate
  (return (+ (/ (Variables|Default|GetRotateSpeed) (Math|Float|Clamp(Float) (* (Variables|Engine|GetReactorSpeed) (Utilities|Select :Index (Variables|Default|GetStatus) :NewEnumerator0 1.0 :NewEnumerator1 (Variables|Engine|GetMultiplySmallBreak) :NewEnumerator2 (Variables|Engine|GetMultiplayHugeBreak))) 0.1)) (Math|Float|SelectFloat 0.1 0.0 (Variables|Default|GetIsTape)))))

(fn GetReactorSpeed
  (params (Another :type Boolean))
  (bind _outactors (Actor|GetAllActorsOfClasswithTag "/Game/Dynamic/Blueprints/Mechanisms/Moduls/BP_Reactor.BP_Reactor_C" (select (== Another (Variables|Engine|GetFirstEngine)) "ReactorSecond" "ReactorFirst")))
  (return (Default|GetCurrentSpeed (Utilities|Array|Get(acopy) _outactors))))

(fn SetSoundandLight
  (switch Utilities|FlowControl|Switch|SwitchonE_ModuleStatus (Variables|Default|GetStatus)
    (:NewEnumerator0
      (CallFunction|SetSound :!label _label))
    (:NewEnumerator1
      (goto _label))
    (:NewEnumerator2
      (Audio|Components|Audio|SetVolumeMultiplier (Variables|Default|GetEngine) 0.0 :!class /Script/Engine.AudioComponent))))