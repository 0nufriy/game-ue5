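; Breakable reactor module, one of a first/second pair, that turns cooling input into speed for its engine.
; On the server, break status scales cooling into the speed sent to its engine, or the other engine if that has dropped, and spins the rotor.
; Tape fixes add a temporary boost to broken reactors.
; When damaged and dropped, it has its matching cooling module resend cooling.
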(event Custom|Rotation
  (params (DeltaRotation :type Rotator))
  (Transformation|AddRelativeRotation (Variables|Default|GetStaticMeshComponent) DeltaRotation false false)
  (Transformation|SetWorldLocation (Variables|Default|GetReactor) (Variables|Rotator|GetSoundLocation) false false))

(event EventBeginPlay
  (|CallParentFunction)
  (bind _outactors (Actor|GetAllActorsOfClass "/Game/Dynamic/Blueprints/Mechanisms/Moduls/BP_Engine.BP_Engine_C"))
  (bind _array_element (Utilities|Array|ForEachLoopwithBreak _outactors)
    (:LoopBody
      (if (Actor|ActorHasTag _array_element (select (Variables|Reactor|GetIsFirst) "EngineFirst" "EngineSecond"))
        (Variables|Reactor|SetEngine _array_element)
        (else
          (Variables|Reactor|SetAnotherEngine _array_element))))))

(event EventTapeFix
  (params (Time :type Float%20%28double-precision%29))
  (bind _status (Variables|Default|GetStatus))
  (Variables|Default|SetIsTape true)
  (if (!= (Variables|Default|GetStatus) 0)
    (Variables|Default|SetStatusForTape _status)
    (CallFunction|SetEngineReactorSpeed (Utilities|Select :Index _status :NewEnumerator0 0.0 :NewEnumerator1 (+ (* (Variables|Reactor|GetSmallBreakSpeed) (Variables|Reactor|GetCooling)) 0.1) :NewEnumerator2 (+ (* (Variables|Reactor|GetHugeBreakSpeed) (Variables|Reactor|GetCooling)) 0.1)))
    (Utilities|FlowControl|Delay Time)
    (Variables|Default|SetIsTape false)
    (CallFunction|SetEngineReactorSpeed (Utilities|Select :Index (Variables|Default|GetStatus) :NewEnumerator0 (Variables|Reactor|GetCooling) :NewEnumerator1 (* (Variables|Reactor|GetSmallBreakSpeed) (Variables|Reactor|GetCooling)) :NewEnumerator2 (* (Variables|Reactor|GetHugeBreakSpeed) (Variables|Reactor|GetCooling))))
    (else
      (Utilities|FlowControl|Delay Time)
      (Variables|Default|SetIsTape false))))

(event EventTick
  (params (DeltaSeconds :type Float%20%28single-precision%29))
  (Networking|SwitchHasAuthority
    (:Authority
      (|CallParentFunction DeltaSeconds)
      (CallFunction|Rotation (Math|Rotator|MakeRotator 0.0 0.0 (* DeltaSeconds (Variables|Rotator|GetRotatorSpeed) (Variables|Reactor|GetCooling) (Utilities|Select :Index (Variables|Default|GetStatus) :NewEnumerator0 1.0 :NewEnumerator1 (+ (Variables|Reactor|GetSmallBreakSpeed) (Math|Float|SelectFloat 0.1 0.0 (Variables|Default|GetIsTape))) :NewEnumerator2 (+ (Variables|Reactor|GetHugeBreakSpeed) (Math|Float|SelectFloat 0.1 0.0 (Variables|Default|GetIsTape))))))))))

(event EventSmallBreakingStop
  (|CallParentFunction)
  (Networking|SwitchHasAuthority
    (:Authority
      (CallFunction|SetEngineReactorSpeed (Variables|Reactor|GetCooling)))))

(event EventHugeBreakingStop
  (|CallParentFunction)
  (Networking|SwitchHasAuthority
    (:Authority
      (CallFunction|SetEngineReactorSpeed (* (Variables|Reactor|GetSmallBreakSpeed) (Variables|Reactor|GetCooling))))))

(event EventHugeBreakingStart
  (|CallParentFunction)
  (Networking|SwitchHasAuthority
    (:Authority
      (Default|SetFire (Variables|Default|GetFire) true)
      (CallFunction|SetEngineReactorSpeed (* (Variables|Reactor|GetHugeBreakSpeed) (Variables|Reactor|GetCooling))))))

(event EventSmallBreakingStart
  (|CallParentFunction)
  (Networking|SwitchHasAuthority
    (:Authority
      (CallFunction|SetEngineReactorSpeed (* (Variables|Reactor|GetSmallBreakSpeed) (Variables|Reactor|GetCooling))))))

(fn ConstructionScript
  (|CallParentFunction)
  (if (Variables|Reactor|GetIsFirst)
    (Variables|Default|SetTags (Utilities|Array|MakeArray "ReactorFirst"))
    (else
      (Variables|Default|SetTags (Utilities|Array|MakeArray "ReactorSecond"))))
  (Variables|Rotator|SetSoundLocation (Transformation|GetWorldLocation (Variables|Default|GetReactor))))

(fn SetCooling
  (params (Cooling :type Float%20%28double-precision%29) (IsAnotherCooling :type Boolean))
  (if IsAnotherCooling
    (Variables|Default|SetIsAnotherCooling true))
  (if (not (and (Variables|Default|GetIsAnotherCooling) (< Cooling (CallFunction|GetCoolingSpeed IsAnotherCooling))))
    (bind _output_get (Variables|Reactor|SetCooling Cooling))
    (CallFunction|SetEngineReactorSpeed (Utilities|Select :Index (Variables|Default|GetStatus) :NewEnumerator0 _output_get :NewEnumerator1 (* (Variables|Reactor|GetSmallBreakSpeed) (Variables|Reactor|GetCooling)) :NewEnumerator2 (* (Variables|Reactor|GetCooling) (Variables|Reactor|GetHugeBreakSpeed))))))

(fn SetSound)

(fn SetEngineReactorSpeed
  (params (Reactor%20speed :type Float%20%28double-precision%29))
  (if (Variables|/Game/Dynamic/Blueprints/Mechanisms/Moduls/BP_ModulBase.BP_ModulBase_C|GetIsDrop (Variables|Reactor|GetEngine))
    (Default|SetReactorSpeed (Variables|Reactor|GetAnotherEngine) Reactor%20speed true)
    (else
      (Default|SetReactorSpeed (Variables|Reactor|GetEngine) Reactor%20speed false))))

(fn ResendSpeed
  (CallFunction|SetCooling (Variables|Reactor|GetCooling) false))

(fn TakeDamage
  (params (DamageInfo :type S%20Damage%20Info%20Structure))
  (bind _newhealth (|CallParentFunction DamageInfo))
  (Utilities|FlowControl|Sequence
    (:then_0
      (if (Variables|Default|GetIsDrop)
        (bind _outactors (Actor|GetAllActorsOfClasswithTag "/Game/Dynamic/Blueprints/Mechanisms/Moduls/BP_Cooling.BP_Cooling_C" (select (Variables|Reactor|GetIsFirst) "CoolingFirst" "CoolingSecond")))
        (for _array_element _outactors
          (Networking|SwitchHasAuthority
            (:Authority
              (Default|ResendCooling _array_element))))))
    (:then_1
      (return _newhealth))))

(fn GetCurrentSpeed
  (return (* (Utilities|Select :Index (Variables|Default|GetStatus) :NewEnumerator0 1.0 :NewEnumerator1 (Variables|Reactor|GetSmallBreakSpeed) :NewEnumerator2 (Variables|Reactor|GetHugeBreakSpeed)) (Variables|Reactor|GetCooling))))

(fn GetCoolingSpeed
  (params (Another :type Boolean))
  (bind _outactors (Actor|GetAllActorsOfClasswithTag "/Game/Dynamic/Blueprints/Mechanisms/Moduls/BP_Cooling.BP_Cooling_C" (select (== Another (Variables|Reactor|GetIsFirst)) "CoolingSecond" "CoolingFirst")))
  (return (Default|GetCurrentSpeed (Utilities|Array|Get(acopy) _outactors))))

(fn SetSoundandLight
  (Audio|Components|Audio|SetVolumeMultiplier (Variables|Default|GetReactor) (Utilities|Select :Index (Variables|Default|GetStatus) :NewEnumerator0 1.0 :NewEnumerator1 0.5 :NewEnumerator2 0.0) :!class /Script/Engine.AudioComponent))