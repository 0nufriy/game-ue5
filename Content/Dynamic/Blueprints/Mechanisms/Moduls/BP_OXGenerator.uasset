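; Oxygen generator module, a breakable mechanism that controls oxygen supply through BP_ModulBoxColision volumes.
; Small breaks cut oxygen in "LittleOXBreak"-tagged volumes, huge breaks cut it everywhere, and each stop event restores the preceding level.
; TapeFix during status 2 temporarily restores oxygen to CameraTag-matched volumes, reverting after a delay if status remains 2.
; Alarm-light materials and generator sound volume follow module status.
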(event EventBeginPlay
  (|CallParentFunction))

(event Collision|EventActorBeginOverlap
  (params (OtherActor :type Actor%20Object%20Reference))
  (|CallParentFunction OtherActor) ; This node is disabled and will not be called.\nDrag off pins to build functionality.
)

(event EventTick
  (params (DeltaSeconds :type Float%20%28single-precision%29))
  (|CallParentFunction DeltaSeconds) ; This node is disabled and will not be called.\nDrag off pins to build functionality.
)

(event EventSmallBreakingStop
  (|CallParentFunction)
  (CallFunction|SetOxAll true))

(event EventHugeBreakingStop
  (|CallParentFunction)
  (CallFunction|SetOxAll true)
  (CallFunction|SetOxSome false))

(event EventHugeBreakingStart
  (|CallParentFunction)
  (CallFunction|SetOxAll false))

(event EventSmallBreakingStart
  (|CallParentFunction)
  (CallFunction|SetOxSome false))

(event EventTapeFix
  (params (Time :type Float%20%28double-precision%29))
  (if (== (Variables|Default|GetStatus) 2)
    (bind _outactors (Actor|GetAllActorsOfClasswithTag "/Game/Dynamic/Blueprints/Mechanisms/BoxColision/BP_ModulBoxColision.BP_ModulBoxColision_C" (Variables|Default|GetCameraTag)))
    (for _array_element _outactors
      (Default|SetOxPermanent _array_element true))
    (Variables|Default|SetIsTape true)
    (Utilities|FlowControl|Delay Time)
    (Variables|Default|SetIsTape false)
    (if (== (Variables|Default|GetStatus) 2)
      (for _array_element_2 _outactors
        (Default|SetOxPermanent _array_element_2 false)))
    (else
      (Variables|Default|SetIsTape true)
      (Utilities|FlowControl|Delay 0.2)
      (Variables|Default|SetIsTape false))))

(fn ConstructionScript
  (|CallParentFunction))

(fn SetOxAll
  (params (Ox :type Boolean))
  (bind _outactors (Actor|GetAllActorsOfClass "/Game/Dynamic/Blueprints/Mechanisms/BoxColision/BP_ModulBoxColision.BP_ModulBoxColision_C"))
  (for _array_element _outactors
    (Default|SetOxPermanent _array_element Ox)))

(fn SetOxSome
  (params (Ox :type Boolean))
  (bind _outactors (Actor|GetAllActorsOfClasswithTag "/Game/Dynamic/Blueprints/Mechanisms/BoxColision/BP_ModulBoxColision.BP_ModulBoxColision_C" "LittleOXBreak"))
  (for _array_element _outactors
    (Default|SetOxPermanent _array_element Ox)))

(fn SetLightandSound
  (params (ModulStatus :type E_ModuleStatus%20Enum :default "NewEnumerator0"))
  (Rendering|Material|SetMaterial (Variables|Default|GetSM_AlarmLight) 0 (Utilities|Select :Index ModulStatus :NewEnumerator0 "/Game/Static/Moduls/ox/Material/MI_AlarmLight_Glass_Green.MI_AlarmLight_Glass_Green" :NewEnumerator1 "/Game/Static/Moduls/ox/Material/MI_AlarmLight_Glass_Yellow.MI_AlarmLight_Glass_Yellow" :NewEnumerator2 "/Game/Static/Moduls/ox/Material/MI_AlarmLight_Glass_Inst.MI_AlarmLight_Glass_Inst"))
  (Rendering|Material|SetMaterial (Variables|Default|GetSM_AlarmLight) 1 (Utilities|Select :Index ModulStatus :NewEnumerator0 "/Game/Static/Moduls/ox/Material/MI_Light_Green.MI_Light_Green" :NewEnumerator1 "/Game/Static/Moduls/ox/Material/MI_Light_Yellow.MI_Light_Yellow" :NewEnumerator2 "/Game/Static/Moduls/ox/Material/MI_Light_Red.MI_Light_Red"))
  (Rendering|Material|SetMaterial (Variables|Default|GetSM_AlarmLight) 2 (Utilities|Select :Index ModulStatus :NewEnumerator0 "/Game/Static/Moduls/ox/Material/MI_AlarmLight_Green.MI_AlarmLight_Green" :NewEnumerator1 "/Game/Static/Moduls/ox/Material/MI_AlarmLight_Yellow.MI_AlarmLight_Yellow" :NewEnumerator2 "/Game/Static/Moduls/ox/Material/MI_AlarmLight.MI_AlarmLight"))
  (Audio|Components|Audio|SetVolumeMultiplier (Variables|Default|GetGeneratorOx) (Utilities|Select :Index ModulStatus :NewEnumerator0 1.0 :NewEnumerator1 0.5 :NewEnumerator2 0.0) :!class /Script/Engine.AudioComponent))

(fn SetSoundandLight
  (CallFunction|SetLightandSound (Variables|Default|GetStatus)))