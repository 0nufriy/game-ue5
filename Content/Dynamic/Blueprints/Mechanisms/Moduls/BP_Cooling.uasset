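; BP_Cooling is a breakable cooling module that feeds a cooling rate to its paired first or second reactor, found by tag.
; Server-side break events set the rate per damage state, with huge breaks lighting a fire and tape fixes adding a temporary boost.
; If the paired reactor's IsDrop is set, cooling goes to the other reactor.
; Rotor spin follows the current rate, and sounds follow the damage state.
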(event Custom|Rotation
  (params (DeltaRotation :type Rotator))
  (Transformation|AddRelativeRotation (Variables|Default|GetStaticMeshComponent) DeltaRotation false false)
  (Transformation|SetWorldLocation (Variables|Default|GetCoolingSpeed) (Variables|Default|GetSoundLocation) false false)
  (Transformation|SetWorldLocation (Variables|Default|GetCooling) (Variables|Default|GetSoundLocation) false false))

(event EventBeginPlay
  (|CallParentFunction)
  (bind _outactors (Actor|GetAllActorsOfClass "/Game/Dynamic/Blueprints/Mechanisms/Moduls/BP_Reactor.BP_Reactor_C"))
  (for _array_element _outactors
    (if (Actor|ActorHasTag _array_element (select (Variables|Cooling|GetIsFirst) "ReactorFirst" "ReactorSecond"))
      (Variables|Cooling|SetReactor _array_element)
      (else
        (Variables|Default|SetAnotherReactor _array_element)))))

(event EventTick
  (params (DeltaSeconds :type Float%20%28single-precision%29))
  (Networking|SwitchHasAuthority
    (:Authority
      (|CallParentFunction DeltaSeconds)
      (CallFunction|Rotation (Math|Rotator|MakeRotator 0.0 0.0 (* DeltaSeconds (CallFunction|GetCurrentSpeed) (Variables|Rotator|GetRotatorSpeed)))))))

(event EventSmallBreakingStop
  (|CallParentFunction)
  (Networking|SwitchHasAuthority
    (:Authority
      (CallFunction|SetReactorCooling 1.0))))

(event EventHugeBreakingStop
  (|CallParentFunction)
  (Networking|SwitchHasAuthority
    (:Authority
      (CallFunction|SetReactorCooling (Variables|Cooling|GetSmallBreakingCooling)))))

(event EventSmallBreakingStart
  (|CallParentFunction)
  (Networking|SwitchHasAuthority
    (:Authority
      (CallFunction|SetReactorCooling (Variables|Cooling|GetSmallBreakingCooling)))))

(event EventHugeBreakingStart
  (|CallParentFunction)
  (Networking|SwitchHasAuthority
    (:Authority
      (CallFunction|SetReactorCooling (Variables|Cooling|GetHugeBreakingCooling))
      (bind _fire (Variables|Default|GetFire)
        (:then
          (Default|SetFire _fire true))
        (:else)))))

(event EventTapeFix
  (params (Time :type Float%20%28double-precision%29))
  (Variables|Default|SetIsTape true)
  (if (!= (Variables|Default|GetStatus) 0)
    (CallFunction|SetReactorCooling (CallFunction|GetCurrentSpeed))
    (Utilities|FlowControl|Delay Time)
    (Variables|Default|SetIsTape false)
    (CallFunction|SetReactorCooling (CallFunction|GetCurrentSpeed))
    (else
      (Utilities|FlowControl|Delay Time)
      (Variables|Default|SetIsTape false))))

(fn ConstructionScript
  (|CallParentFunction)
  (Variables|Default|SetSoundLocation (Transformation|GetWorldLocation (Variables|Default|GetCoolingSpeed)))
  (Variables|Default|SetTags (Utilities|Array|MakeArray (select (Variables|Cooling|GetIsFirst) "CoolingFirst" "CoolingSecond"))))

(fn SetSound
  (switch Utilities|FlowControl|Switch|SwitchonE_ModuleStatus (Variables|Default|GetStatus)
    (:NewEnumerator0
      (Audio|Components|Audio|Play (Variables|Default|GetCoolingSpeed) 0.0)
      (Audio|Components|Audio|Stop (Variables|Default|GetCooling)))
    (:NewEnumerator1
      (Audio|Components|Audio|Stop (Variables|Default|GetCoolingSpeed))
      (Audio|Components|Audio|Play (Variables|Default|GetCooling) 0.0))
    (:NewEnumerator2
      (Audio|Components|Audio|Stop (Variables|Default|GetCoolingSpeed))
      (Audio|Components|Audio|Stop (Variables|Default|GetCooling)))))

(fn SetReactorCooling
  (params (Cooling :type Float%20%28double-precision%29))
  (if (Variables|/Game/Dynamic/Blueprints/Mechanisms/Moduls/BP_ModulBase.BP_ModulBase_C|GetIsDrop (Variables|Cooling|GetReactor))
    (Default|SetCooling (Variables|Default|GetAnotherReactor) Cooling true)
    (else
      (Default|SetCooling (Variables|Cooling|GetReactor) Cooling false))))

(fn ResendCooling
  (CallFunction|SetReactorCooling (CallFunction|GetCurrentSpeed)))

(fn GetCurrentSpeed
  (return (Utilities|Select :Index (Variables|Default|GetStatus) :NewEnumerator0 1.0 :NewEnumerator1 (+ (Variables|Cooling|GetSmallBreakingCooling) (Math|Float|SelectFloat 0.1 0.0 (Variables|Default|GetIsTape))) :NewEnumerator2 (+ (Variables|Cooling|GetHugeBreakingCooling) (Math|Float|SelectFloat 0.1 0.0 (Variables|Default|GetIsTape))))))

(fn SetSoundandLight
  (CallFunction|SetSound))