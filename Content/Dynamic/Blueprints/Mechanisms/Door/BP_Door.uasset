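; Sliding, damageable door between a module and a corridor that opens for the player through a timeline-driven trigger.
; DoorID tags pair it with its twin and corridor, and it waits while the twin is open.
; Opening and breaking update module and corridor state, including oxygen.
; Death jams it open, healing past half or temporary tape closes it, and dropping the module seals it against damage and repair.
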(event OnComponentBeginOverlap(Trigger)
  (params (OverlappedComponent :type Primitive%20Component%20Object%20Reference) (OtherActor :type Actor%20Object%20Reference) (OtherComp :type Primitive%20Component%20Object%20Reference) (OtherBodyIndex :type Integer) (bFromSweep :type Boolean) (SweepResult :type Hit%20Result%20Structure%20%28by%20ref%29))
  (if (Math|Boolean|ANDBoolean (not (Variables|Door|GetPermanentOpen)) (== (Utilities|GetClass OtherActor) "/Game/Dynamic/Blueprints/BP_PlayerCharacter.BP_PlayerCharacter_C") (!= (Utilities|GetClass OtherComp) "/Script/UMG.WidgetComponent"))
    (bind _anotherdoor (Variables|Door|GetAnotherDoor :!label _label)
      (:then
        (if (not (CallFunction|IsDoorOpen _anotherdoor))
          (Variables|Door|SetisOpen true :!label _label_2)
          (Default|CallOnOpened OtherActor)
          (Utilities|IsValid (Variables|Door|GetModulBox)
            (:Is%20Valid
              (Default|DoOptimize (Variables|Door|GetModulBox))
              (Utilities|IsValid (Variables|Door|GetCoridor)
                (:Is%20Valid
                  (Default|DoorOpen (Variables|Door|GetCoridor) (Variables|Door|GetModulBox))
                  (bind _doorposition (Timeline|Timeline_0 Play)
                    (:Update
                      (Transformation|SetWorldLocation (Variables|Default|GetStaticMeshComponent) (Math|Vector|Lerp(Vector) (Variables|Door|GetDoorClosed) (Variables|Door|GetDoorOpen) _doorposition) false false)
                      (Transformation|SetWorldLocation (Variables|Default|GetTrigger) (Variables|Door|GetTrigerStartWorldLocation) false false))
                    (:Finished
                      (if (Utilities|Operators|EqualEqual (Transformation|GetWorldLocation (Variables|Default|GetStaticMeshComponent)) (Variables|Door|GetDoorClosed) 0.1)
                        (Variables|Door|SetisOpen false)
                        (Utilities|IsValid (Variables|Door|GetModulBox)
                          (:Is%20Valid
                            (Default|DoOptimize (Variables|Door|GetModulBox))))))))
                (:Is%20Not%20Valid
                  (Timeline|Timeline_0 Play))))
            (:Is%20Not%20Valid
              (Timeline|Timeline_0 Play)))
          (else
            (Utilities|FlowControl|Delay 0.4)
            (if (> (Utilities|Array|Length (Collision|GetOverlappingActors (Variables|Default|GetTrigger) "/Game/Dynamic/Blueprints/BP_PlayerCharacter.BP_PlayerCharacter_C" :!class /Script/Engine.PrimitiveComponent)) 0)
              (goto _label)))))
      (:else
        (goto _label_2)))))

(event OnComponentEndOverlap(Trigger)
  (params (OverlappedComponent :type Primitive%20Component%20Object%20Reference) (OtherActor :type Actor%20Object%20Reference) (OtherComp :type Primitive%20Component%20Object%20Reference) (OtherBodyIndex :type Integer))
  (if (Math|Boolean|ANDBoolean (not (Variables|Door|GetPermanentOpen)) (== (Utilities|GetClass OtherActor) "/Game/Dynamic/Blueprints/BP_PlayerCharacter.BP_PlayerCharacter_C") (!= (Utilities|GetClass OtherComp) "/Script/UMG.WidgetComponent"))
    (bind _doorposition (Timeline|Timeline_0 Reverse)
      (:Update
        (Transformation|SetWorldLocation (Variables|Default|GetStaticMeshComponent) (Math|Vector|Lerp(Vector) (Variables|Door|GetDoorClosed) (Variables|Door|GetDoorOpen) _doorposition) false false)
        (Transformation|SetWorldLocation (Variables|Default|GetTrigger) (Variables|Door|GetTrigerStartWorldLocation) false false))
      (:Finished
        (if (Utilities|Operators|EqualEqual (Transformation|GetWorldLocation (Variables|Default|GetStaticMeshComponent)) (Variables|Door|GetDoorClosed) 0.1)
          (Variables|Door|SetisOpen false)
          (Utilities|IsValid (Variables|Door|GetModulBox)
            (:Is%20Valid
              (Default|DoOptimize (Variables|Door|GetModulBox)))))))))

(event OnDeath(BPC_HealthSystem)
  (CallFunction|HugeBreakingStart))

(event EventBeginPlay
  (bind _trigger (Variables|Default|GetTrigger))
  (bind _overlappingactors (Collision|GetOverlappingActors _trigger "/Game/Dynamic/Blueprints/Mechanisms/BoxColision/BP_ModulBoxColision.BP_ModulBoxColision_C" :!class /Script/Engine.PrimitiveComponent))
  (Utilities|FlowControl|Sequence
    (:then_0
      (bind _outactors (Actor|GetAllActorsOfClasswithTag "BP_Door_C" (CallFunction|IntIdtoTag (Variables|Door|GetDoorID))))
      (bind _array_element (Utilities|Array|ForEachLoopwithBreak _outactors :!label _label)
        (:LoopBody
          (if (!= _array_element self)
            (Variables|Door|SetAnotherDoor _array_element)
            (goto _label Break)))))
    (:then_1
      (bind _outactors_2 (Actor|GetAllActorsOfClasswithTag "/Game/Dynamic/Blueprints/Mechanisms/BoxColision/BP_CoridorBoxColision.BP_CoridorBoxColision_C" (CallFunction|IntIdtoTag (Variables|Door|GetDoorID))))
      (bind _array_element_2 (Utilities|Array|ForEachLoopwithBreak _outactors_2 :!label _label_2)
        (:LoopBody
          (Variables|Door|SetCoridor _array_element_2)
          (goto _label_2 Break))))
    (:then_2
      (if (Utilities|Array|IsNotEmpty _overlappingactors)
        _
        (else
          (Utilities|FlowControl|DelayUntilNextTick)))
      (bind _array_element_3 (Utilities|Array|ForEachLoopwithBreak _overlappingactors :!label _label_3)
        (:LoopBody
          (bind _asbp_modul_box_colision (Utilities|Casting|CastToBP_ModulBoxColision _array_element_3))
          (Variables|Door|SetModulBox _asbp_modul_box_colision)
          (goto _label_3 Break))))))

(event EventOptimizeCoridor
  (bind _coridor (Variables|Door|GetCoridor))
  (Utilities|IsValid _coridor
    (:Is%20Valid
      (Default|DoOptimize _coridor))))

(event EventTapeFix
  (params (Time :type Float%20%28double-precision%29))
  (if (and (Variables|Door|GetPermanentOpen) (not (Variables|Door|GetIsDrop)))
    (Variables|Door|SetIsType true)
    (CallFunction|HugeBreakingStop)
    (Variables|Door|SetPermanentOpen true)
    (Utilities|FlowControl|Delay Time)
    (Variables|Door|SetIsType false)
    (if (Variables|Door|GetPermanentOpen)
      (CallFunction|HugeBreakingStart))
    (else
      (Variables|Door|SetIsType true)
      (Utilities|FlowControl|Delay Time)
      (Variables|Door|SetIsType false))))

(event EventFix
  (params (FixValue :type Float%20%28double-precision%29) (PlayerStats :type BPC%20Player%20Stats%20System%20Object%20Reference) (ToolFixModulEfficiency :type Integer) (ToolFixHoleEfficiency :type Integer))
  (bind _bpc_healthsystem (Variables|Default|GetBPC_HealthSystem))
  (if (!= (Default|GetMaxHealth _bpc_healthsystem) (Default|GetCurrentHealth _bpc_healthsystem))
    (bind _fix (CallFunction|CalculateFixEfficiency FixValue PlayerStats ToolFixHoleEfficiency))
    (CallFunction|Heal _fix)))

(event EventDropModule
  (CallFunction|HugeBreakingStop)
  (Variables|Door|SetPermanentOpen true)
  (Variables|Door|SetIsDrop true))

(event EventEndOverlap
  (if (not (Variables|Door|GetPermanentOpen))
    (bind _doorposition (Timeline|Timeline_0 Reverse)
      (:Update
        (Transformation|SetWorldLocation (Variables|Default|GetStaticMeshComponent) (Math|Vector|Lerp(Vector) (Variables|Door|GetDoorClosed) (Variables|Door|GetDoorOpen) _doorposition) false false)
        (Transformation|SetWorldLocation (Variables|Default|GetTrigger) (Variables|Door|GetTrigerStartWorldLocation) false false))
      (:Finished
        (if (Utilities|Operators|EqualEqual (Transformation|GetWorldLocation (Variables|Default|GetStaticMeshComponent)) (Variables|Door|GetDoorClosed) 0.1)
          (Variables|Door|SetisOpen false)
          (Utilities|IsValid (Variables|Door|GetModulBox)
            (:Is%20Valid
              (Default|DoOptimize (Variables|Door|GetModulBox)))))))))

(event EventHugeBreakingStart
  (Variables|Door|SetPermanentOpen true)
  (Variables|Door|SetisOpen false)
  (Utilities|IsValid (Variables|Door|GetModulBox)
    (:Is%20Valid
      (Default|DoOptimize (Variables|Door|GetModulBox))
      (Utilities|IsValid (Variables|Door|GetCoridor)
        (:Is%20Valid
          (CallFunction|OpenDoorPerm)
          (bind _doorposition (Timeline|Timeline_0 Play)
            (:Update
              (Transformation|SetWorldLocation (Variables|Default|GetStaticMeshComponent) (Math|Vector|Lerp(Vector) (Variables|Door|GetDoorClosed) (Variables|Door|GetDoorOpen) _doorposition) false false)
              (Transformation|SetWorldLocation (Variables|Default|GetTrigger) (Variables|Door|GetTrigerStartWorldLocation) false false))
            (:Finished
              (if (Utilities|Operators|EqualEqual (Transformation|GetWorldLocation (Variables|Default|GetStaticMeshComponent)) (Variables|Door|GetDoorClosed) 0.1)
                (Variables|Door|SetisOpen false)
                (Utilities|IsValid (Variables|Door|GetModulBox)
                  (:Is%20Valid
                    (Default|DoOptimize (Variables|Door|GetModulBox))))))))
        (:Is%20Not%20Valid
          (Timeline|Timeline_0 Play))))
    (:Is%20Not%20Valid
      (Timeline|Timeline_0 Play))))

(event EventHugeBreakingStop
  (Class|AIPerceptionStimuliSourceComponent|RegisterforSense (Variables|Default|GetAIPerceptionStimuliSource) "/Script/AIModule.AISense_Sight")
  (Variables|Door|SetPermanentOpen false)
  (Utilities|IsValid (Variables|Door|GetModulBox)
    (:Is%20Valid
      (Default|SetCoridorOx (Variables|Door|GetModulBox) self true)
      (Utilities|IsValid (Variables|Door|GetCoridor)
        (:Is%20Valid
          (Variables|/Game/Dynamic/Blueprints/Mechanisms/BoxColision/BP_CoridorBoxColision.BP_CoridorBoxColision_C|SetPermanentBreath (Variables|Door|GetCoridor) true)
          (Default|DoorOpen (Variables|Door|GetCoridor) (Variables|Door|GetModulBox))
          (CallFunction|RecalculateAllDoor)
          (bind _doorposition (Timeline|Timeline_0 Reverse)
            (:Update
              (Transformation|SetWorldLocation (Variables|Default|GetStaticMeshComponent) (Math|Vector|Lerp(Vector) (Variables|Door|GetDoorClosed) (Variables|Door|GetDoorOpen) _doorposition) false false)
              (Transformation|SetWorldLocation (Variables|Default|GetTrigger) (Variables|Door|GetTrigerStartWorldLocation) false false))
            (:Finished
              (if (Utilities|Operators|EqualEqual (Transformation|GetWorldLocation (Variables|Default|GetStaticMeshComponent)) (Variables|Door|GetDoorClosed) 0.1)
                (Variables|Door|SetisOpen false)
                (Utilities|IsValid (Variables|Door|GetModulBox)
                  (:Is%20Valid
                    (Default|DoOptimize (Variables|Door|GetModulBox))))))))
        (:Is%20Not%20Valid
          (Timeline|Timeline_0 Reverse))))
    (:Is%20Not%20Valid
      (Timeline|Timeline_0 Reverse))))

(fn ConstructionScript
  (Variables|Default|SetTags (Utilities|Array|MakeArray (CallFunction|IntIdtoTag (Variables|Door|GetDoorID)) "Door"))
  (Variables|Door|SetDoorOpen (+ (Transformation|GetWorldLocation (Variables|Default|GetStaticMeshComponent)) (Variables|Door|GetDoorOpen)))
  (Variables|Door|SetDoorClosed (+ (Transformation|GetWorldLocation (Variables|Default|GetStaticMeshComponent)) (Variables|Door|GetDoorClosed)))
  (Variables|Door|SetTrigerStartWorldLocation (Transformation|GetWorldLocation (Variables|Default|GetTrigger))))

(fn IntIdtoTag
  (params (InInt :type Integer))
  (return (Utilities|String|StringToName (Utilities|String|Append (Utilities|String|MakeLiteralString "Door") (Utilities|String|ToString(Integer) InInt)))))

(fn IsDoorOpen
  (return (Variables|Door|GetisOpen)))

(fn Heal
  (params (HealAmount :type Float%20%28double-precision%29))
  (if (not (Variables|Door|GetIsDrop))
    (bind _newhealth (|CallParentFunction HealAmount))
    (Utilities|FlowControl|Sequence
      (:then_0
        (bind _maxhealth (CallFunction|GetMaxHealth))
        (if (and (> (/ _newhealth _maxhealth) 0.5) (Variables|Door|GetPermanentOpen))
          (CallFunction|HugeBreakingStop)))
      (:then_1
        (return 0.0)))))

(fn RecalculateAllDoor
  (bind _outactors (Actor|GetAllActorsOfClass "BP_Door_C"))
  (for _array_element _outactors
    (bind _permanentopen (Class|BPIDoor|GetPermanentOpen(Message) _array_element))
    (if _permanentopen
      (CallFunction|OpenDoorPerm _array_element))))

(fn OpenDoorPerm
  (Default|DoorOpenwhenPermanent (Variables|Door|GetCoridor) (Variables|Door|GetModulBox) self))

(fn TakeDamage
  (params (DamageInfo :type S%20Damage%20Info%20Structure))
  (if (not (Variables|Door|GetIsDrop))
    (bind _newhealth (|CallParentFunction DamageInfo))
    (return _newhealth)))

(fn CalculateFixEfficiency
  (params (FixValue :type Float%20%28double-precision%29) (PlayerStat :type BPC%20Player%20Stats%20System%20Object%20Reference) (ToolFixEfficiency :type Integer))
  (return (* FixValue ToolFixEfficiency (Variables|/Game/Dynamic/Blueprints/Components/StatsSystemComponent/Player/BPC_Player_StatsSystem.BPC_Player_StatsSystem_C|GetSolderingSkill PlayerStat))))

(fn GetAnotherDoor
  (return (Variables|Door|GetAnotherDoor)))

(fn GetCoridor
  (return (Variables|Door|GetCoridor)))

(fn GetHealthPercent
  (bind _bpc_healthsystem (Variables|Default|GetBPC_HealthSystem))
  (return (/ (Default|GetCurrentHealth _bpc_healthsystem) (Default|GetMaxHealth _bpc_healthsystem))))

(fn GetIsDrop
  (return (Variables|Door|GetIsDrop)))

(fn GetIsTape
  (return (Variables|Door|GetIsType)))

(fn GetModule
  (return (Variables|Door|GetModulBox)))

(fn GetPermanentOpen
  (return (Variables|Door|GetPermanentOpen)))

(fn GetSelf
  (return self))

(fn IsBig
  (return (Variables|Door|GetIsBigDoor)))

(fn IsOpenDoor
  (return (Variables|Door|GetisOpen)))