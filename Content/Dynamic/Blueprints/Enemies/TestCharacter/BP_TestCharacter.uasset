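; Test enemy character with placeholder health and combat functions that reacts to damage by wandering nearby.
; TakeDamage calls SetFocus on its AI controller and starts MoveToRandomLocation, which chains AI moves to random reachable points until a movement counter runs out.
; Health, healing, death and attack-token functions return fixed values, and TakeDamage applies no damage.
; BeginPlay looks up a player-stats row by Class, but the result is unused.
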(event Custom|MoveToRandomLocation
  (bind _returnvalue (Transformation|GetActorLocation))
  (bind (_randomlocation _returnvalue_2) (AI|Navigation|GetRandomReachablePointinRadius _returnvalue 3.5e+02 0 0))
  (Variables|Default|SetMovementCounter (Variables|Default|GetMaxMovements))
  (if (> (Variables|Default|GetMovementCounter) 0) :!label _label
    (Variables|Default|SetMovementCounter (- (Variables|Default|GetMovementCounter) 1))
    (if _returnvalue_2
      (AI|AIMoveTo self _randomlocation 0 5.0 false
        (:OnSuccess
          (goto _label))))))

(event EventBeginPlay
  (Variables|Default|SetMovementCounter (Variables|Default|GetMaxMovements))
  (Utilities|GetDataTableRow "/Game/Dynamic/Blueprints/Character/DT_PlayerStats.DT_PlayerStats" (Utilities|Name|EnumtoName (Variables|Default|GetClass))))

(fn ConstructionScript)

(fn GetCurrentHealth
  (return 0.0))

(fn GetMaxHealth
  (return 0.0))

(fn Heal
  (params (HealAmount :type Float%20%28double-precision%29))
  (return 0.0))

(fn IsDead
  (return false))

(fn ReserveAttackTokens
  (params (Amount :type Integer))
  (return true))

(fn TakeDamage
  (params (DamageInfo :type S%20Damage%20Info%20Structure))
  (AI|SetFocus (AI|GetAIController self))
  (CallFunction|MovetoRandomLocation)
  (return 0.0))