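; BP_TestEnemies is a test enemy actor that exposes health and damage functions backed by a BPC_HealthSystem component.
; TakeDamage, Heal, IsDead and the health getters forward to the component, whose OnDeath event destroys the actor on death.
; ReserveAttackTokens always returns false, and an unconnected branch holds leftover environmental damage-over-time logic for a hit actor.
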(event Custom|DeathEvent
  (Actor|DestroyActor))

(event EventBeginPlay
  (EventDispatchers|BindEventtoOnDeath (Variables|Default|GetBPC_HealthSystem) (delegate Custom|DeathEvent)))

(event Collision|EventActorBeginOverlap
  (params (OtherActor :type Actor%20Object%20Reference)))

(event EventTick
  (params (DeltaSeconds :type Float%20%28single-precision%29)))

(event Collision|EventHit
  (params (MyComp :type Primitive%20Component%20Object%20Reference) (Other :type Actor%20Object%20Reference) (OtherComp :type Primitive%20Component%20Object%20Reference) (bSelfMoved :type Boolean) (HitLocation :type Vector :default "0, 0, 0") (HitNormal :type Vector :default "0, 0, 0") (NormalImpulse :type Vector :default "0, 0, 0") (Hit :type Hit%20Result%20Structure%20%28by%20ref%29)))

(fn ConstructionScript)

(fn ReserveAttackTokens
  (params (Amount :type Integer))
  (return false))

(fn IsDead
  (return (Default|IsDead (Variables|Default|GetBPC_HealthSystem))))

(fn Heal
  (params (HealAmount :type Float%20%28double-precision%29))
  (bind _newhealth (Default|Heal (Variables|Default|GetBPC_HealthSystem) HealAmount))
  (return _newhealth))

(fn GetMaxHealth
  (return (Default|GetMaxHealth (Variables|Default|GetBPC_HealthSystem))))

(fn GetCurrentHealth
  (return (Default|GetCurrentHealth (Variables|Default|GetBPC_HealthSystem))))

(fn TakeDamage
  (params (DamageInfo :type S%20Damage%20Info%20Structure))
  (bind _currenthealth (Default|TakeDamage (Variables|Default|GetBPC_HealthSystem) DamageInfo))
  (return _currenthealth))