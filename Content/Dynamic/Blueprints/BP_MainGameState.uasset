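; Main game state that signals when all players' characters have loaded in a multiplayer match.
; The RepNotify on the PlayerCharacters array compares its length with the player count fetched from the game instance through an interface message.
; Once the array holds at least that many entries, it fires the OnAllCharactersLoaded dispatcher and passes the character list along.
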(fn ConstructionScript)

(fn OnRepPlayerCharacters
  (bind _returnvalue (CallFunction|AllPlayersLoaded))
  (if _returnvalue
    (Default|CallOnAllCharactersLoaded (Variables|GameState|GetPlayerCharacters))))

(fn AllPlayersLoaded
  (bind _count (Class|BPIMultiplayer|GetMultiplayerPlayerCount(Message) (Game|GetGameInstance)))
  (return (<= _count (Utilities|Array|Length (Variables|GameState|GetPlayerCharacters)))))