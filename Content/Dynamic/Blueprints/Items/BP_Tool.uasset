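; Base handheld tool item that repairs actors implementing BPI_Fix while held in use and draining ammo.
; The authority applies fixes from the aim hit, scaled by DeltaTime with module and hole efficiencies, while remotes call an empty cosmetic hook.
; Guarded active and target states drive use sounds and the owner's health-percent message.
; The locally controlled owner gets an ammo HUD widget, and recharging is authority-only and clamped.
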(event Custom|Deactivate
  ;[0.01042 0.01042 0.01042] Usage Start / Stop
  (Variables|Default|SetbIsActive false)
  (CallFunction|TryLooseTarget)
  (Audio|Components|Audio|Stop (Variables|Default|GetUseSound))
  (Audio|Components|Audio|Stop (Variables|Default|GetUseActiveSound)))

(event Custom|Fix
  (params (PlayerStat :type BPC%20Player%20Stats%20System%20Object%20Reference) (DeltaTime :type Float%20%28double-precision%29) (HitResult :type Hit%20Result%20Structure))
  (bind _hitactor (Collision|BreakHitResult HitResult))
  (Class|BPIFix|Fix(Message) _hitactor DeltaTime PlayerStat (Variables|Fix|GetFixModulEfficiency) (Variables|Fix|GetFixHoleEfficiency))
  (bind _percent (Class|BPIFix|GetHealthPercent(Message) _hitactor))
  (Class|BPIWidgetFix|SetWidget(Message) (Variables|Default|GetCurrentOwner) (.ImpactPoint (Collision|BreakHitResult HitResult)) _percent)
  (CallFunction|TryGetTarget))

(event Custom|UseUniq
  (params (AimComponent :type BP%20Grab%20Component%20Object%20Reference) (PlayerStats :type BPC%20Player%20Stats%20System%20Object%20Reference) (DeltaTime :type Float%20%28double-precision%29))
  ;[0.01042 0.01042 0.01042] Hand Item Interface
  (bind _hitresult (Default|AimtoFix AimComponent))
  (CallFunction|UsewithHitResult PlayerStats _hitresult DeltaTime))

(event Custom|TryGetTarget
  ;[0.01042 0.01042 0.01042] Target Got / Lost
  (if (not (Variables|Default|GetbHasTarget))
    (CallFunction|GotTarget)))

(event Custom|RemoveWidget
  ;[0.01042 0.01042 0.01042] HUD Update
  (Widget|RemovefromParent (Variables|Default|GetWidget))
  (Variables|Default|SetWidget 0))

(event Custom|TryLooseTarget
  ;[0.01042 0.01042 0.01042] Target Got / Lost
  (if (Variables|Default|GetbHasTarget)
    (CallFunction|LostTarget)))

(event Custom|TryActivate
  ;[0.01042 0.01042 0.01042] Usage Start / Stop
  (if (not (Variables|Default|GetbIsActive))
    (CallFunction|Activate)))

(event Custom|TryDeactivate
  ;[0.01042 0.01042 0.01042] Usage Start / Stop
  (if (Variables|Default|GetbIsActive)
    (CallFunction|Deactivate)))

(event Custom|GotTarget
  ;[0.01042 0.01042 0.01042] Target Got / Lost
  (Variables|Default|SetbHasTarget true)
  (Audio|Components|Audio|Play (Variables|Default|GetUseActiveSound) 0.0))

(event Custom|Activate
  ;[0.01042 0.01042 0.01042] Usage Start / Stop
  (Variables|Default|SetbIsActive true)
  (if (> (Variables|Fix|GetAmmo) 0.0)
    (Audio|Components|Audio|Play (Variables|Default|GetUseSound) 0.0)))

(event Custom|UseWithHitResult
  (params (PlayerStat :type BPC%20Player%20Stats%20System%20Object%20Reference) (HitResult :type Hit%20Result%20Structure) (DeltaSecond :type Float%20%28double-precision%29))
  (bind (_bblockinghit _binitialoverlap _time _distance _location _impactpoint _normal _impactnormal _physmat _hitactor) (Collision|BreakHitResult HitResult))
  ;[0.01042 0.01042 0.01042] Hand Item Interface
  (if (and _bblockinghit (Utilities|DoesObjectImplementInterface _hitactor "/Game/Dynamic/Interfaces/BPI_Fix.BPI_Fix_C"))
    (CallFunction|Fix PlayerStat DeltaSecond HitResult)
    (else
      (CallFunction|TryLooseTarget))))

(event Custom|LostTarget
  ;[0.01042 0.01042 0.01042] Target Got / Lost
  (Variables|Default|SetbHasTarget false)
  (Audio|Components|Audio|Stop (Variables|Default|GetUseActiveSound))
  (Class|BPIWidgetFix|ClearWidget(Message) (Variables|Default|GetCurrentOwner)))

(event Custom|SetAmmoOnHUD
  ;[0.01042 0.01042 0.01042] HUD Update
  (Default|SetAmmo (Variables|Default|GetWidget) (Variables|Fix|GetAmmo) (Variables|Fix|GetAmmoMax)))

(event EventBeginPlay
  (|CallParentFunction) ; This node is disabled and will not be called.\nDrag off pins to build functionality.
)

(event Collision|EventActorBeginOverlap
  (params (OtherActor :type Actor%20Object%20Reference))
  (|CallParentFunction OtherActor) ; This node is disabled and will not be called.\nDrag off pins to build functionality.
)

(event EventUse
  (params (AimComponent :type BP%20Grab%20Component%20Object%20Reference) (PlayerStats :type BPC%20Player%20Stats%20System%20Object%20Reference) (DeltaTime :type Float%20%28double-precision%29))
  ;[0.01042 0.01042 0.01042] Hand Item Interface
  (if (> (Variables|Fix|GetAmmo) 0.0)
    (Utilities|FlowControl|Sequence
      (:then_0
        (CallFunction|TryActivate))
      (:then_1
        (Variables|Fix|SetAmmo (- (Variables|Fix|GetAmmo) DeltaTime))
        (if (Pawn|IsLocallyControlled (Variables|Default|GetCurrentOwner))
          (CallFunction|SetAmmoonHUD)))
      (:then_2
        (Networking|SwitchHasAuthority
          (:Authority
            (CallFunction|UseUniq AimComponent PlayerStats DeltaTime))
          (:Remote
            (bind _hitresult (Default|AimtoFix AimComponent))
            (CallFunction|UseHitResultCosmetic _hitresult)))))
    (else
      (CallFunction|TryDeactivate))))

(event EventReleasUse
  ;[0.01042 0.01042 0.01042] Hand Item Interface
  (|CallParentFunction)
  (CallFunction|TryDeactivate))

(event EventTick
  (params (DeltaSeconds :type Float%20%28single-precision%29))
  (|CallParentFunction DeltaSeconds) ; This node is disabled and will not be called.\nDrag off pins to build functionality.
)

(event EventDrop
  (params (Impulse :type Vector :default "0, 0, 0"))
  ;[0.01042 0.01042 0.01042] Intercat / Drop
  (|CallParentFunction Impulse)
  (Utilities|FlowControl|Sequence
    (:then_0
      (CallFunction|TryDeactivate))
    (:then_1
      (Networking|SwitchHasAuthority
        (:Authority
          (CallFunction|RemoveWidget))))))

(event EventInteract
  (params (Owner :type Pawn%20Object%20Reference))
  (bind _currentowner (Variables|Default|GetCurrentOwner))
  ;[0.01042 0.01042 0.01042] Intercat / Drop
  (|CallParentFunction Owner)
  (Utilities|FlowControl|Sequence
    (:then_0
      (if (Pawn|IsLocallyControlled _currentowner)
        (bind _returnvalue (UserInterface|CreateWidget "/Game/Dynamic/Blueprints/UI/GrabItem/UI_Tools.UI_Tools_C" (.AsPlayer%20Controller (Utilities|Casting|CastToPlayerController (Pawn|GetController _currentowner)))))
        (bind _output_get (Variables|Default|SetWidget _returnvalue))
        (UserInterface|Viewport|AddtoPlayerScreen _output_get)
        (CallFunction|SetAmmoonHUD)))))

(event EventAddCurrentCharge
  (params (Amount :type Float%20%28double-precision%29))
  (Networking|SwitchHasAuthority
    (:Authority
      (Variables|Fix|SetAmmo (Math|Float|Clamp(Float) (+ Amount (Variables|Fix|GetAmmo)) 0.0 (Variables|Fix|GetAmmoMax)))
      (CallFunction|SetAmmoonHUD))))

(fn ConstructionScript
  (|CallParentFunction))

(fn GetToolAmmoType
  (return (Variables|Default|GetToolAmmoType)))

(fn UseHitResultCosmetic
  (params (HitResult :type Hit%20Result%20Structure)))

(fn GetCurrentCharge
  (return (Variables|Fix|GetAmmo)))

(fn GetMaxCharge
  (return (Variables|Fix|GetAmmoMax)))