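; Fire extinguisher tool that puts out burning objects the player aims at and plays an effect while active.
; On use, it gets targets from the aim component's AimToExtinguish and sends the extinguish message to each one implementing BPI_Fire.
; Activate and Deactivate call the parent logic, then switch the usage VFX on or off.
; Player stats and delta time are passed to the extinguish event but go unused.
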(event Custom|Extingush
  (params (PlayerStats :type BPC%20Player%20Stats%20System%20Object%20Reference) (Deltatime :type Float%20%28double-precision%29) (Array :type Array%20of%20Actor%20Object%20References))
  (for _array_element Array
    (if (Utilities|DoesObjectImplementInterface _array_element "/Game/Dynamic/Interfaces/BPI_Fire.BPI_Fire_C")
      (Class|BPIFire|SetIsExtingush(Message) _array_element true))))

(event Custom|ActivateUsageFX
  ;[0.01042 0.01042 0.01042] VFX
  (Components|Activation|Activate (Variables|Default|GetUsageVFX) false))

(event Custom|DeactivateUsageFX
  ;[0.01042 0.01042 0.01042] VFX
  (Components|Activation|Deactivate (Variables|Default|GetUsageVFX)))

(event EventUseUniq
  (params (AimComponent :type BP%20Grab%20Component%20Object%20Reference) (PlayerStats :type BPC%20Player%20Stats%20System%20Object%20Reference) (DeltaTime :type Float%20%28double-precision%29))
  (bind _actor (Default|AimtoExtinguish AimComponent))
  (CallFunction|Extingush PlayerStats DeltaTime _actor))

(event EventActivate
  ;[0.01042 0.01042 0.01042] Activate / Deactivate
  (|CallParentFunction)
  (CallFunction|ActivateUsageFX))

(event EventDeactivate
  ;[0.01042 0.01042 0.01042] Activate / Deactivate
  (|CallParentFunction)
  (CallFunction|DeactivateUsageFX))

(fn ConstructionScript
  (|CallParentFunction))