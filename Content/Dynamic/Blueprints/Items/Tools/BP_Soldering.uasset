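; BP_Soldering is a soldering repair tool that adds laser and soldering visual effects to its parent tool class's behavior.
; Activate and Deactivate toggle the laser, while gaining or losing a target toggles the soldering effect.
; Hit-result use, both regular and cosmetic, sets the beam end to the impact point, or trace end on a miss.
; Fix moves the soldering effect to the impact point and passes it the surface normal.
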(event Custom|UpdateSolderingVFX
  (params (HitLocation :type Vector) (ImpactNormal :type Vector))
  ;[0.01042 0.01042 0.01042] VFX
  (Transformation|SetWorldLocation (Variables|Default|GetSolderingVFX) HitLocation false true)
  (Niagara|SetNiagaraVariable(Vector3) (Variables|Default|GetSolderingVFX) "ImpactNormal" ImpactNormal))

(event Custom|ActivateSolderingVFX
  ;[0.01042 0.01042 0.01042] VFX
  (Components|Activation|Activate (Variables|Default|GetSolderingVFX) true))

(event Custom|DeactivateSolderingVFX
  ;[0.01042 0.01042 0.01042] VFX
  (Components|Activation|Deactivate (Variables|Default|GetSolderingVFX)))

(event Custom|ActivateLaserFX
  ;[0.01042 0.01042 0.01042] VFX
  (Components|Activation|Activate (Variables|Default|GetLaserVFX) true))

(event Custom|DeactivateLaserFX
  ;[0.01042 0.01042 0.01042] VFX
  (Components|Activation|Deactivate (Variables|Default|GetLaserVFX)))

(event Custom|UpdateLaserFX
  (params (HitLocation :type Vector))
  ;[0.01042 0.01042 0.01042] VFX
  (Niagara|SetNiagaraVariable(Vector3) (Variables|Default|GetLaserVFX) "BeamEnd" HitLocation))

(event EventBeginPlay
  (|CallParentFunction) ; This node is disabled and will not be called.\nDrag off pins to build functionality.
)

(event Collision|EventActorBeginOverlap
  (params (OtherActor :type Actor%20Object%20Reference))
  (|CallParentFunction OtherActor) ; This node is disabled and will not be called.\nDrag off pins to build functionality.
)

(event EventUsewithHitResult
  (params (PlayerStat :type BPC%20Player%20Stats%20System%20Object%20Reference) (HitResult :type Hit%20Result%20Structure) (DeltaSecond :type Float%20%28double-precision%29))
  (bind (_bblockinghit _binitialoverlap _time _distance _location _impactpoint _normal _impactnormal _physmat _hitactor _hitcomponent _hitbonename _bonename _hititem _elementindex _faceindex _tracestart _traceend) (Collision|BreakHitResult HitResult))
  (|CallParentFunction PlayerStat HitResult DeltaSecond)
  (CallFunction|UpdateLaserFX (Math|Vector|SelectVector _impactpoint _traceend _bblockinghit)))

(event EventTick
  (params (DeltaSeconds :type Float%20%28single-precision%29))
  (|CallParentFunction DeltaSeconds) ; This node is disabled and will not be called.\nDrag off pins to build functionality.
)

(event EventFix
  (params (PlayerStat :type BPC%20Player%20Stats%20System%20Object%20Reference) (DeltaTime :type Float%20%28double-precision%29) (HitResult :type Hit%20Result%20Structure))
  (bind (_bblockinghit _binitialoverlap _time _distance _location _impactpoint _normal _impactnormal) (Collision|BreakHitResult HitResult))
  (|CallParentFunction PlayerStat DeltaTime HitResult)
  (CallFunction|UpdateSolderingVFX _impactpoint _impactnormal))

(event EventActivate
  ;[0.01042 0.01042 0.01042] Activate / Deactivate
  (|CallParentFunction)
  (CallFunction|ActivateLaserFX))

(event EventGotTarget
  ;[0.01042 0.01042 0.01042] Target Got / Lost
  (|CallParentFunction)
  (CallFunction|ActivateSolderingVFX))

(event EventLostTarget
  ;[0.01042 0.01042 0.01042] Target Got / Lost
  (|CallParentFunction)
  (CallFunction|DeactivateSolderingVFX))

(event EventDeactivate
  ;[0.01042 0.01042 0.01042] Activate / Deactivate
  (|CallParentFunction)
  (CallFunction|DeactivateLaserFX))

(fn ConstructionScript
  (|CallParentFunction))

(fn UseHitResultCosmetic
  (params (HitResult :type Hit%20Result%20Structure))
  (bind (_bblockinghit _binitialoverlap _time _distance _location _impactpoint _normal _impactnormal _physmat _hitactor _hitcomponent _hitbonename _bonename _hititem _elementindex _faceindex _tracestart _traceend) (Collision|BreakHitResult HitResult))
  (|CallParentFunction HitResult)
  (CallFunction|UpdateLaserFX (Math|Vector|SelectVector _impactpoint _traceend _bblockinghit)))