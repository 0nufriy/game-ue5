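; BP_DebugDamage is a debug tool item that, while used, deals physical damage to the aimed-at actor if it implements the BPI_Fix interface.
; Use requires ammo, updates the ammo HUD and passes the aim hit to DamageMulticast, which applies time-scaled, non-stunning damage.
; It shows target health at the impact point through the owner's widget and plays a looping-use sound, clearing both for invalid targets.
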(event Custom|DamageMulticast
  (params (ActorToFix :type Actor%20Object%20Reference) (DeltaTime :type Float%20%28double-precision%29) (ImpactPoint :type Vector))
  (if (Utilities|DoesObjectImplementInterface ActorToFix "/Game/Dynamic/Interfaces/BPI_Fix.BPI_Fix_C")
    (Class|BPIDamagable|TakeDamage(Message) ActorToFix (Utilities|Struct|MakeS_DamageInfo (* DeltaTime 1e+01) "/Game/Dynamic/Blueprints/DamageTypes/BP_PhysicalDamage.BP_PhysicalDamage_C" false))
    (bind _percent (Class|BPIFix|GetHealthPercent(Message) ActorToFix))
    (Class|BPIWidgetFix|SetWidget(Message) (Variables|Default|GetCurrentOwner) ImpactPoint _percent)
    (if (not (Audio|Components|Audio|IsPlaying (Variables|Default|GetUseActiveSound)))
      (Audio|Components|Audio|Play (Variables|Default|GetUseActiveSound) 0.0))
    (else
      (Audio|Components|Audio|Stop (Variables|Default|GetUseActiveSound))
      (Class|BPIWidgetFix|ClearWidget(Message) (Variables|Default|GetCurrentOwner)))))

(event EventBeginPlay
  (|CallParentFunction) ; This node is disabled and will not be called.\nDrag off pins to build functionality.
)

(event Collision|EventActorBeginOverlap
  (params (OtherActor :type Actor%20Object%20Reference))
  (|CallParentFunction OtherActor) ; This node is disabled and will not be called.\nDrag off pins to build functionality.
)

(event EventTick
  (params (DeltaSeconds :type Float%20%28single-precision%29))
  (|CallParentFunction DeltaSeconds) ; This node is disabled and will not be called.\nDrag off pins to build functionality.
)

(event EventUse
  (params (AimComponent :type BP%20Grab%20Component%20Object%20Reference) (PlayerStats :type BPC%20Player%20Stats%20System%20Object%20Reference) (DeltaTime :type Float%20%28double-precision%29))
  (if (> (Variables|Default|GetAmmo) 0.0)
    (CallFunction|SetAmmoonHUD)
    (bind _hitresult (Default|AimtoFix AimComponent))
    (CallFunction|DamageMulticast (.HitActor (Collision|BreakHitResult _hitresult)) DeltaTime (.ImpactPoint (Collision|BreakHitResult _hitresult)))
    (else
      (CallFunction|StopUse))))

(fn ConstructionScript
  (|CallParentFunction))