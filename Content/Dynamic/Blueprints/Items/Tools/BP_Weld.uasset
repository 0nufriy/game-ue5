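; BP_Weld is a welding tool item that fixes targets and deals damage over time to enemies it hits.
; It extends parent tool events, toggling a laser beam on activation and welding sparks on target gain or loss.
; Use and cosmetic hits steer the beam end, while Fix positions the welding effect.
; Enemy-tagged hits trigger damage from authority through a multicast, and other blocking hits spawn randomly rotated, fading scorch decals.
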(event Custom|UpdateWeldingFX
  (params (HitLocation :type Vector) (ImpactNormal :type Vector))
  (bind _weldingvfx (Variables|Default|GetWeldingVFX))
  ;[0.01042 0.01042 0.01042] VFX
  (Transformation|SetWorldLocation _weldingvfx HitLocation false true)
  (Niagara|SetNiagaraVariable(Vector3) _weldingvfx "ImpactNormal" ImpactNormal))

(event Custom|DeactivateWieldingVX
  ;[0.01042 0.01042 0.01042] VFX
  (Components|Activation|Deactivate (Variables|Default|GetWeldingVFX)))

(event Custom|ActivateWeldingFX
  ;[0.01042 0.01042 0.01042] VFX
  (Components|Activation|Activate (Variables|Default|GetWeldingVFX) true))

(event Custom|ActivateLaserFX
  ;[0.01042 0.01042 0.01042] VFX
  (Components|Activation|Activate (Variables|Default|GetLaserVFX) true))

(event Custom|DeactivateLaserFX
  ;[0.01042 0.01042 0.01042] VFX
  (Components|Activation|Deactivate (Variables|Default|GetLaserVFX)))

(event Custom|UpdateLaserFX
  (params (HitLocation :type Vector))
  ;[0.01042 0.01042 0.01042] VFX
  (Niagara|SetNiagaraVariable(Vector3) (Variables|Default|GetLaserVFX) "BeamEnd" HitLocation))

(event Custom|SpawnDecal
  (params (ActorToAttachTo :type Actor%20Object%20Reference) (AttachPoint :type Vector) (Normal :type Vector))
  (bind _returnvalue (Class|GameplayStatics|SpawnDecalAttached "/Game/Dynamic/VFX/Niagara/Welding/WeldingDecal/M_WeldingHitDecal.M_WeldingHitDecal" "6.000000,4.000000,4.000000" (Variables|/Script/Engine.Actor|GetRootComponent ActorToAttachTo) "None" AttachPoint (Math|Conversions|RotationFromXVector Normal) "KeepWorldPosition" 5.0))
  (Rendering|Components|Decal|SetFadeOut _returnvalue 0.0 5.0 false)
  (Transformation|AddLocalRotation _returnvalue (Math|Rotator|MakeRotator (Math|Random|RandomFloatinRange -1.8e+02 1.8e+02) 0.0 0.0) false false)
  (Rendering|Components|Decal|SetFadeScreenSize _returnvalue 0.002))

(event Custom|ApplyDamage_Multicast
  (params (Actor :type Object%20Object%20Reference) (DeltaTime :type Float%20%28double-precision%29))
  (Class|BPIDamagable|TakeDamage(Message) Actor (Utilities|Struct|MakeS_DamageInfo (* DeltaTime (Variables|Default|GetHitDamage)) "/Game/Dynamic/Blueprints/DamageTypes/BP_PhysicalDamage.BP_PhysicalDamage_C" false)))

(event EventBeginPlay
  (|CallParentFunction) ; This node is disabled and will not be called.\nDrag off pins to build functionality.
)

(event Collision|EventActorBeginOverlap
  (params (OtherActor :type Actor%20Object%20Reference))
  (|CallParentFunction OtherActor) ; This node is disabled and will not be called.\nDrag off pins to build functionality.
)

(event EventUsewithHitResult
  (params (PlayerStat :type BPC%20Player%20Stats%20System%20Object%20Reference) (HitResult :type Hit%20Result%20Structure) (DeltaSecond :type Float%20%28double-precision%29))
  (bind (_bblockinghit _binitialoverlap _time _distance _location _impactpoint _normal _impactnormal _physmat _hitactor _hitcomponent _hitbonename _bonename _hititem _elementindex _faceindex _tracestart _traceend) (Collision|BreakHitResult HitResult))
  (bind (_bblockinghit_2 _binitialoverlap_2 _time_2 _distance_2 _location_2 _impactpoint_2 _normal_2 _impactnormal_2 _physmat_2 _hitactor_2) (Collision|BreakHitResult HitResult))
  (|CallParentFunction PlayerStat HitResult DeltaSecond)
  (Utilities|FlowControl|Sequence
    (:then_0
      (CallFunction|UpdateLaserFX (Math|Vector|SelectVector _impactpoint _traceend _bblockinghit)))
    (:then_1
      (if _bblockinghit_2
        (bind _returnvalue (GameplayTags|HasMatchingGameplayTag(Message) _hitactor_2 "(TagName=\"Damageable.Character.Enemy\")"))
        (if _returnvalue
          (Networking|SwitchHasAuthority
            (:Authority
              (CallFunction|ApplyDamageMulticast _hitactor_2 DeltaSecond)))
          (else
            (CallFunction|SpawnDecal _hitactor_2 _impactpoint_2 _impactnormal_2)))))))

(event EventTick
  (params (DeltaSeconds :type Float%20%28single-precision%29))
  (|CallParentFunction DeltaSeconds) ; This node is disabled and will not be called.\nDrag off pins to build functionality.
)

(event EventFix
  (params (PlayerStat :type BPC%20Player%20Stats%20System%20Object%20Reference) (DeltaTime :type Float%20%28double-precision%29) (HitResult :type Hit%20Result%20Structure))
  (bind (_bblockinghit _binitialoverlap _time _distance _location _impactpoint _normal _impactnormal) (Collision|BreakHitResult HitResult))
  (|CallParentFunction PlayerStat DeltaTime HitResult)
  (CallFunction|UpdateWeldingFX _impactpoint _impactnormal))

(event EventActivate
  ;[0.01042 0.01042 0.01042] Activate / Deactivate
  (|CallParentFunction)
  (CallFunction|ActivateLaserFX))

(event EventGotTarget
  ;[0.01042 0.01042 0.01042] Target Got / Lost
  (|CallParentFunction)
  (CallFunction|ActivateWeldingFX))

(event EventLostTarget
  ;[0.01042 0.01042 0.01042] Target Got / Lost
  (|CallParentFunction)
  (CallFunction|DeactivateWieldingVX))

(event EventDeactivate
  ;[0.01042 0.01042 0.01042] Activate / Deactivate
  (|CallParentFunction)
  (CallFunction|DeactivateLaserFX))

(fn ConstructionScript
  (|CallParentFunction))

(fn UseHitResultCosmetic
  (params (HitResult :type Hit%20Result%20Structure))
  (bind (_bblockinghit _binitialoverlap _time _distance _location _impactpoint _normal _impactnormal _physmat _hitactor _hitcomponent _hitbonename _bonename _hititem _elementindex _faceindex _tracestart _traceend) (Collision|BreakHitResult HitResult))
  (|CallParentFunction HitResult)
  (CallFunction|UpdateLaserFX (Math|Vector|SelectVector _impactpoint _traceend _bblockinghit)))