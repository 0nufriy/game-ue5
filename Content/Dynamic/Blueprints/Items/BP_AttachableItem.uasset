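; BP_AttachableItem is a wieldable item that pawns pick up, drop with an impulse and can use as a projectile to damage enemies.
; Interact disables physics and collision, and runs automatically on BeginPlay when a pawn owns the item; Drop restores both.
; Authority multicasts hits, which ignore the last owner and stop further pawn collision.
; A DoOnce, re-armed on pickup, limits physical damage and its damage-event report to one enemy.
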(event Custom|HitMulticast
  (params (Actor :type Actor%20Object%20Reference) (HitLocation :type Vector))
  (bind _staticmesh (Variables|Default|GetStaticMesh))
  (if (!= Actor (Variables|Components|GetLastOwner))
    (Class|PrimitiveComponent|SetNotifyRigidBodyCollision _staticmesh false)
    (Collision|SetCollisionResponsetoChannel _staticmesh "ECC_Pawn" "ECR_Ignore")
    (bind _returnvalue (GameplayTags|HasMatchingGameplayTag(Message) Actor "(TagName=\"Damageable.Character.Enemy\")"))
    (if _returnvalue
      (Utilities|FlowControl|DoOnce false
        (:Completed
          (Class|BPIDamagable|TakeDamage(Message) Actor (Utilities|Struct|MakeS_DamageInfo (Variables|Combat|GetDamageFromHit_0) "/Game/Dynamic/Blueprints/DamageTypes/BP_PhysicalDamage.BP_PhysicalDamage_C" false))
          (Class|AISenseDamage|ReportDamageEvent 0 (Variables|Components|GetLastOwner) (Variables|Combat|GetDamageFromHit_0) HitLocation "0, 0, 0" "None"))))))

(event Custom|ResetDamagaCausing
  (Utilities|FlowControl|DoOnce false) ; enters at Reset
)

(event EventInteract
  (params (Owner :type Pawn%20Object%20Reference))
  (bind _staticmesh (Variables|Default|GetStaticMesh))
  ;[0.01042 0.01042 0.01042] Interaction
  (|CallParentFunction Owner)
  (Physics|SetSimulatePhysics _staticmesh false)
  (Collision|SetCollisionEnabled _staticmesh "NoCollision")
  (Variables|Components|SetCurrentOwner Owner)
  (Variables|Default|SetIsWielded true)
  (CallFunction|ResetDamagaCausing))

(event EventBeginPlay
  (|CallParentFunction)
  (bind _aspawn (Utilities|Casting|CastToPawn (Components|GetOwner)))
  (CallFunction|Interact _aspawn))

(event Collision|EventHit
  (params (MyComp :type Primitive%20Component%20Object%20Reference) (Other :type Actor%20Object%20Reference) (OtherComp :type Primitive%20Component%20Object%20Reference) (bSelfMoved :type Boolean) (HitLocation :type Vector :default "0, 0, 0") (HitNormal :type Vector :default "0, 0, 0") (NormalImpulse :type Vector :default "0, 0, 0") (Hit :type Hit%20Result%20Structure%20%28by%20ref%29))
  (Networking|SwitchHasAuthority
    (:Authority
      (CallFunction|HitMulticast Other HitLocation))))

(event EventApplyImpulse
  (params (Impulse :type Vector :default "0, 0, 0"))
  (if (not (Variables|Default|GetIsWielded))
    (Physics|AddImpulse (Variables|Default|GetStaticMesh) Impulse "None" false)))

(event EventDrop
  (params (Impulse :type Vector :default "0, 0, 0"))
  (bind _staticmesh (Variables|Default|GetStaticMesh))
  ;[0.01042 0.01042 0.01042] Interaction
  (Physics|SetSimulatePhysics _staticmesh true)
  (Collision|SetCollisionEnabled _staticmesh "QueryAndPhysics")
  (Collision|SetCollisionResponsetoChannel _staticmesh "ECC_Pawn" "ECR_Block")
  (Physics|AddImpulse _staticmesh Impulse "None" true)
  (Class|PrimitiveComponent|SetNotifyRigidBodyCollision _staticmesh true)
  (Variables|Components|SetLastOwner (Variables|Components|GetCurrentOwner))
  (Variables|Components|SetCurrentOwner 0)
  (Variables|Default|SetIsWielded false))

(fn ConstructionScript)

(fn GetAttachSocket
  (return (Variables|Initialization|GetAttachSocket)))