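; BP_OxTank is an attachable oxygen tank item that supplies the player's oxygen stat.
; On Interact it attaches its current and max values to the owner's BPC_Player_StatsSystem, binds to the oxygen run-out event and sets the owner's tank message.
; On Drop it unbinds, copies the oxygen values back and detaches.
; DoOnZero signals tank detachment and clears the tank message.
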(event EventDrop
  (params (Impulse :type Vector :default "0, 0, 0"))
  (|CallParentFunction Impulse)
  (EventDispatchers|UnbindEventfromOnOxRunOut (Variables|Default|GetPlayerStats) (EventDispatchers|CreateEvent :!event OnZeroStat))
  (Variables|Default|SetCurrentStat (Variables|/Game/Dynamic/Blueprints/Components/StatsSystemComponent/Player/BPC_Player_StatsSystem.BPC_Player_StatsSystem_C|GetOxCurent (Variables|Default|GetPlayerStats)))
  (Variables|Default|SetMaxStat (Variables|/Game/Dynamic/Blueprints/Components/StatsSystemComponent/Player/BPC_Player_StatsSystem.BPC_Player_StatsSystem_C|GetOxMax (Variables|Default|GetPlayerStats)))
  (Default|DetachTank (Variables|Default|GetPlayerStats))
  (Variables|Default|SetPlayerStats 0))

(event Collision|EventActorBeginOverlap
  (params (OtherActor :type Actor%20Object%20Reference))
  (|CallParentFunction OtherActor) ; This node is disabled and will not be called.\nDrag off pins to build functionality.
)

(event EventTick
  (params (DeltaSeconds :type Float%20%28single-precision%29))
  (|CallParentFunction DeltaSeconds) ; This node is disabled and will not be called.\nDrag off pins to build functionality.
)

(event EventInteract
  (params (Owner :type Pawn%20Object%20Reference))
  (bind _currentowner (Variables|Default|GetCurrentOwner))
  (|CallParentFunction Owner)
  (bind _hasoxygen (Class|BPIHasOxygen|HasOxygen(Message) _currentowner))
  (if _hasoxygen
    (Class|BPIHasOxygen|DropOxygen(Message) _currentowner))
  (bind _output_get (Variables|Default|SetPlayerStats (Actor|GetComponentbyClass (Variables|Default|GetCurrentOwner) "/Game/Dynamic/Blueprints/Components/StatsSystemComponent/Player/BPC_Player_StatsSystem.BPC_Player_StatsSystem_C")))
  (Default|AttachTank _output_get (Variables|Default|GetCurrentStat) (Variables|Default|GetMaxStat))
  (EventDispatchers|BindEventtoOnOxRunOut (Variables|Default|GetPlayerStats) (EventDispatchers|CreateEvent :!event OnZeroStat))
  (Class|BPIHasOxygen|SetOxygenTank(Message) (Variables|Default|GetCurrentOwner) self))

(fn ConstructionScript
  (|CallParentFunction))

(fn DoonZero
  (Default|CallOnOxTankDetached (Variables|Default|GetPlayerStats))
  (Class|BPIHasOxygen|ClearOxygenTank(Message) (Variables|Default|GetCurrentOwner)))