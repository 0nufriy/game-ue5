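; BP_AttachableResource is an attachable resource actor with a depletable stat, set to its maximum on BeginPlay.
; When OnZeroStat fires, only the authority acts, calling OnZeroMulticast and then destroying the actor.
; The multicast event runs DoOnZero, an empty function that appears to be a hook for child Blueprints to add depletion behavior.
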(event Custom|OnZeroStat
  (Networking|SwitchHasAuthority
    (:Authority
      (CallFunction|OnZeroMulticast)
      (Actor|DestroyActor))))

(event Custom|OnZeroMulticast
  (CallFunction|DoonZero))

(event EventBeginPlay
  (|CallParentFunction)
  (Variables|Default|SetCurrentStat (Variables|Default|GetMaxStat)))

(event Collision|EventActorBeginOverlap
  (params (OtherActor :type Actor%20Object%20Reference))
  (|CallParentFunction OtherActor) ; This node is disabled and will not be called.\nDrag off pins to build functionality.
)

(event EventTick
  (params (DeltaSeconds :type Float%20%28single-precision%29))
  (|CallParentFunction DeltaSeconds) ; This node is disabled and will not be called.\nDrag off pins to build functionality.
)

(fn ConstructionScript
  (|CallParentFunction))

(fn DoonZero)