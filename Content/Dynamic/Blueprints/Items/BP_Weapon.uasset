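; Wieldable projectile weapon item with ammo, fire rate, overheat, recoil and a HUD widget created for the local owner on pickup.
; Use checks cooldown, heat and magazine, then asks the owner's controller to spawn the bullet and spend ammo.
; Tick drains cooldown and heat; shots play sound and report noise.
; In multiplayer the wielding client simulates fire state, passing it to its controller on drop, while authority multicasts it on pickup.
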(event Custom|OnTriggerEnd
  (Updates|UpdateStatsforTrigger)
  (Variables|Default|SetAim%20Component 0))

(event Custom|ApplyRecoil
  (bind _player (Class|BPIPlayers|GetPlayer(Message) (Variables|Default|GetCurrentOwner)))
  (Utilities|IsValid _player
    (:Is%20Valid
      (Default|Recoil _player (Variables|Recoil|GetRecoil%20Amp) (Variables|Recoil|GetSideways) (Variables|Recoil|GetRandom%20Max) (Variables|Recoil|GetRandom%20Min)))))

(event Custom|Client_SetOverheatHUD
  (Default|SetOverHeat (Variables|Default|GetWeaponWidget) (Variables|Compat|GetOverHeatNow) (Variables|Compat|GetOverHeat) (Variables|Compat|GetIsOverHeat)))

(event Custom|AddSoundForFire
  (params (ShotLocation :type Vector))
  (Audio|Components|Audio|Play (Variables|Default|GetGunShot) 0.0)
  (Class|AISenseHearing|ReportNoiseEvent ShotLocation 1.0 (Variables|Default|GetCurrentOwner) 0.0 "None"))

(event Custom|SetWeaponState
  (params (FireTime :type Float%20%28double-precision%29) (OverHeatNow :type Float%20%28double-precision%29))
  (Variables|Compat|SetFireTime FireTime)
  (Variables|Compat|SetOverHeatNow OverHeatNow))

(event Custom|SetWeaponStateMulticast
  (params (FireTime :type Float%20%28double-precision%29) (OverHeatNow :type Float%20%28double-precision%29))
  (Variables|Compat|SetFireTime FireTime)
  (Variables|Compat|SetOverHeatNow OverHeatNow))

(event Custom|Client_SetAmmoOnHUD
  (params (Ammo :type Integer))
  (Default|SetAmmo (Variables|Default|GetWeaponWidget) Ammo))

(event Custom|Client_RemoveWidget
  (Widget|RemovefromParent (Variables|Default|GetWeaponWidget)))

(event Custom|SpawnBullet
  (bind _aim_component (Variables|Default|GetAim%20Component))
  (bind _returnvalue (Transformation|GetWorldLocation _aim_component))
  (bind _returnvalue_2 (Transformation|GetWorldRotation _aim_component))
  (bind _returnvalue_3 (Game|SpawnActorfromClass (Variables|Compat|GetProjectail) (Math|Transform|MakeTransform _returnvalue _returnvalue_2 "1.000000,1.000000,1.000000") "Undefined" "MultiplyWithRoot" 0 (Variables|Default|GetCurrentOwner)))
  (if (Variables|Debug|GetDrawDebugTrace)
    (Debug|DrawDebugArrow _returnvalue _returnvalue_2))
  (Variables|/Game/Dynamic/Blueprints/Items/Weapons/Projectile/BP_Projectaile.BP_Projectaile_C|SetDamage _returnvalue_3 (Variables|Compat|GetDamage))
  (CallFunction|AddSoundforFire _returnvalue))

(event EventBeginPlay
  (|CallParentFunction) ; This node is disabled and will not be called.\nDrag off pins to build functionality.
)

(event Collision|EventActorBeginOverlap
  (params (OtherActor :type Actor%20Object%20Reference))
  (|CallParentFunction OtherActor) ; This node is disabled and will not be called.\nDrag off pins to build functionality.
)

(event EventTick
  (params (DeltaSeconds :type Float%20%28single-precision%29))
  (|CallParentFunction DeltaSeconds)
  (bind _ismultiplayer (Class|BPIMultiplayer|GetIsMultiplayer(Message) (Game|GetGameInstance)))
  (if _ismultiplayer
    (if (Variables|Default|GetIsWielded)
      (if (Pawn|IsLocallyControlled (Variables|Default|GetCurrentOwner))
        (if (<= (Variables|Compat|GetFireTime) 0.0) :!label _label
          _
          (else
            (Variables|Compat|SetFireTime (- (Variables|Compat|GetFireTime) DeltaSeconds))))
        (if (<= (Variables|Compat|GetOverHeatNow) 0.0)
          (if (Variables|Compat|GetIsOverHeat)
            (Variables|Compat|SetIsOverHeat false)
            (if (Variables|Default|GetIsWielded) :!label _label_2
              (CallFunction|ClientSetOverheatHUD)))
          (else
            (Variables|Compat|SetOverHeatNow (- (Variables|Compat|GetOverHeatNow) DeltaSeconds))
            (goto _label_2))))
      (elif (Networking|IsServer)
        (goto _label)))
    (else
      (goto _label))))

(event EventAddCurrentCharge
  (params (Amount :type Float%20%28double-precision%29))
  (bind _returnvalue (Class|KismetMathLibrary|ToInt64(Float) Amount))
  (bind _returnvalue_2 (Math|Conversions|ToInteger(Byte) _returnvalue))
  (Networking|SwitchHasAuthority
    (:Authority
      (if (> _returnvalue_2 0)
        (bind _output_get (Variables|Compat|SetBullet (Math|Integer|Clamp(Integer) (+ (Variables|Compat|GetBullet) _returnvalue_2) 1 (Variables|Compat|GetBulletMax))))
        (CallFunction|ClientSetAmmoonHUD _output_get)))))

(event EventUse
  (params (AimComponent :type BP%20Grab%20Component%20Object%20Reference) (PlayerStats :type BPC%20Player%20Stats%20System%20Object%20Reference) (DeltaTime :type Float%20%28double-precision%29))
  (Variables|Default|SetAim%20Component AimComponent)
  (bind _ismultiplayer (Class|BPIMultiplayer|GetIsMultiplayer(Message) (Game|GetGameInstance)))
  (if _ismultiplayer
    (if (Pawn|IsLocallyControlled (Variables|Default|GetCurrentOwner))
      (if (Checks|CanFire) :!label _label
        (Shooting|Trigger)))
    (else
      (goto _label))))

(event EventDrop
  (params (Impulse :type Vector :default "0, 0, 0"))
  (bind _currentowner (Variables|Default|GetCurrentOwner))
  (Utilities|FlowControl|Sequence
    (:then_0
      (bind _ismultiplayer (Class|BPIMultiplayer|GetIsMultiplayer(Message) (Game|GetGameInstance)))
      (if (and _ismultiplayer (Pawn|IsLocallyControlled _currentowner))
        (Class|BPIController|SetWeaponState(Message) (Pawn|GetController _currentowner) (Variables|Compat|GetFireTime) (Variables|Compat|GetOverHeatNow) self)))
    (:then_1
      (Networking|SwitchHasAuthority
        (:Authority
          (CallFunction|ClientRemoveWidget))))
    (:then_2
      (|CallParentFunction Impulse))))

(event EventInteract
  (params (Owner :type Pawn%20Object%20Reference))
  (bind _currentowner (Variables|Default|GetCurrentOwner))
  (|CallParentFunction Owner)
  (Utilities|FlowControl|Sequence
    (:then_0
      (if (Pawn|IsLocallyControlled _currentowner)
        (bind _asplayer_controller (Utilities|Casting|CastToPlayerController (Pawn|GetController _currentowner)))
        (bind _returnvalue (UserInterface|CreateWidget "/Game/Dynamic/Blueprints/UI/GrabItem/UI_Weapon.UI_Weapon_C" _asplayer_controller (Variables|Compat|GetBulletMax)))
        (bind _output_get (Variables|Default|SetWeaponWidget _returnvalue))
        (UserInterface|Viewport|AddtoPlayerScreen _output_get)
        (CallFunction|ClientSetAmmoonHUD (Variables|Compat|GetBullet))
        (CallFunction|ClientSetOverheatHUD)))
    (:then_1
      (bind _ismultiplayer (Class|BPIMultiplayer|GetIsMultiplayer(Message) (Game|GetGameInstance)))
      (if _ismultiplayer
        (Networking|SwitchHasAuthority
          (:Authority
            (CallFunction|SetWeaponStateMulticast (Variables|Compat|GetFireTime) (Variables|Compat|GetOverHeatNow))))))))

(fn ConstructionScript
  (|CallParentFunction))

(fn SetAmmoonHUD
  (Default|SetAmmo (Variables|Default|GetWeaponWidget) (Variables|Compat|GetBullet)))

(fn DrawDebugArrow
  (params (Start :type Vector) (RotationToTargetPoint :type Rotator))
  (Rendering|Debug|DrawDebugArrow :LineStart Start :LineEnd (+ (* (Math|Vector|GetForwardVector RotationToTargetPoint) 1e+03) Start) :ArrowSize 1.0 :Duration 1e+01 :Thickness 1.0))

(fn GetAmmoType
  (return (Variables|Default|GetAmmoType)))

(fn CanFire
  (return (Math|Boolean|ANDBoolean (not (Variables|Compat|GetIsOverHeat)) (<= (Variables|Compat|GetFireTime) 0.0) (not (Checks|IsMagazineEmpty)))))

(fn Trigger
  (Shooting|Fire)
  (Updates|UpdateStatsforTrigger))

(fn GetOverheatforTrigger
  (return (Variables|Compat|GetOverHeatByFire)))

(fn Fire
  (Utilities|FlowControl|Sequence
    (:then_0
      (Class|BPIController|SpawnBullet(Message) (Pawn|GetController (Variables|Default|GetCurrentOwner)) self))
    (:then_1
      (CallFunction|ApplyRecoil))
    (:then_2
      (Class|BPIController|DecreasBullet(Message) (Pawn|GetController (Variables|Default|GetCurrentOwner)) self))))

(fn UpdateBulletsforFire
  (bind _output_get (Variables|Compat|SetBullet (- (Variables|Compat|GetBullet) 1)))
  (Networking|SwitchHasAuthority
    (:Authority
      (CallFunction|ClientSetAmmoonHUD _output_get))))

(fn UpdateStatsforTrigger
  (Variables|Compat|SetFireTime (/ 1.0 (Variables|Compat|GetFireRate)))
  (Variables|Compat|SetOverHeatNow (+ (Variables|Compat|GetOverHeatNow) (CallFunction|GetOverheatforTrigger)))
  (if (>= (Variables|Compat|GetOverHeatNow) (Variables|Compat|GetOverHeat))
    (Updates|SetIsOverheat)))

(fn IsMagazineEmpty
  (return (== (Variables|Compat|GetBullet) 0)))

(fn SetIsOverheat
  (Variables|Compat|SetIsOverHeat true))

(fn OnRepOverHeatNow
  (Default|SetOverHeat (Variables|Default|GetWeaponWidget) (Variables|Compat|GetOverHeatNow) (Variables|Compat|GetOverHeat) (Variables|Compat|GetIsOverHeat)))

(fn OnRepIsOverHeat
  (if (Variables|Compat|GetIsOverHeat)
    (Default|CallOnOverheat)
    (Audio|Components|Audio|Play (Variables|Default|GetGunOverHeat) 0.0)))

(fn GetCurrentCharge
  (return (Math|Conversions|ToFloat(Integer) (Variables|Compat|GetBullet))))

(fn GetMaxCharge
  (return (Math|Conversions|ToFloat(Integer) (Variables|Compat|GetBulletMax))))