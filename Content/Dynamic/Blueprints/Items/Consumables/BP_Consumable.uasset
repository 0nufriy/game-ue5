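; Base consumable item that a character uses by playing a usage montage, with an empty multicast consume event.
; StartUse plays the montage on the owner's mesh; on completion the authority fires the consume multicast, tells the owner to drop the item and destroys it.
; Releasing or dropping blends the montage out to cancel consumption.
; ConsumeBegin, ConsumeTick and ConsumeEnd track clamped use time and report it as normalized fullness.
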(event Custom|ConsumeMulticast
  ;[0.01042 0.01042 0.01042] Consume
)

(event Custom|StopConsumption
  (bind _usagemontage (Variables|Default|GetUsageMontage))
  (if (Variables|Default|GetbIsConsuming)
    (Class|AnimInstance|MontageStopwithBlendOut (Components|SkeletalMesh|GetAnimInstance (Variables|Default|GetOwnerMesh)) (Class|AnimMontage|GetBlendOutArgs _usagemontage) _usagemontage)))

(event Custom|ConsumeServerOnly
  ;[0.01042 0.01042 0.01042] Consume
  (CallFunction|ConsumeMulticast)
  (bind _player (Class|BPIPlayers|GetPlayer(Message) (Variables|Default|GetCurrentOwner)))
  (Default|DropItemMulticast _player)
  (Actor|DestroyActor))

(event EventStartUse
  ;[0.01042 0.01042 0.01042] Use
  (|CallParentFunction)
  (bind _ownermesh (Variables|Default|GetOwnerMesh)
    (:then
      (Animation|Montage|PlayMontage _ownermesh (Variables|Default|GetUsageMontage)
        (:then
          (Variables|Default|SetbIsConsuming true))
        (:OnCompleted
          (Variables|Default|SetbIsConsuming false)
          (Networking|SwitchHasAuthority
            (:Authority
              (CallFunction|ConsumeServerOnly))))
        (:OnInterrupted
          (Variables|Default|SetbIsConsuming false))))
    (:else)))

(event EventUse
  (params (AimComponent :type BP%20Grab%20Component%20Object%20Reference) (PlayerStats :type BPC%20Player%20Stats%20System%20Object%20Reference) (DeltaTime :type Float%20%28double-precision%29))
  ;[0.01042 0.01042 0.01042] Use
  (|CallParentFunction AimComponent PlayerStats DeltaTime))

(event EventInteract
  (params (Owner :type Pawn%20Object%20Reference))
  ;[0.01042 0.01042 0.01042] Interactable
  (|CallParentFunction Owner)
  (bind _ascharacter (Utilities|Casting|CastToCharacter (Variables|Default|GetCurrentOwner)))
  (Variables|Default|SetOwnerMesh (Variables|/Script/Engine.Character|GetMesh _ascharacter)))

(event EventConsumeBegin
  (params (Duration :type Float%20%28double-precision%29))
  ;[0.01042 0.01042 0.01042] Consumer
  (Variables|Default|SetTimeToDone Duration)
  (CallFunction|SetCurrentUseTime 0.0))

(event EventReleasUse
  ;[0.01042 0.01042 0.01042] Use
  (|CallParentFunction)
  (CallFunction|StopConsumption))

(event EventDrop
  (params (Impulse :type Vector :default "0, 0, 0"))
  ;[0.01042 0.01042 0.01042] Interactable
  (|CallParentFunction Impulse)
  (Variables|Default|SetCurrentUseTime 0.0)
  (CallFunction|StopConsumption))

(event EventConsumeTick
  ;[0.01042 0.01042 0.01042] Consumer
  (CallFunction|SetCurrentUseTime (+ (Variables|Default|GetCurrentUseTime) (Utilities|Time|GetWorldDeltaSeconds))))

(event EventConsumeEnd
  (params (ReachedEnd :type Boolean))
  ;[0.01042 0.01042 0.01042] Consumer
  (CallFunction|SetCurrentUseTime (Variables|Default|GetTimeToDone)))

(fn ConstructionScript
  (|CallParentFunction))

(fn DoonConsume)

(fn SetCurrentUseTime
  (params (NewUseTime :type Float%20%28double-precision%29))
  (Variables|Default|SetCurrentUseTime (Math|Float|Clamp(Float) NewUseTime 0.0 (Variables|Default|GetTimeToDone)))
  (Default|CallOnFullnessChange (Math|Float|Clamp(Float) (/ (Variables|Default|GetCurrentUseTime) (Variables|Default|GetTimeToDone)))))