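; Health consumable item, a child of a consumable base class, that heals its current owner by HealAmount.
; On BeginPlay it creates a dynamic material for the mesh's tube slot, and fullness change events drive its Fullness parameter with the inverted percent.
; Both the ConsumeMulticast event and the DoOnConsume function send HealMessage to the owner, with the multicast then calling its parent implementation.
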(event EventBeginPlay
  (|CallParentFunction)
  (bind _returnvalue (Rendering|Material|CreateDynamicMaterialInstance (Variables|Default|GetStaticMesh) 8 "/Game/Static/Items/SciFiSyringe/Materials/Tube_001.Tube_001" "None" :!class /Script/Engine.PrimitiveComponent))
  (Variables|Default|SetTubeMaterial _returnvalue))

(event Collision|EventActorBeginOverlap
  (params (OtherActor :type Actor%20Object%20Reference))
  (|CallParentFunction OtherActor) ; This node is disabled and will not be called.\nDrag off pins to build functionality.
)

(event EventTick
  (params (DeltaSeconds :type Float%20%28single-precision%29))
  (|CallParentFunction DeltaSeconds) ; This node is disabled and will not be called.\nDrag off pins to build functionality.
)

(event EventConsumeMulticast
  (Class|BPIDamagable|Heal(Message) (Variables|Default|GetCurrentOwner) (Variables|Default|GetHealAmount))
  (|CallParentFunction))

(event EventOnFullnessChangeEvent
  (params (NewPercent :type Float%20%28double-precision%29))
  (Rendering|Material|SetScalarParameterValue (Variables|Default|GetTubeMaterial) "Fullness" (- 1.0 NewPercent) :!class /Script/Engine.MaterialInstanceDynamic))

(fn ConstructionScript
  (|CallParentFunction))

(fn DoonConsume
  (Class|BPIDamagable|Heal(Message) (Variables|Default|GetCurrentOwner) (Variables|Default|GetHealAmount)))