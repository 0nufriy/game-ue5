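; Consumable item Blueprint whose use progress drains gradually after the player lets go, going by its SoftRelease name and release logic.
; Use clears the Restoring flag and ReleasUse sets it, each after calling the parent logic.
; While Restoring, the authority's Tick calls ReleaseMulticast, which lowers CurrentUseTime by the frame delta and clears the flag when it equals zero.
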(event Custom|ReleaseMulticast
  (params (Deltatime :type Float%20%28double-precision%29))
  (CallFunction|SetCurrentUseTime (- (Variables|Default|GetCurrentUseTime) Deltatime))
  (if (== (Variables|Default|GetCurrentUseTime) 0.0)
    (Variables|Default|SetbRestoring false)))

(event EventBeginPlay
  (|CallParentFunction) ; This node is disabled and will not be called.\nDrag off pins to build functionality.
)

(event Collision|EventActorBeginOverlap
  (params (OtherActor :type Actor%20Object%20Reference))
  (|CallParentFunction OtherActor) ; This node is disabled and will not be called.\nDrag off pins to build functionality.
)

(event EventTick
  (params (DeltaSeconds :type Float%20%28single-precision%29))
  (|CallParentFunction DeltaSeconds)
  (Networking|SwitchHasAuthority
    (:Authority
      (if (Variables|Default|GetbRestoring)
        (CallFunction|ReleaseMulticast DeltaSeconds)))))

(event EventReleasUse
  (|CallParentFunction)
  (Variables|Default|SetbRestoring true))

(event EventUse
  (params (AimComponent :type BP%20Grab%20Component%20Object%20Reference) (PlayerStats :type BPC%20Player%20Stats%20System%20Object%20Reference) (DeltaTime :type Float%20%28double-precision%29))
  (|CallParentFunction AimComponent PlayerStats DeltaTime)
  (Variables|Default|SetbRestoring false))

(fn ConstructionScript
  (|CallParentFunction))