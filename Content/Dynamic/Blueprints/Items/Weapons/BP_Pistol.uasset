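; BP_Pistol is a pistol weapon Blueprint that fires semi-automatically, one shot per press of use.
; It extends a parent weapon class, overriding Trigger to set an IsFire flag before calling the parent.
; CanFire passes only if the parent allows it and IsFire is false, and ReleasUse clears the flag so the next press can fire.
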(event EventBeginPlay
  (|CallParentFunction))

(event Collision|EventActorBeginOverlap
  (params (OtherActor :type Actor%20Object%20Reference))
  (|CallParentFunction OtherActor) ; This node is disabled and will not be called.\nDrag off pins to build functionality.
)

(event EventTick
  (params (DeltaSeconds :type Float%20%28single-precision%29))
  (|CallParentFunction DeltaSeconds) ; This node is disabled and will not be called.\nDrag off pins to build functionality.
)

(event EventReleasUse
  (|CallParentFunction)
  (Variables|Default|SetIsFire? false))

(fn ConstructionScript
  (|CallParentFunction))

(fn CanFire
  (return (and (|CallParentFunction) (not (Variables|Default|GetIsFire?)))))

(fn Trigger
  (Variables|Default|SetIsFire? true)
  (|CallParentFunction))