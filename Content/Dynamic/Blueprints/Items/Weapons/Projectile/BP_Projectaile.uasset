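; Projectile actor for weapons that applies physical damage to enemy characters it hits, then destroys itself.
; Hit processing runs only with authority, with an optional debug sphere at the impact point, and forwards through a server event.
; Targets tagged as damageable enemies receive damage through a message call and a damage event report.
; Every processed hit also reports a "Bullet" noise event at the impact location.
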(event Custom|Hit%20Actor
  (params (HitActor :type Actor%20Object%20Reference) (HitLocation :type Vector))
  (Utilities|FlowControl|Sequence
    (:then_0
      (bind _returnvalue (GameplayTags|HasMatchingGameplayTag(Message) HitActor "(TagName=\"Damageable.Character.Enemy\")"))
      (if _returnvalue
        (Class|BPIDamagable|TakeDamage(Message) HitActor (Utilities|Struct|MakeS_DamageInfo (Variables|Shoot|GetDamage) "/Game/Dynamic/Blueprints/DamageTypes/BP_PhysicalDamage.BP_PhysicalDamage_C" false))
        (Class|AISenseDamage|ReportDamageEvent HitActor (Variables|Actor|GetInstigator) (Variables|Shoot|GetDamage) HitLocation "0, 0, 0" "None")))
    (:then_1
      (Class|AISenseHearing|ReportNoiseEvent HitLocation 1.0 (Variables|Actor|GetInstigator) 0.0 "Bullet"))
    (:then_2
      (Actor|DestroyActor))))

(event Custom|HitActorServer
  (params (HitActor :type Actor%20Object%20Reference) (HitLocation :type Vector))
  (CallFunction|HitActor HitActor HitLocation))

(event EventTick
  (params (DeltaSeconds :type Float%20%28single-precision%29))
  ;[1 1 1] If need to debug projectile movement
)

(event Collision|EventHit
  (params (MyComp :type Primitive%20Component%20Object%20Reference) (Other :type Actor%20Object%20Reference) (OtherComp :type Primitive%20Component%20Object%20Reference) (bSelfMoved :type Boolean) (HitLocation :type Vector :default "0, 0, 0") (HitNormal :type Vector :default "0, 0, 0") (NormalImpulse :type Vector :default "0, 0, 0") (Hit :type Hit%20Result%20Structure%20%28by%20ref%29))
  (Networking|SwitchHasAuthority
    (:Authority
      (if (Variables|Debug|GetShowHitPoint)
        (Rendering|Debug|DrawDebugSphere HitLocation 1.0 12 "(R=0.057249,G=1.000000,B=0.000000,A=1.000000)" 3.0 2.0))
      (CallFunction|HitActorServer Other HitLocation))))

(fn ConstructionScript)