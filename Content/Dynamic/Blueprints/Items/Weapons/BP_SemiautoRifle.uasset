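; Semi-automatic rifle weapon that fires one burst per trigger pull, extending a parent weapon Blueprint.
; Trigger fires the first shot and starts a looping timer for the follow-up shots, with TryFire stopping it when the burst or magazine runs out.
; CanFire blocks new shots until the trigger is released and the timer has ended.
; Overheat per trigger scales with the number of bullets fired in the burst.
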(event Custom|TryFire
  (if (or (<= (Variables|Default|GetBulletsLeftInBurst) 0) (CallFunction|IsMagazineEmpty))
    (Variables|Default|SetBulletsLeftInBurst (Variables|Default|GetMaxBulletsInBurst))
    (Utilities|Time|ClearandInvalidateTimerbyHandle (Variables|Default|GetSemiTimer))
    (CallFunction|OnTriggerEnd)
    (else
      (Variables|Default|SetBulletsLeftInBurst (- (Variables|Default|GetBulletsLeftInBurst) 1))
      (CallFunction|Fire))))

(event EventBeginPlay
  (|CallParentFunction)
  (Variables|Default|SetBulletsLeftInBurst (Variables|Default|GetMaxBulletsInBurst)))

(event Collision|EventActorBeginOverlap
  (params (OtherActor :type Actor%20Object%20Reference))
  (|CallParentFunction OtherActor) ; This node is disabled and will not be called.\nDrag off pins to build functionality.
)

(event EventTick
  (params (DeltaSeconds :type Float%20%28single-precision%29))
  (|CallParentFunction DeltaSeconds) ; This node is disabled and will not be called.\nDrag off pins to build functionality.
)

(event EventReleasUse
  (|CallParentFunction)
  (Variables|Default|SetTriggeredFire? false))

(fn ConstructionScript
  (|CallParentFunction))

(fn CanFire
  (return (Math|Boolean|ANDBoolean (|CallParentFunction) (not (Variables|Default|GetTriggeredFire?)) (not (Utilities|Time|IsTimerActivebyHandle (Variables|Default|GetSemiTimer))))))

(fn GetOverheatforTrigger
  (return (* (Variables|Default|GetOverHeatByFire) (- (Variables|Default|GetMaxBulletsInBurst) (Variables|Default|GetBulletsLeftInBurst)))))

(fn UpdateBulletsforFire
  (|CallParentFunction))

(fn UpdateStatsforTrigger
  (|CallParentFunction))

(fn Trigger
  (Variables|Default|SetTriggeredFire? true)
  (CallFunction|Fire)
  (Variables|Default|SetBulletsLeftInBurst (- (Variables|Default|GetBulletsLeftInBurst) 1))
  (bind _returnvalue (Utilities|Time|SetTimerbyEvent (EventDispatchers|CreateEvent :!event Custom|TryFire) (Variables|Default|GetDelayBetweenBullets) true))
  (Variables|Default|SetSemiTimer _returnvalue))